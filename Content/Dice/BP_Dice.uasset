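; BP_Dice is a tabletop RPG dice roller supporting d4 through d100 with modifiers, advantage and critical detection.
; Roll sums RollDie results per die type, then adds the static modifier and the roller's stat and proficiency bonuses found by map lookup.
; RollDie uses the sign of Advantage to select between random values for each die.
; A math expression flags a critical when the raw dice total equals the maximum possible.
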(fn Roll
  (params (Roller :type BP%20Game%20Character%20Object%20Reference) (StaticModifier :type Integer) (AmountD4 :type Integer) (AmountD6 :type Integer) (AmountD8 :type Integer) (AmountD10 :type Integer) (AmountD12 :type Integer) (AmountD20 :type Integer) (AmountD100 :type Integer) (StatModifiers :type Array%20of%20Enum_Stat%20Enums :default "NewEnumerator0") (ProficiencyModifiers :type Array%20of%20Enum_Proficiency%20Enums :default "NewEnumerator0") (Advantaje :type Integer))
  (Utilities|FlowControl|Sequence
    (:then_0
      (LocalVariables|SetTotalRoll (+ (LocalVariables|GetTotalRoll) StaticModifier)))
    (:then_1
      (bind _roll (CallFunction|RollDie 4 AmountD4 Advantaje))
      (bind _roll_2 (CallFunction|RollDie 6 AmountD6 Advantaje))
      (bind _roll_3 (CallFunction|RollDie 8 AmountD8 Advantaje))
      (bind _roll_4 (CallFunction|RollDie 10 AmountD10 Advantaje))
      (bind _roll_5 (CallFunction|RollDie 12 AmountD12 Advantaje))
      (bind _roll_6 (CallFunction|RollDie 20 AmountD20 Advantaje))
      (bind _roll_7 (CallFunction|RollDie 100 AmountD100 Advantaje))
      (bind _output_get (LocalVariables|SetTotalDiceResult (+ _roll _roll_2 _roll_3 _roll_4 _roll_5 _roll_6 _roll_7)))
      (LocalVariables|SetTotalRoll (+ _output_get (LocalVariables|GetTotalRoll)))
      (LocalVariables|SetCriticalRoll (|((((((((D4*4)+(D6*6))+(D8*8))+(D10*10))+(D12*12))+(D20*20))+(D100*100))==Roll) AmountD4 AmountD6 AmountD8 AmountD10 AmountD12 AmountD20 AmountD100 (+ _roll _roll_2 _roll_3 _roll_4 _roll_5 _roll_6 _roll_7))))
    (:then_2
      (for _array_element StatModifiers
        (if (.ReturnValue (Utilities|Map|Find (Variables|/Game/Actors/Characters/BP_GameCharacter.BP_GameCharacter_C|GetStats Roller) _array_element))
          (LocalVariables|SetTotalRoll (+ (Utilities|CalculateStatModifier (.Value (Utilities|Map|Find (Variables|/Game/Actors/Characters/BP_GameCharacter.BP_GameCharacter_C|GetStats Roller) _array_element))) (LocalVariables|GetTotalRoll))))))
    (:then_3
      (for _array_element_2 ProficiencyModifiers
        (if (.ReturnValue (Utilities|Map|Find (Variables|/Game/Actors/Characters/BP_GameCharacter.BP_GameCharacter_C|GetProficiencies Roller) _array_element_2))
          (LocalVariables|SetTotalRoll (+ (.Value (Utilities|Map|Find (Variables|/Game/Actors/Characters/BP_GameCharacter.BP_GameCharacter_C|GetProficiencies Roller) _array_element_2)) (LocalVariables|GetTotalRoll))))))
    (:then_4
      (return (LocalVariables|GetTotalRoll) (LocalVariables|GetTotalDiceResult) (LocalVariables|GetCriticalRoll)))))

(fn RollDie
  (params (NumberOfSides :type Integer) (NumberOfDices :type Integer) (Advantage :type Integer))
  (bind _returnvalue (Math|Random|RandomInteger NumberOfSides))
  (bind _returnvalue_2 (Math|Random|RandomInteger NumberOfSides))
  (bind _returnvalue_3 (+ _returnvalue 1))
  (bind _returnvalue_4 (+ _returnvalue_2 1))
  (for _index (range 1 NumberOfDices)
    (if (== Advantage 0)
      (LocalVariables|SetTotalRoll (+ (LocalVariables|GetTotalRoll) (+ (Math|Random|RandomInteger NumberOfSides) 1)))
      (else
        (LocalVariables|SetTotalRoll (+ (LocalVariables|GetTotalRoll) (Math|Integer|SelectInt _returnvalue_4 _returnvalue_3 (|(((A>B)&&(Adv>0))||((A<B)&&(Adv<0))) _returnvalue_4 _returnvalue_3 Advantage)))))))
  (return (LocalVariables|GetTotalRoll)))