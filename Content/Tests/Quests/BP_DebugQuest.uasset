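; BP_DebugQuest is a test quest with a "Go to the Inn" objective that grants the player experience as its reward.
; On accept, it binds to the GoTo event on the game instance's EventDispatchManager and advances the objective when the reported zone is "Test".
; On completion it unbinds from that event, and the reward step adds the experience to player 0's BP_PlayerCharacter.
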(event Custom|CheckGoTo
  (params (ZoneName :type Name))
  (if (== ZoneName "Test")
    (CallFunction|AdvanceObjetive)))

(event EventGiveRewards
  (bind _asbp_player_character (Utilities|Casting|CastToBP_PlayerCharacter (Game|GetPlayerCharacter (Variables|Default|GetWorld%20Context%20Object))))
  (Default|AddExp _asbp_player_character 200))

(event EventOnAccept
  (bind _asbp_game_instance (Utilities|Casting|CastToBP_GameInstance (Game|GetGameInstance (Variables|Default|GetWorld%20Context%20Object))))
  (EventDispatchers|BindEventtoGotoEvent (Variables|/Game/GameInstance/BP_GameInstance.BP_GameInstance_C|GetEventDispatchManager _asbp_game_instance) (delegate Custom|CheckGoTo)))

(event EventOnComplete
  (bind _asbp_game_instance (Utilities|Casting|CastToBP_GameInstance (Game|GetGameInstance (Variables|Default|GetWorld%20Context%20Object))))
  (EventDispatchers|UnbindEventfromGotoEvent (Variables|/Game/GameInstance/BP_GameInstance.BP_GameInstance_C|GetEventDispatchManager _asbp_game_instance) (delegate Custom|CheckGoTo)))

(fn GetObjetiveText
  (|CallParentFunction)
  (return "Go to the Inn"))