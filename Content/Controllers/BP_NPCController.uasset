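; AI controller for hostile NPCs in a turn-based RPG, handling their turns and player detection.
; MakeTurn restores resources, notifies passives, then ends the turn if stunned or runs the NPC's behavior tree, which EndTurn stops.
; Cast validates and fires actions at the player.
; Perception registers the NPC as an observer, notifies the player's passives and starts combat with its group unless already fighting or the player is stealthed.
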(event OnTargetPerceptionUpdated(AIPerception)
  (params (Actor :type Actor%20Object%20Reference) (Stimulus :type AI%20Stimulus%20Structure))
  (bind _asbp_player_character (Utilities|Casting|CastToBP_PlayerCharacter Actor))
  (CallFunction|PlayerDetected _asbp_player_character))

(event Custom|RestoreSeePlayer
  (bind _asbp_rol_game_mode (Utilities|Casting|CastToBP_RolGameMode (Game|GetGameMode)))
  (if (or (not (Variables|/Game/GameMode/BP_RolGameMode.BP_RolGameMode_C|GetisInCombat _asbp_rol_game_mode)) (Variables|Default|GethasTurn))
    (Variables|Default|SetSeesPlayer false)
    (bind _asbp_player_character (Utilities|Casting|CastToBP_PlayerCharacter (Game|GetPlayerCharacter 0)))
    (bind _asbp_hostile_npc (Utilities|Casting|CastToBP_HostileNPC (Pawn|GetControlledPawn)))
    (Utilities|Array|RemoveItem (Variables|/Game/Actors/Characters/BP_GameCharacter.BP_GameCharacter_C|GetObservers _asbp_player_character) _asbp_hostile_npc)))

(event Custom|Cast
  (params (Action :type BP%20Action%20Object%20Reference))
  (bind _asbp_game_character (Utilities|Casting|CastToBP_GameCharacter (Pawn|GetControlledPawn)))
  (bind _availability (Class|BPIUsable|CheckAvailability(Message) Action _asbp_game_character))
  (bind _asbp_player_character (Utilities|Casting|CastToBP_PlayerCharacter (Game|GetPlayerCharacter 0)))
  (bind _validtarget (Default|CheckTargetIsValid Action _asbp_game_character _asbp_player_character (Transformation|GetActorLocation _asbp_player_character)))
  (if (and _availability _validtarget)
    (Default|Cast Action _asbp_game_character _asbp_player_character (Transformation|GetActorLocation _asbp_player_character))))

(event Custom|PlayerDetected
  (params (PlayerCharacter :type BP%20Player%20Character%20Object%20Reference))
  (Variables|Default|SetAuxCharArray (Utilities|Array|MakeArray))
  (if (not (Variables|Default|GetSeesPlayer))
    (Variables|Default|SetSeesPlayer true)
    (bind _asbp_hostile_npc (Utilities|Casting|CastToBP_HostileNPC (Pawn|GetControlledPawn)))
    (Utilities|Array|Add (Variables|/Game/Actors/Characters/BP_GameCharacter.BP_GameCharacter_C|GetObservers PlayerCharacter) _asbp_hostile_npc)
    (bind _arrayelement (Utilities|Array|ReverseforEachLoop (Variables|/Game/Actors/Characters/BP_GameCharacter.BP_GameCharacter_C|GetPassives PlayerCharacter))
      (:LoopBody
        (bind _asbp_hostile_npc_2 (Utilities|Casting|CastToBP_HostileNPC (Pawn|GetControlledPawn)))
        (Class|BPIonSeenTrigger|OnSeen(Message) _arrayelement _asbp_hostile_npc_2 PlayerCharacter))
      (:Completed
        (bind _asbp_rol_game_mode (Utilities|Casting|CastToBP_RolGameMode (Game|GetGameMode)))
        (if (not (or (Variables|/Game/GameMode/BP_RolGameMode.BP_RolGameMode_C|GetisInCombat _asbp_rol_game_mode) (GameplayTags|HasTag (Variables|/Game/Actors/Characters/BP_GameCharacter.BP_GameCharacter_C|GetGameplayTags PlayerCharacter) "(TagName=\"Status.Stealth\")" true)))
          (bind _asbp_rol_game_mode_2 (Utilities|Casting|CastToBP_RolGameMode (Game|GetGameMode)))
          (bind _asbp_hostile_npc_3 (Utilities|Casting|CastToBP_HostileNPC (Pawn|GetControlledPawn)))
          (Utilities|Array|AppendArray (Variables|Default|GetAuxCharArray) (Variables|/Game/Actors/Characters/HostileCharacters/BP_HostileNPC.BP_HostileNPC_C|GetCombatGroup _asbp_hostile_npc_3))
          (Utilities|Array|Add (Variables|Default|GetAuxCharArray) PlayerCharacter)
          (Default|StartCombat _asbp_rol_game_mode_2 (Variables|Default|GetAuxCharArray)))))))

(event EventMakeTurn
  (Variables|Default|SethasTurn true)
  (Utilities|FlowControl|Delay 1.0)
  (bind _asbp_hostile_npc (Utilities|Casting|CastToBP_HostileNPC (Pawn|GetControlledPawn)))
  (Default|RestoreTurnResources _asbp_hostile_npc)
  (bind _arrayelement (Utilities|Array|ReverseforEachLoop (Variables|/Game/Actors/Characters/BP_GameCharacter.BP_GameCharacter_C|GetPassives _asbp_hostile_npc))
    (:LoopBody
      (Class|BPIonBeginningTurnTrigger|OnBegginingTurn(Message) _arrayelement _asbp_hostile_npc))
    (:Completed
      (if (GameplayTags|HasAnyTags (Variables|/Game/Actors/Characters/BP_GameCharacter.BP_GameCharacter_C|GetGameplayTags _asbp_hostile_npc) (GameplayTags|MakeLiteralGameplayTagContainer "(GameplayTags=((TagName=\"Status.Stunned\")))") true)
        (bind _asbp_rol_game_mode (Utilities|Casting|CastToBP_RolGameMode (Game|GetGameMode)))
        (Default|EndTurn _asbp_rol_game_mode)
        (else
          (AI|RunBehaviorTree (Variables|/Game/Actors/Characters/HostileCharacters/BP_HostileNPC.BP_HostileNPC_C|GetBehaviorTree _asbp_hostile_npc)))))))

(event EventEndTurn
  (Variables|Default|SethasTurn false)
  (AI|Logic|StopLogic (Variables|Default|GetBrainComponent) ""))

(fn ConstructionScript
  (bind _asbp_rol_game_mode (Utilities|Casting|CastToBP_RolGameMode (Game|GetGameMode)))
  (EventDispatchers|BindEventtoOnTurnChanged _asbp_rol_game_mode (EventDispatchers|CreateEvent :!event Custom|RestoreSeePlayer)))