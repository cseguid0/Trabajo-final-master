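; Base trap actor that can be hidden, spotted, triggered or disarmed, with an empty OnTrapTriggered event as the effect hook.
; Player overlap with the detection sphere runs a proficiency check against SpotDifficulty, revealing the mesh on success.
; Any game character entering the activation sphere fires the trigger unless disarmed.
; Construction restores disarmed and visible state from GameInstance TrapData by ActorGuid, and GetSaveData returns both flags.
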(event OnComponentBeginOverlap(DetectionSphere)
  (params (OverlappedComponent :type Primitive%20Component%20Object%20Reference) (OtherActor :type Actor%20Object%20Reference) (OtherComp :type Primitive%20Component%20Object%20Reference) (OtherBodyIndex :type Integer) (bFromSweep :type Boolean) (SweepResult :type Hit%20Result%20Structure%20%28by%20ref%29))
  (bind _asbp_player_character (Utilities|Casting|CastToBP_PlayerCharacter OtherActor))
  (bind _success (Utilities|ProficiencyCheck _asbp_player_character "NewEnumerator11" (Variables|Default|GetSpotDifficulty)))
  (if _success
    (CallFunction|Spot)))

(event OnComponentBeginOverlap(ActivationSphere)
  (params (OverlappedComponent :type Primitive%20Component%20Object%20Reference) (OtherActor :type Actor%20Object%20Reference) (OtherComp :type Primitive%20Component%20Object%20Reference) (OtherBodyIndex :type Integer) (bFromSweep :type Boolean) (SweepResult :type Hit%20Result%20Structure%20%28by%20ref%29))
  (if (not (Variables|Default|GetisDisarmed))
    (bind _asbp_game_character (Utilities|Casting|CastToBP_GameCharacter OtherActor))
    (CallFunction|OnTrapTriggered _asbp_game_character)))

(event Custom|OnTrapTriggered
  (params (Character :type BP%20Game%20Character%20Object%20Reference)))

(event Custom|Spot
  (Rendering|SetVisibility (Variables|Default|GetStaticMesh) true true)
  (Variables|Default|SetisVisible true))

(event EventBeginPlay)

(event Collision|EventActorBeginOverlap
  (params (OtherActor :type Actor%20Object%20Reference)))

(event EventTick
  (params (DeltaSeconds :type Float%20%28single-precision%29)))

(fn ConstructionScript
  (CallFunction|LoadData)
  (Components|Sphere|SetSphereRadius (Variables|Default|GetActivationSphere) (Variables|Default|GetActivationRadius) true)
  (Components|Sphere|SetSphereRadius (Variables|Default|GetDetectionSphere) (Variables|Default|GetDetectionRadius) true)
  (Rendering|SetVisibility (Variables|Default|GetStaticMesh) (Variables|Default|GetisVisible) true))

(fn LoadData
  (bind _asbp_game_instance (Utilities|Casting|CastToBP_GameInstance (Game|GetGameInstance)))
  (if (.ReturnValue (Utilities|Map|Find (Variables|/Game/GameInstance/BP_GameInstance.BP_GameInstance_C|GetTrapData _asbp_game_instance) (Variables|Default|GetActorGuid)))
    (Variables|Default|SetisDisarmed (.isDisarmed (Utilities|Struct|BreakST_TrapData (.Value (Utilities|Map|Find (Variables|/Game/GameInstance/BP_GameInstance.BP_GameInstance_C|GetTrapData _asbp_game_instance) (Variables|Default|GetActorGuid))))))
    (Variables|Default|SetisVisible (.isVisible (Utilities|Struct|BreakST_TrapData (.Value (Utilities|Map|Find (Variables|/Game/GameInstance/BP_GameInstance.BP_GameInstance_C|GetTrapData _asbp_game_instance) (Variables|Default|GetActorGuid))))))))

(fn GetSaveData
  (return (Utilities|Struct|MakeST_TrapData (Variables|Default|GetisDisarmed) (Variables|Default|GetisVisible))))