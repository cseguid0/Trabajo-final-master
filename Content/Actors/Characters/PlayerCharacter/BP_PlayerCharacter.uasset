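; Player character for an RPG with stats, archetypes, passives, equipment and inventory.
; LoadData restores state from the GameInstance's PlayerData, applying transform only for save-file loads, and GetSaveData packs it back.
; Rest refills HP and resources, clears shielding, consumes supplies and notifies passives in reverse.
; Passive changes refresh the character screen, a sphere hides overlapping actors until they exit, and zero HP after damage opens GameOver.
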(event OnComponentBeginOverlap(Sphere)
  (params (OverlappedComponent :type Primitive%20Component%20Object%20Reference) (OtherActor :type Actor%20Object%20Reference) (OtherComp :type Primitive%20Component%20Object%20Reference) (OtherBodyIndex :type Integer) (bFromSweep :type Boolean) (SweepResult :type Hit%20Result%20Structure%20%28by%20ref%29))
  (Rendering|SetActorHiddenInGame OtherActor true))

(event OnComponentEndOverlap(Sphere)
  (params (OverlappedComponent :type Primitive%20Component%20Object%20Reference) (OtherActor :type Actor%20Object%20Reference) (OtherComp :type Primitive%20Component%20Object%20Reference) (OtherBodyIndex :type Integer))
  (Rendering|SetActorHiddenInGame OtherActor false))

(event Custom|AddExp
  (params (Exp :type Integer))
  (Variables|CharacterAttributes|SetExp (+ Exp (Variables|CharacterAttributes|GetExp))))

(event Custom|Rest
  (Variables|Default|SetHP (Variables|Default|GetMaxHP))
  (Variables|Default|SetResources (Utilities|Map|MakeMap))
  (Variables|Default|SetShielded 0)
  (bind (_keypin _valuepin) (Utilities|Map|ForEachLoop(Map) (Variables|Default|GetMaxResources))
    (:then
      (Utilities|Map|Add (Variables|Default|GetResources) _keypin _valuepin))
    (:CompletedPin
      (Default|RemoveItem (Variables|Default|GetInventory) "/Game/Data/Items/Supply/DA_Supply.DA_Supply" 20)
      (bind _arrayelement (Utilities|Array|ReverseforEachLoop (Variables|Default|GetPassives))
        (:LoopBody
          (Class|BPIonRestTrigger|OnRest(Message) _arrayelement self))))))

(event Custom|AddMoney
  (params (Money :type Integer))
  (Variables|CharacterAttributes|SetMoney (+ Money (Variables|CharacterAttributes|GetMoney))))

(event EventBeginPlay
  (CallFunction|LoadData))

(event EventAddPassive
  (params (Passive :type BP%20Passive%20Object%20Reference))
  (|CallParentFunction Passive)
  (bind _asbp_player_controller (Utilities|Casting|CastToBP_PlayerController (Pawn|GetController)))
  (bind _asbp_player_hud (Utilities|Casting|CastToBP_PlayerHUD (HUD|GetHUD _asbp_player_controller)))
  (Utilities|IsValid (Variables|/Game/UI/PlayerHUD/BP_PlayerHUD.BP_PlayerHUD_C|GetCharacterScreen _asbp_player_hud)
    (:Is%20Valid
      (Default|UpdateUI (Variables|/Game/UI/PlayerHUD/BP_PlayerHUD.BP_PlayerHUD_C|GetCharacterScreen _asbp_player_hud)))))

(event EventRemovePassive
  (params (Passive :type BP%20Passive%20Object%20Reference))
  (|CallParentFunction Passive)
  (bind _asbp_player_controller (Utilities|Casting|CastToBP_PlayerController (Pawn|GetController)))
  (bind _asbp_player_hud (Utilities|Casting|CastToBP_PlayerHUD (HUD|GetHUD _asbp_player_controller)))
  (Utilities|IsValid (Variables|/Game/UI/PlayerHUD/BP_PlayerHUD.BP_PlayerHUD_C|GetCharacterScreen _asbp_player_hud)
    (:Is%20Valid
      (Default|UpdateUI (Variables|/Game/UI/PlayerHUD/BP_PlayerHUD.BP_PlayerHUD_C|GetCharacterScreen _asbp_player_hud)))))

(fn ConstructionScript
  (|CallParentFunction))

(fn LoadData
  (|CallParentFunction)
  (bind _asbp_game_instance (Utilities|Casting|CastToBP_GameInstance (Game|GetGameInstance)))
  (Variables|Default|SetMaxHP (.maxhp (Variables|/Game/GameInstance/BP_GameInstance.BP_GameInstance_C|GetPlayerData _asbp_game_instance)))
  (Variables|Default|SetHP (.hp (Variables|/Game/GameInstance/BP_GameInstance.BP_GameInstance_C|GetPlayerData _asbp_game_instance)))
  (Variables|Default|SetShielded (.shielded (Variables|/Game/GameInstance/BP_GameInstance.BP_GameInstance_C|GetPlayerData _asbp_game_instance)))
  (Variables|Default|SetAC (.ac (Variables|/Game/GameInstance/BP_GameInstance.BP_GameInstance_C|GetPlayerData _asbp_game_instance)))
  (Variables|Default|SetStats (.stats (Variables|/Game/GameInstance/BP_GameInstance.BP_GameInstance_C|GetPlayerData _asbp_game_instance)))
  (Variables|Default|SetProficiencies (.proficiencies (Variables|/Game/GameInstance/BP_GameInstance.BP_GameInstance_C|GetPlayerData _asbp_game_instance)))
  (Variables|Default|SetPassives (.passives (Variables|/Game/GameInstance/BP_GameInstance.BP_GameInstance_C|GetPlayerData _asbp_game_instance)))
  (Variables|Default|SetResources (.resources (Variables|/Game/GameInstance/BP_GameInstance.BP_GameInstance_C|GetPlayerData _asbp_game_instance)))
  (Variables|Default|SetArmorSlot (.armorslot (Variables|/Game/GameInstance/BP_GameInstance.BP_GameInstance_C|GetPlayerData _asbp_game_instance)))
  (Variables|Default|SetRightWeaponSlot (.rightweaponslot (Variables|/Game/GameInstance/BP_GameInstance.BP_GameInstance_C|GetPlayerData _asbp_game_instance)))
  (Variables|Default|SetLeftWeaponSlot (.leftweaponslot (Variables|/Game/GameInstance/BP_GameInstance.BP_GameInstance_C|GetPlayerData _asbp_game_instance)))
  (Variables|Default|SetRangedWeaponSlot (.rangedweaponslot (Variables|/Game/GameInstance/BP_GameInstance.BP_GameInstance_C|GetPlayerData _asbp_game_instance)))
  (Variables|Default|SetInteractionRange (.interactionrange (Variables|/Game/GameInstance/BP_GameInstance.BP_GameInstance_C|GetPlayerData _asbp_game_instance)))
  (Variables|Default|SetActions (.actions (Variables|/Game/GameInstance/BP_GameInstance.BP_GameInstance_C|GetPlayerData _asbp_game_instance)))
  (Variables|Default|SetMovement (.movement (Variables|/Game/GameInstance/BP_GameInstance.BP_GameInstance_C|GetPlayerData _asbp_game_instance)))
  (Variables|Default|SetMaxResources (.maxresources (Variables|/Game/GameInstance/BP_GameInstance.BP_GameInstance_C|GetPlayerData _asbp_game_instance)))
  (Variables|Default|SetRemainingMovement (.remainingmovement (Variables|/Game/GameInstance/BP_GameInstance.BP_GameInstance_C|GetPlayerData _asbp_game_instance)))
  (Variables|CharacterAttributes|SetExp (.exp (Variables|/Game/GameInstance/BP_GameInstance.BP_GameInstance_C|GetPlayerData _asbp_game_instance)))
  (Default|SetInventory (Variables|Default|GetInventory) (.inventory (Variables|/Game/GameInstance/BP_GameInstance.BP_GameInstance_C|GetPlayerData _asbp_game_instance)))
  (Variables|Default|SetLevel (.level (Variables|/Game/GameInstance/BP_GameInstance.BP_GameInstance_C|GetPlayerData _asbp_game_instance)))
  (Variables|CharacterAttributes|SetArchetypes (.archetypes (Variables|/Game/GameInstance/BP_GameInstance.BP_GameInstance_C|GetPlayerData _asbp_game_instance)))
  (Variables|CharacterAttributes|SetMoney (.money (Variables|/Game/GameInstance/BP_GameInstance.BP_GameInstance_C|GetPlayerData _asbp_game_instance)))
  (Variables|CharacterAttributes|SetSubarchetypes (.subarchetypes (Variables|/Game/GameInstance/BP_GameInstance.BP_GameInstance_C|GetPlayerData _asbp_game_instance)))
  (Variables|Default|SetPassivesData (.passivesdata (Variables|/Game/GameInstance/BP_GameInstance.BP_GameInstance_C|GetPlayerData _asbp_game_instance)))
  (Variables|Default|SetGameplayTags (.gameplaytags (Variables|/Game/GameInstance/BP_GameInstance.BP_GameInstance_C|GetPlayerData _asbp_game_instance)))
  (if (Variables|/Game/GameInstance/BP_GameInstance.BP_GameInstance_C|GetLoadingFromSaveFile _asbp_game_instance)
    (Transformation|SetActorTransform (.transform (Variables|/Game/GameInstance/BP_GameInstance.BP_GameInstance_C|GetPlayerData _asbp_game_instance)))))

(fn GetSaveData
  (return (Utilities|Struct|MakeST_PlayerData (Variables|Default|GetMaxHP) (Variables|Default|GetHP) (Variables|Default|GetShielded) (Variables|Default|GetAC) (Variables|Default|GetStats) (Variables|Default|GetProficiencies) (Variables|Default|GetPassives) (Variables|Default|GetResources) (Variables|Default|GetArmorSlot) (Variables|Default|GetRightWeaponSlot) (Variables|Default|GetLeftWeaponSlot) (Variables|Default|GetRangedWeaponSlot) (Variables|Default|GetInteractionRange) (Variables|Default|GetActions) (Variables|Default|GetMovement) (Variables|Default|GetMaxResources) (Variables|Default|GetRemainingMovement) (Variables|CharacterAttributes|GetExp) (Default|GetInventory (Variables|Default|GetInventory)) (Variables|Default|GetLevel) (Variables|CharacterAttributes|GetArchetypes) (Variables|CharacterAttributes|GetMoney) (Variables|CharacterAttributes|GetSubarchetypes) (Transformation|GetActorTransform) (Variables|Default|GetPassivesData) (Variables|Default|GetGameplayTags))))

(fn ReceiveDamagePrivate
  (params (Damage :type Integer) (Attack :type BP%20Action%20Object%20Reference) (AttackSource :type BP%20Game%20Character%20Object%20Reference))
  (|CallParentFunction Damage Attack AttackSource)
  (if (== (Variables|Default|GetHP) 0)
    (Game|OpenLevel(byName) "GameOver")))