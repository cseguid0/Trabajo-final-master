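; BP_BanditBoss is the bandit boss hostile character, a child Blueprint that inherits its behavior from its parent class.
; Its only active addition is a CheckDeath override that runs the parent check, then calls CallBanditBossKill on the GameInstance's EventDispatchManager.
; The override tests no death result itself, so that call follows every parent check whenever the BP_GameInstance cast succeeds.
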(event EventBeginPlay)

(event Collision|EventActorBeginOverlap
  (params (OtherActor :type Actor%20Object%20Reference))
  (|CallParentFunction OtherActor) ; This node is disabled and will not be called.\nDrag off pins to build functionality.
)

(event EventTick
  (params (DeltaSeconds :type Float%20%28single-precision%29))
  (|CallParentFunction DeltaSeconds) ; This node is disabled and will not be called.\nDrag off pins to build functionality.
)

(fn ConstructionScript
  (|CallParentFunction))

(fn CheckDeath
  (|CallParentFunction)
  (bind _asbp_game_instance (Utilities|Casting|CastToBP_GameInstance (Game|GetGameInstance)))
  (Default|CallBanditBossKill (Variables|/Game/GameInstance/BP_GameInstance.BP_GameInstance_C|GetEventDispatchManager _asbp_game_instance)))