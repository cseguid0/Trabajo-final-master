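; BP_GuardCaptain is the friendly Guard Captain character that the player can click to interact with.
; A click on its capsule asks BP_PlayerController to schedule an interaction with the captain.
; Its Interact event runs the parent behavior, then calls the SpeakWithTheCaptain event through the EventDispatchManager held by BP_GameInstance.
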(event OnClicked(CapsuleComponent)
  (params (TouchedComponent :type Primitive%20Component%20Object%20Reference) (ButtonPressed :type Key%20Structure :default "None"))
  (bind _asbp_player_controller (Utilities|Casting|CastToBP_PlayerController (Game|GetPlayerController 0)))
  (Default|ScheduleInteraction _asbp_player_controller self))

(event EventBeginPlay)

(event Collision|EventActorBeginOverlap
  (params (OtherActor :type Actor%20Object%20Reference)))

(event EventTick
  (params (DeltaSeconds :type Float%20%28single-precision%29)))

(event EventInteract
  (|CallParentFunction)
  (bind _asbp_game_instance (Utilities|Casting|CastToBP_GameInstance (Game|GetGameInstance)))
  (Default|CallSpeakwiththeCaptain (Variables|/Game/GameInstance/BP_GameInstance.BP_GameInstance_C|GetEventDispatchManager _asbp_game_instance)))

(fn ConstructionScript
  (|CallParentFunction))