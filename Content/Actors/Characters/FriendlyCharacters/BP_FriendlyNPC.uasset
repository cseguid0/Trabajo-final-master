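; Friendly NPC character that the player can talk to, with vendor storage and persistent state.
; Interacting opens a dialogue widget built from its DialogueTree, flags the player controller as interacting and switches the view target to the NPC.
; Stats, transform, vendor items, passives and tags are exposed for saving and restored from the GameInstance's NPC data by actor GUID.
; Range checks pass within either the player's or the NPC's interaction range.
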(event EventInteract
  (bind _returnvalue (Game|GetPlayerController 0))
  (bind _returnvalue_2 (UserInterface|CreateWidget "/Game/UI/DialogueWindow/UI_DialogueWindow.UI_DialogueWindow_C" 0 (Variables|Default|GetDialogueTree) self))
  (UserInterface|Viewport|AddtoViewport _returnvalue_2 0)
  (bind _asbp_player_controller (Utilities|Casting|CastToBP_PlayerController _returnvalue))
  (Variables|/Game/Controllers/BP_PlayerController.BP_PlayerController_C|SetisInteracting _asbp_player_controller true)
  (Game|Player|SetViewTargetwithBlend _returnvalue self 0.0 "VTBlend_Linear" 0.0 false))

(fn ConstructionScript
  (|CallParentFunction))

(fn GetSaveData
  (return (Utilities|Struct|MakeST_NPCData (Variables|Default|GetHP) (Variables|Default|GetShielded) (Variables|Default|GetRemainingMovement) (Variables|Default|GetResources) (Transformation|GetActorTransform) (Variables|Default|GetVendorStorage) (Variables|Default|GetPassivesData) (Variables|Default|GetGameplayTags))))

(fn LoadData
  (|CallParentFunction)
  (bind _asbp_game_instance (Utilities|Casting|CastToBP_GameInstance (Game|GetGameInstance)))
  (if (.ReturnValue (Utilities|Map|Find (Variables|/Game/GameInstance/BP_GameInstance.BP_GameInstance_C|GetNPCData _asbp_game_instance) (Variables|Default|GetActorGuid)))
    (Variables|Default|SetHP (.HP (Utilities|Struct|BreakST_NPCData (.Value (Utilities|Map|Find (Variables|/Game/GameInstance/BP_GameInstance.BP_GameInstance_C|GetNPCData _asbp_game_instance) (Variables|Default|GetActorGuid))))))
    (Variables|Default|SetShielded (.Shield (Utilities|Struct|BreakST_NPCData (.Value (Utilities|Map|Find (Variables|/Game/GameInstance/BP_GameInstance.BP_GameInstance_C|GetNPCData _asbp_game_instance) (Variables|Default|GetActorGuid))))))
    (Variables|Default|SetRemainingMovement (.RemainingMovement (Utilities|Struct|BreakST_NPCData (.Value (Utilities|Map|Find (Variables|/Game/GameInstance/BP_GameInstance.BP_GameInstance_C|GetNPCData _asbp_game_instance) (Variables|Default|GetActorGuid))))))
    (Variables|Default|SetResources (.Resources (Utilities|Struct|BreakST_NPCData (.Value (Utilities|Map|Find (Variables|/Game/GameInstance/BP_GameInstance.BP_GameInstance_C|GetNPCData _asbp_game_instance) (Variables|Default|GetActorGuid))))))
    (Transformation|SetActorTransform (.Transform (Utilities|Struct|BreakST_NPCData (.Value (Utilities|Map|Find (Variables|/Game/GameInstance/BP_GameInstance.BP_GameInstance_C|GetNPCData _asbp_game_instance) (Variables|Default|GetActorGuid))))))
    (Variables|Default|SetVendorStorage (.Items (Utilities|Struct|BreakST_NPCData (.Value (Utilities|Map|Find (Variables|/Game/GameInstance/BP_GameInstance.BP_GameInstance_C|GetNPCData _asbp_game_instance) (Variables|Default|GetActorGuid))))))
    (Variables|Default|SetPassivesData (.PassivesData (Utilities|Struct|BreakST_NPCData (.Value (Utilities|Map|Find (Variables|/Game/GameInstance/BP_GameInstance.BP_GameInstance_C|GetNPCData _asbp_game_instance) (Variables|Default|GetActorGuid))))))
    (Variables|Default|SetGameplayTags (.GameplayTags (Utilities|Struct|BreakST_NPCData (.Value (Utilities|Map|Find (Variables|/Game/GameInstance/BP_GameInstance.BP_GameInstance_C|GetNPCData _asbp_game_instance) (Variables|Default|GetActorGuid))))))))

(fn InPlayerRange
  (bind _returnvalue (Game|GetPlayerCharacter 0))
  (bind _self self)
  (bind _returnvalue_2 (Transformation|GetDistanceTo _returnvalue _self))
  (bind _asbp_player_character (Utilities|Casting|CastToBP_PlayerCharacter _returnvalue))
  (return (or (<= _returnvalue_2 (Variables|/Game/Actors/Characters/BP_GameCharacter.BP_GameCharacter_C|GetInteractionRange _asbp_player_character)) (<= _returnvalue_2 (Variables|Default|GetInteractionRange)))))