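; Hostile NPC character that starts ordered combat when it spots the player and yields experience and loot when killed.
; Pawn sensing passes its CombatGroup plus the player to BP_RolGameMode to start combat.
; At zero HP it leaves the combat order, awards XP, spawns a loot-filled corpse, hides itself and triggers a combat-end check.
; Its state saves and reloads by ID through BP_GameInstance, recreating the corpse if dead.
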(event OnSeePawn(PawnSensing)
  (params (Pawn :type Pawn%20Object%20Reference))
  (Variables|Default|SetAuxCharArray (Utilities|Array|MakeArray))
  (bind _asbp_player_character (Utilities|Casting|CastToBP_PlayerCharacter Pawn))
  (bind _asbp_rol_game_mode (Utilities|Casting|CastToBP_RolGameMode (Game|GetGameMode)))
  (Utilities|Array|AppendArray (Variables|Default|GetAuxCharArray) (Variables|Default|GetCombatGroup))
  (Utilities|Array|Add (Variables|Default|GetAuxCharArray) _asbp_player_character)
  (Default|StartCombat _asbp_rol_game_mode (Variables|Default|GetAuxCharArray)))

(event EventBeginPlay)

(event Collision|EventActorBeginOverlap
  (params (OtherActor :type Actor%20Object%20Reference)))

(event EventTick
  (params (DeltaSeconds :type Float%20%28single-precision%29)))

(event EventDamage
  (params (Damage :type Integer))
  (|CallParentFunction Damage)
  (if (== (Variables|Default|GetHP) 0)
    (bind _asbp_rol_game_mode (Utilities|Casting|CastToBP_RolGameMode (Game|GetGameMode)))
    (Default|RemovefromCombatOrder _asbp_rol_game_mode self)
    (bind _asbp_player_character (Utilities|Casting|CastToBP_PlayerCharacter (Game|GetPlayerCharacter 0)))
    (Default|AddExp _asbp_player_character (Variables|Default|GetExpLoot))
    (CallFunction|ToRecipient)
    (Default|CheckCombatEnd _asbp_rol_game_mode)))

(fn ConstructionScript
  (|CallParentFunction))

(fn LoadData
  (|CallParentFunction)
  (bind _asbp_game_instance (Utilities|Casting|CastToBP_GameInstance (Game|GetGameInstance)))
  (if (.isvalid (Utilities|Array|Get(acopy) (Variables|/Game/GameInstance/BP_GameInstance.BP_GameInstance_C|GetNPCData _asbp_game_instance) (Variables|Default|GetID)))
    (Variables|Default|SetHP (.hp (Utilities|Array|Get(acopy) (Variables|/Game/GameInstance/BP_GameInstance.BP_GameInstance_C|GetNPCData _asbp_game_instance) (Variables|Default|GetID))))
    (Variables|Default|SetRemainingMovement (.remainingmovement (Utilities|Array|Get(acopy) (Variables|/Game/GameInstance/BP_GameInstance.BP_GameInstance_C|GetNPCData _asbp_game_instance) (Variables|Default|GetID))))
    (Variables|Default|SetResources (.resources (Utilities|Array|Get(acopy) (Variables|/Game/GameInstance/BP_GameInstance.BP_GameInstance_C|GetNPCData _asbp_game_instance) (Variables|Default|GetID))))
    (Transformation|SetActorTransform (.transform (Utilities|Array|Get(acopy) (Variables|/Game/GameInstance/BP_GameInstance.BP_GameInstance_C|GetNPCData _asbp_game_instance) (Variables|Default|GetID))))
    (Variables|Default|SetLoot (.items (Utilities|Array|Get(acopy) (Variables|/Game/GameInstance/BP_GameInstance.BP_GameInstance_C|GetNPCData _asbp_game_instance) (Variables|Default|GetID))))
    (if (== (Variables|Default|GetHP) 0)
      (CallFunction|ToRecipient))))

(fn GetSaveData
  (return (Utilities|Struct|MakeST_NPCData (Variables|Default|GetHP) (Variables|Default|GetRemainingMovement) (Variables|Default|GetResources) (Transformation|GetActorTransform) (Variables|Default|GetLoot) true)))

(fn ToRecipient
  (bind _returnvalue (Game|SpawnActorfromClass "/Game/Actors/Recipients/BP_Corpse.BP_Corpse_C" (Transformation|GetActorTransform) "Undefined" "MultiplyWithRoot" 0 0))
  (Default|SetInventory (Variables|/Game/Actors/Recipients/BP_Recipient.BP_Recipient_C|GetInventory _returnvalue) (Variables|Default|GetLoot))
  (Rendering|SetActorHiddenInGame true))