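; Player character for an RPG with D&D-like stats, restored from player data held in BP_GameInstance.
; On BeginPlay, LoadPlayer passes combat stats, equipment slots and actions to LoadCharacter, then sets experience, inventory, money, level and archetypes itself.
; Damage runs the parent handling, then opens the GameOver level when HP equals zero.
; An AddExp event updates experience.
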(event Custom|AddExp
  (params (Exp :type Integer))
  (Variables|Default|SetExp (+ Exp (Variables|Default|GetExp))))

(event EventBeginPlay
  (bind _asbp_game_instance (Utilities|Casting|CastToBP_GameInstance (Game|GetGameInstance)))
  (CallFunction|LoadPlayer (Variables|/Game/GameInstance/BP_GameInstance.BP_GameInstance_C|GetPlayerData _asbp_game_instance)))

(event Collision|EventActorBeginOverlap
  (params (OtherActor :type Actor%20Object%20Reference)))

(event EventTick
  (params (DeltaSeconds :type Float%20%28single-precision%29)))

(event EventDamage
  (params (Damage :type Integer))
  (|CallParentFunction Damage)
  (if (== (Variables|Default|GetHP) 0)
    (Game|OpenLevel(byName) "GameOver")))

(fn ConstructionScript
  (|CallParentFunction))

(fn LoadPlayer
  (params (Data :type ST%20Player%20Data%20Structure))
  (CallFunction|LoadCharacter (Utilities|Struct|MakeST_CharacterData (.maxhp Data) (.hp Data) (.ac Data) (.stats Data) (.proficiencies Data) (.passives Data) (.maxresources Data) (.resources Data) (.armorslot Data) (.rightweaponslot Data) (.leftweaponslot Data) (.rangedweaponslot Data) (.actions Data) (.remainingmovement Data)))
  (Variables|Default|SetExp (.exp Data))
  (Variables|/Game/Actors/Components/BP_InventoryComponent.BP_InventoryComponent_C|SetInventory (Variables|Default|GetInventory) (.inventory Data))
  (Variables|Default|SetMoney (.money Data))
  (Variables|Default|SetLevel (.level Data))
  (Variables|Default|SetArchetypes (.archetypes Data))
  (Variables|Default|SetSubarchetypes (.subarchetypes Data)))