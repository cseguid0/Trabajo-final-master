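; Base character for turn-based RPG combat, handling passives, stealth, equipment slots, initiative, turn resources, shields and HP.
; Passives react to equipment changes and modify damage and healing through interface-driven flat and factor modifiers.
; Incoming attacks and damage scan reaction passives in reverse, pausing on a confirmation widget for players and auto-casting otherwise.
; A capsule sized from interaction range triggers opportunity attacks when the turn-holding character leaves it during combat.
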(event OnComponentEndOverlap(ReactionAttackChecker)
  (params (OverlappedComponent :type Primitive%20Component%20Object%20Reference) (OtherActor :type Actor%20Object%20Reference) (OtherComp :type Primitive%20Component%20Object%20Reference) (OtherBodyIndex :type Integer))
  (bind _asbp_game_character (Utilities|Casting|CastToBP_GameCharacter OtherActor))
  (bind _asbp_rol_game_mode (Utilities|Casting|CastToBP_RolGameMode (Game|GetGameMode)))
  (bind _asbp_player_controller (Utilities|Casting|CastToBP_PlayerController (Pawn|GetController _asbp_game_character))
    (:then
      (if (and (Variables|/Game/GameMode/BP_RolGameMode.BP_RolGameMode_C|GetisInCombat _asbp_rol_game_mode) (Variables|/Game/Controllers/BP_PlayerController.BP_PlayerController_C|GethasTurn _asbp_player_controller))
        (CallFunction|DoOpportunityAttack _asbp_game_character)))
    (:CastFailed
      (bind _asbp_npccontroller (Utilities|Casting|CastToBP_NPCController (Pawn|GetController _asbp_game_character)))
      (if (and (Variables|/Game/GameMode/BP_RolGameMode.BP_RolGameMode_C|GetisInCombat _asbp_rol_game_mode) (Variables|/Game/Controllers/BP_NPCController.BP_NPCController_C|GethasTurn _asbp_npccontroller))
        (CallFunction|DoOpportunityAttack _asbp_game_character)))))

(event Custom|ReceiveShield
  (params (Shield :type Integer))
  (Variables|CharacterAttributes|SetShielded (+ Shield (Variables|CharacterAttributes|GetShielded))))

(event Custom|ReceiveDamage
  (params (Damage :type Integer) (Attack :type BP%20Action%20Object%20Reference) (AttackSource :type BP%20Game%20Character%20Object%20Reference))
  (bind _passives (Variables|CharacterAttributes|GetPassives))
  (Variables|Default|SetDamage Damage)
  (Variables|Default|SetAttack%20Type Attack)
  (Variables|Default|SetAttack%20Source AttackSource)
  (Variables|Default|SetReceiveDamageIndex (Utilities|Array|Length _passives))
  (bind (_array_index _array_element) (Utilities|ReverseforEachLoopwithBreak _passives :!label _label)
    (:Loop%20Body
      (if (== _array_index (- (Variables|Default|GetReceiveDamageIndex) 1))
        (bind _asbp_reaction_passive (Utilities|Casting|CastToBP_ReactionPassive _array_element)
          (:then
            (bind _trigger (Class|BPIonDamageAttackReactionTrigger|OnBeforeDamageReaction(Message) _asbp_reaction_passive self (Variables|Default|GetAttack%20Type)))
            (if (and _trigger (Utilities|DoesObjectImplementInterface _asbp_reaction_passive "/Game/Data/Effects/BPI_OnDamageAttackReactionTrigger.BPI_OnDamageAttackReactionTrigger_C"))
              (Utilities|Casting|CastToBP_PlayerController (Pawn|GetController)
                (:then
                  (bind _returnvalue (UserInterface|CreateWidget "/Game/UI/ReactionConfirmationWindow/UI_ReactionConfirmationWindow.UI_ReactionConfirmationWindow_C" 0 (Variables|/Game/Data/Effects/BP_ReactionPassive.BP_ReactionPassive_C|GetReaction _asbp_reaction_passive) self (Variables|Default|GetAttack%20Source)))
                  (EventDispatchers|BindEventtoOnContinuation _returnvalue (delegate Custom|ContinueReceiveDamage))
                  (UserInterface|Viewport|AddtoViewport _returnvalue 0)
                  (goto _label Break))
                (:CastFailed
                  (Default|Cast (Variables|/Game/Data/Effects/BP_ReactionPassive.BP_ReactionPassive_C|GetReaction _asbp_reaction_passive) self (Variables|Default|GetAttack%20Source) "0, 0, 0")))
              (else
                (Variables|Default|SetReceiveDamageIndex (- (Variables|Default|GetReceiveDamageIndex) 1) :!label _label_2))))
          (:CastFailed
            (goto _label_2)))))
    (:Conplete
      (if (== (Variables|Default|GetReceiveDamageIndex) 0)
        (CallFunction|ReceiveDamagePrivate (Variables|Default|GetDamage) (Variables|Default|GetAttack%20Type) (Variables|Default|GetAttack%20Source))))))

(event Custom|ContinueReceiveDamage
  (bind _attack_source (Variables|Default|GetAttack%20Source))
  (Variables|Default|SetReceiveDamageIndex (- (Variables|Default|GetReceiveDamageIndex) 1))
  (bind (_array_index _array_element) (Utilities|ReverseforEachLoopwithBreak (Variables|CharacterAttributes|GetPassives) :!label _label)
    (:Loop%20Body
      (if (== _array_index (- (Variables|Default|GetReceiveDamageIndex) 1))
        (bind _asbp_reaction_passive (Utilities|Casting|CastToBP_ReactionPassive _array_element)
          (:then
            (bind _trigger (Class|BPIonDamageAttackReactionTrigger|OnBeforeDamageReaction(Message) _asbp_reaction_passive self (Variables|Default|GetAttack%20Type)))
            (if (and _trigger (Utilities|DoesObjectImplementInterface _asbp_reaction_passive "/Game/Data/Effects/BPI_OnDamageAttackReactionTrigger.BPI_OnDamageAttackReactionTrigger_C"))
              (Utilities|Casting|CastToBP_PlayerController (Pawn|GetController)
                (:then
                  (bind _returnvalue (UserInterface|CreateWidget "/Game/UI/ReactionConfirmationWindow/UI_ReactionConfirmationWindow.UI_ReactionConfirmationWindow_C" 0 (Variables|/Game/Data/Effects/BP_ReactionPassive.BP_ReactionPassive_C|GetReaction _asbp_reaction_passive) self _attack_source))
                  (EventDispatchers|BindEventtoOnContinuation _returnvalue (delegate Custom|ContinueReceiveDamage))
                  (UserInterface|Viewport|AddtoViewport _returnvalue 0)
                  (goto _label Break))
                (:CastFailed
                  (Default|Cast (Variables|/Game/Data/Effects/BP_ReactionPassive.BP_ReactionPassive_C|GetReaction _asbp_reaction_passive) self _attack_source "0, 0, 0")))
              (else
                (Variables|Default|SetReceiveDamageIndex (- (Variables|Default|GetReceiveDamageIndex) 1) :!label _label_2))))
          (:CastFailed
            (goto _label_2)))))
    (:Conplete
      (if (== (Variables|Default|GetReceiveDamageIndex) 0)
        (CallFunction|ReceiveDamagePrivate (Variables|Default|GetDamage) (Variables|Default|GetAttack%20Type) (Variables|Default|GetAttack%20Source))))))

(event Custom|OnReceiveAttackReaction
  (params (Source%20Character :type BP%20Game%20Character%20Object%20Reference) (Attack :type BP%20Action%20Object%20Reference))
  (bind _self self)
  (bind _passives (Variables|CharacterAttributes|GetPassives))
  (Variables|Default|SetReceivedAttackSourceCharacter Source%20Character)
  (Variables|Default|SetReceivedAttack Attack)
  (Variables|Default|SetReceiveAttackIndex (Utilities|Array|Length _passives))
  (bind (_array_index _array_element) (Utilities|ReverseforEachLoopwithBreak _passives :!label _label)
    (:Loop%20Body
      (if (== _array_index (- (Variables|Default|GetReceiveAttackIndex) 1))
        (bind _asbp_reaction_passive (Utilities|Casting|CastToBP_ReactionPassive _array_element)
          (:then
            (bind _trigger (Class|BPIonReceiveAttackReactionTrigger|OnBeforeAttackReaction(Message) _asbp_reaction_passive self (Variables|Default|GetReceivedAttack)))
            (if (and _trigger (Utilities|DoesObjectImplementInterface _asbp_reaction_passive "/Game/Data/Effects/BPI_OnReceiveAttackReactionTrigger.BPI_OnReceiveAttackReactionTrigger_C"))
              (Utilities|Casting|CastToBP_PlayerController (Pawn|GetController)
                (:then
                  (bind _returnvalue (UserInterface|CreateWidget "/Game/UI/ReactionConfirmationWindow/UI_ReactionConfirmationWindow.UI_ReactionConfirmationWindow_C" 0 (Variables|/Game/Data/Effects/BP_ReactionPassive.BP_ReactionPassive_C|GetReaction _asbp_reaction_passive) _self (Variables|Default|GetReceivedAttackSourceCharacter)))
                  (EventDispatchers|BindEventtoOnContinuation _returnvalue (delegate Custom|ContinueReceiveAttackReaction))
                  (UserInterface|Viewport|AddtoViewport _returnvalue 0)
                  (goto _label Break))
                (:CastFailed
                  (Default|Cast (Variables|/Game/Data/Effects/BP_ReactionPassive.BP_ReactionPassive_C|GetReaction _asbp_reaction_passive) _self (Variables|Default|GetReceivedAttackSourceCharacter) "0, 0, 0")))
              (else
                (Variables|Default|SetReceiveAttackIndex (- (Variables|Default|GetReceiveAttackIndex) 1) :!label _label_2))))
          (:CastFailed
            (goto _label_2)))))
    (:Conplete
      (if (== (Variables|Default|GetReceiveAttackIndex) 0)
        (Default|ContinueCast (Variables|Default|GetReceivedAttack) (Variables|Default|GetReceivedAttackSourceCharacter) self "0, 0, 0")))))

(event Custom|AddPassive
  (params (Passive :type BP%20Passive%20Object%20Reference))
  (bind _passives (Variables|CharacterAttributes|GetPassives))
  (if (Utilities|Array|ContainsItem _passives Passive)
    (CallFunction|RemovePassive Passive))
  (Utilities|Array|Add _passives Passive)
  (Class|BPIonAddedTrigger|OnAdded(Message) Passive self))

(event Custom|RemovePassive
  (params (Passive :type BP%20Passive%20Object%20Reference))
  (bind _returnvalue (Utilities|Array|RemoveItem (Variables|CharacterAttributes|GetPassives) Passive))
  (if _returnvalue
    (Class|BPIonRemovedTrigger|OnRemoved(Message) Passive self)))

(event Custom|ContinueReceiveAttackReaction
  (bind _self self)
  (bind _receivedattacksourcecharacter (Variables|Default|GetReceivedAttackSourceCharacter))
  (Variables|Default|SetReceiveAttackIndex (- (Variables|Default|GetReceiveAttackIndex) 1))
  (bind (_array_index _array_element) (Utilities|ReverseforEachLoopwithBreak (Variables|CharacterAttributes|GetPassives) :!label _label)
    (:Loop%20Body
      (if (== _array_index (- (Variables|Default|GetReceiveAttackIndex) 1))
        (bind _asbp_reaction_passive (Utilities|Casting|CastToBP_ReactionPassive _array_element)
          (:then
            (bind _trigger (Class|BPIonReceiveAttackReactionTrigger|OnBeforeAttackReaction(Message) _asbp_reaction_passive self (Variables|Default|GetReceivedAttack)))
            (if (and _trigger (Utilities|DoesObjectImplementInterface _asbp_reaction_passive "/Game/Data/Effects/BPI_OnReceiveAttackReactionTrigger.BPI_OnReceiveAttackReactionTrigger_C"))
              (Utilities|Casting|CastToBP_PlayerController (Pawn|GetController)
                (:then
                  (bind _returnvalue (UserInterface|CreateWidget "/Game/UI/ReactionConfirmationWindow/UI_ReactionConfirmationWindow.UI_ReactionConfirmationWindow_C" 0 (Variables|/Game/Data/Effects/BP_ReactionPassive.BP_ReactionPassive_C|GetReaction _asbp_reaction_passive) _self _receivedattacksourcecharacter))
                  (EventDispatchers|BindEventtoOnContinuation _returnvalue (delegate Custom|ContinueReceiveAttackReaction))
                  (UserInterface|Viewport|AddtoViewport _returnvalue 0)
                  (goto _label Break))
                (:CastFailed
                  (Default|Cast (Variables|/Game/Data/Effects/BP_ReactionPassive.BP_ReactionPassive_C|GetReaction _asbp_reaction_passive) _self _receivedattacksourcecharacter "0, 0, 0")))
              (else
                (Variables|Default|SetReceiveAttackIndex (- (Variables|Default|GetReceiveAttackIndex) 1) :!label _label_2))))
          (:CastFailed
            (goto _label_2)))))
    (:Conplete
      (if (== (Variables|Default|GetReceiveAttackIndex) 0)
        (Default|ContinueCast (Variables|Default|GetReceivedAttack) (Variables|Default|GetReceivedAttackSourceCharacter) self "0, 0, 0")))))

(event Custom|ToggleStealth
  (if (GameplayTags|HasTag (Variables|CharacterAttributes|GetGameplayTags) "(TagName=\"Status.Stealth\")" true)
    (CallFunction|LoseStealth)
    (else
      (CallFunction|GainStealth))))

(event Custom|GainStealth
  (CallFunction|AddPassive "/Game/Data/Effects/Stealth/DA_Stealth.DA_Stealth"))

(event Custom|LoseStealth
  (CallFunction|RemovePassive "/Game/Data/Effects/Stealth/DA_Stealth.DA_Stealth"))

(event EventHighlight
  (Rendering|Material|SetOverlayMaterial (Variables|Character|GetMesh) "/Game/Media/Materials/Outlines/MatIns_Outline.MatIns_Outline" :!class /Script/Engine.MeshComponent))

(event EventUnhighlight
  (Rendering|Material|SetOverlayMaterial (Variables|Character|GetMesh) 0 :!class /Script/Engine.MeshComponent))

(fn ConstructionScript
  (CallFunction|LoadData)
  (Components|Capsule|SetCapsuleRadius (Variables|Default|GetReactionAttackChecker) (+ (Variables|CharacterAttributes|GetInteractionRange) 5e+01) true))

(fn EquipArmor
  (params (Armor :type BP%20Armor%20Object%20Reference))
  (bind _equipedarmor (CallFunction|RemoveArmor))
  (bind _output_get (Variables|CharacterAttributes|SetArmorSlot Armor))
  (Default|OnEquip _output_get self)
  (CallFunction|OnEquipPassiveTrigger Armor)
  (return _equipedarmor))

(fn RemoveArmor
  (Utilities|IsValid (Variables|CharacterAttributes|GetArmorSlot)
    (:Is%20Valid
      (bind _output_get (LocalVariables|SetAux (Variables|CharacterAttributes|GetArmorSlot)))
      (Default|OnRemove _output_get self)
      (Variables|CharacterAttributes|SetArmorSlot 0)
      (CallFunction|OnRemoveEquipmentPassiveTrigger (LocalVariables|GetAux))
      (return (LocalVariables|GetAux)))
    (:Is%20Not%20Valid
      (return 0))))

(fn EquipLeftHand
  (params (Weapon :type BP%20One%20Handed%20Object%20Reference))
  (bind _equipedweapon (CallFunction|RemoveLeftHand))
  (bind _output_get (Variables|CharacterAttributes|SetLeftWeaponSlot Weapon))
  (Default|OnEquip _output_get self)
  (CallFunction|OnEquipPassiveTrigger Weapon)
  (return _equipedweapon))

(fn RemoveLeftHand
  (Utilities|IsValid (Variables|CharacterAttributes|GetLeftWeaponSlot)
    (:Is%20Valid
      (bind _output_get (LocalVariables|SetAux (Variables|CharacterAttributes|GetLeftWeaponSlot)))
      (Default|OnRemove _output_get self)
      (Variables|CharacterAttributes|SetLeftWeaponSlot 0)
      (CallFunction|OnRemoveEquipmentPassiveTrigger (LocalVariables|GetAux))
      (return (LocalVariables|GetAux)))
    (:Is%20Not%20Valid
      (return 0))))

(fn EquipRightHand
  (params (Weapon :type BP%20Melee%20Weapon%20Object%20Reference))
  (bind _equipedweapon (CallFunction|RemoveRightHand))
  (bind _output_get (Variables|CharacterAttributes|SetRightWeaponSlot Weapon))
  (Default|OnEquip _output_get self)
  (CallFunction|OnEquipPassiveTrigger Weapon)
  (return _equipedweapon))

(fn RemoveRightHand
  (Utilities|IsValid (Variables|CharacterAttributes|GetRightWeaponSlot)
    (:Is%20Valid
      (bind _output_get (LocalVariables|SetAux (Variables|CharacterAttributes|GetRightWeaponSlot)))
      (Default|OnRemove _output_get self)
      (Variables|CharacterAttributes|SetRightWeaponSlot 0)
      (CallFunction|OnRemoveEquipmentPassiveTrigger (LocalVariables|GetAux))
      (return (LocalVariables|GetAux)))
    (:Is%20Not%20Valid
      (return 0))))

(fn EquipRanged
  (params (Weapon :type BP%20Ranged%20Weapon%20Object%20Reference))
  (bind _equipedweapon (CallFunction|RemoveRanged))
  (bind _output_get (Variables|CharacterAttributes|SetRangedWeaponSlot Weapon))
  (Default|OnEquip _output_get self)
  (CallFunction|OnEquipPassiveTrigger Weapon)
  (return _equipedweapon))

(fn RemoveRanged
  (Utilities|IsValid (Variables|CharacterAttributes|GetRangedWeaponSlot)
    (:Is%20Valid
      (bind _output_get (LocalVariables|SetAux (Variables|CharacterAttributes|GetRangedWeaponSlot)))
      (Default|OnRemove _output_get self)
      (Variables|CharacterAttributes|SetRangedWeaponSlot 0)
      (CallFunction|OnRemoveEquipmentPassiveTrigger (LocalVariables|GetAux))
      (return (LocalVariables|GetAux)))
    (:Is%20Not%20Valid
      (return 0))))

(fn RollInitiative
  (bind _roll (Default|Roll (LocalVariables|GetDice) self 0 0 0 0 0 0 1 0 (Utilities|Array|MakeArray "NewEnumerator1") "NewEnumerator0"))
  (return _roll))

(fn RestoreTurnResources
  (Utilities|Map|Add (Variables|CharacterAttributes|GetResources) "NewEnumerator0" (.Value (Utilities|Map|Find (Variables|CharacterAttributes|GetMaxResources) "NewEnumerator0")))
  (Utilities|Map|Add (Variables|CharacterAttributes|GetResources) "NewEnumerator1" (.Value (Utilities|Map|Find (Variables|CharacterAttributes|GetMaxResources) "NewEnumerator1")))
  (Utilities|Map|Add (Variables|CharacterAttributes|GetResources) "NewEnumerator2" (.Value (Utilities|Map|Find (Variables|CharacterAttributes|GetMaxResources) "NewEnumerator2")))
  (Variables|CharacterAttributes|SetRemainingMovement (Variables|CharacterAttributes|GetMovement)))

(fn LoadData)

(fn ReceiveDamagePrivate
  (params (Damage :type Integer) (Attack :type BP%20Action%20Object%20Reference) (AttackSource :type BP%20Game%20Character%20Object%20Reference))
  (LocalVariables|SetTotalDamage Damage)
  (bind _arrayelement (Utilities|Array|ReverseforEachLoop (Variables|BP_GameCharacter_C|GetPassives AttackSource))
    (:LoopBody
      (if (Utilities|DoesObjectImplementInterface _arrayelement "/Game/Data/Effects/BPI_OnDealingDamageTrigger.BPI_OnDealingDamageTrigger_C")
        (bind (_plaindamagemodifier _factordmamagemodifier) (Class|BPIonDealingDamageTrigger|OnDealingDamage(Message) _arrayelement AttackSource (LocalVariables|GetTotalDamage) Attack))
        (LocalVariables|SetDamageModifier _plaindamagemodifier)
        (LocalVariables|SetDamageFactor _factordmamagemodifier)))
    (:Completed
      (bind _arrayelement_2 (Utilities|Array|ReverseforEachLoop (Variables|CharacterAttributes|GetPassives))
        (:LoopBody
          (if (Utilities|DoesObjectImplementInterface _arrayelement_2 "/Game/Data/Effects/BPI_OnReceivingDamageTrigger.BPI_OnReceivingDamageTrigger_C")
            (bind (_plaindamagemodifier_2 _factordamagemodifier) (Class|BPIonReceivingDamageTrigger|OnReceivingDamage(Message) _arrayelement_2 (LocalVariables|GetTotalDamage) self (Variables|/Game/Data/Actions/BP_Action.BP_Action_C|GetClassification Attack)))
            (LocalVariables|SetDamageModifier (+ _plaindamagemodifier_2 (LocalVariables|GetDamageModifier)))
            (LocalVariables|SetDamageFactor (* _factordamagemodifier (LocalVariables|GetDamageFactor)))))
        (:Completed
          (Variables|CharacterAttributes|SetHP (Math|Integer|Clamp(Integer) (- (Variables|CharacterAttributes|GetHP) (Math|Integer|Max(Integer) (- (Math|Float|Round (* (Math|Integer|Max(Integer) (+ (LocalVariables|GetTotalDamage) (LocalVariables|GetDamageModifier))) (LocalVariables|GetDamageFactor))) (Variables|CharacterAttributes|GetShielded)))) 0 (Variables|CharacterAttributes|GetMaxHP)))
          (Variables|CharacterAttributes|SetShielded (Math|Integer|Max(Integer) 0 (- (Variables|CharacterAttributes|GetShielded) (Math|Float|Round (* (Math|Integer|Max(Integer) (+ (LocalVariables|GetTotalDamage) (LocalVariables|GetDamageModifier))) (LocalVariables|GetDamageFactor)))))))))))

(fn ReceiveHealing
  (params (Heal :type Integer))
  (LocalVariables|SetTotalHealing Heal)
  (bind _arrayelement (Utilities|Array|ReverseforEachLoop (Variables|CharacterAttributes|GetPassives))
    (:LoopBody
      (if (Utilities|DoesObjectImplementInterface _arrayelement "/Game/Data/Effects/BPI_OnReceivingHealTrigger.BPI_OnReceivingHealTrigger_C")
        (bind (_plain_heal_modifier _factor_heal_modifier) (Class|BPIonReceivingHealTrigger|OnReceivingHeal(Message) _arrayelement (LocalVariables|GetTotalHealing) self))
        (LocalVariables|SetHealingModifier (+ _plain_heal_modifier (LocalVariables|GetHealingModifier)))
        (LocalVariables|SetHealingFactor (* _factor_heal_modifier (LocalVariables|GetHealingFactor)))))
    (:Completed
      (Variables|CharacterAttributes|SetHP (Math|Integer|Clamp(Integer) (+ (Variables|CharacterAttributes|GetHP) (Math|Float|Round (* (+ (LocalVariables|GetTotalHealing) (LocalVariables|GetHealingModifier)) (LocalVariables|GetHealingFactor)))) 0 (Variables|CharacterAttributes|GetMaxHP))))))

(fn DoOpportunityAttack
  (params (Target :type BP%20Game%20Character%20Object%20Reference))
  (bind _canafford (Default|CanAfford (LocalVariables|GetOpportunityAttack) self))
  (if (and _canafford (not (GameplayTags|HasAnyTags (Variables|BP_GameCharacter_C|GetGameplayTags Target) (Utilities|Struct|MakeGameplayTagContainer (Utilities|Array|MakeArray "(TagName=\"Ignore.OpportunityAttack\")")) true)))
    (Default|Cast (LocalVariables|GetOpportunityAttack) self Target "0, 0, 0")))

(fn OnEquipPassiveTrigger
  (params (Equipment :type BP%20Equipable%20Item%20Object%20Reference))
  (bind _arrayelement (Utilities|Array|ReverseforEachLoop (Variables|CharacterAttributes|GetPassives))
    (:LoopBody
      (Class|BPIonEquipTrigger|OnEquip(Message) _arrayelement self Equipment))))

(fn OnRemoveEquipmentPassiveTrigger
  (params (Equipment :type BP%20Equipable%20Item%20Object%20Reference))
  (bind _arrayelement (Utilities|Array|ReverseforEachLoop (Variables|CharacterAttributes|GetPassives))
    (:LoopBody
      (Class|BPIonRemoveEquipmentTrigger|OnRemoveEquipment(Message) _arrayelement self Equipment))))