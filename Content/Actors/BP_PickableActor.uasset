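; World pickup actor holding an item stack that the player clicks to collect into their inventory.
; On BeginPlay it async-loads the item's mesh, and clicking that mesh has the player controller schedule an interaction.
; Interact adds units one at a time until an add fails, keeping the remainder and destroying the actor when none are left.
; It also exposes a player range check and save data of item and transform.
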(event OnClicked(StaticMesh)
  (params (TouchedComponent :type Primitive%20Component%20Object%20Reference) (ButtonPressed :type Key%20Structure))
  (bind _asbp_player_controller (Utilities|Casting|CastToBP_PlayerController (Game|GetPlayerController 0)))
  (Default|ScheduleInteraction _asbp_player_controller self))

(event EventBeginPlay
  (bind _object (Utilities|AsyncLoadAsset (Variables|/Game/Data/Items/BP_Item.BP_Item_C|GetMesh (.item (Variables|Default|GetItem))))
    (:Completed
      (bind _asstatic_mesh (Utilities|Casting|CastToStaticMesh _object))
      (Components|StaticMesh|SetStaticMesh (Variables|Default|GetStaticMesh) _asstatic_mesh))))

(event Collision|EventActorBeginOverlap
  (params (OtherActor :type Actor%20Object%20Reference)))

(event EventTick
  (params (DeltaSeconds :type Float%20%28single-precision%29)))

(event EventInteract
  (Utilities|FlowControl|ForLoopwithBreak 1 (.amount (Variables|Default|GetItem)) :!label _label
    (:LoopBody
      (bind _asbp_player_character (Utilities|Casting|CastToBP_PlayerCharacter (Game|GetPlayerCharacter 0)))
      (bind _added (Default|AddItem (Variables|/Game/Actors/Characters/BP_PlayerCharacter.BP_PlayerCharacter_C|GetInventory _asbp_player_character) (.item (Variables|Default|GetItem))))
      (if _added
        (Variables|Default|SetItem (Utilities|Struct|MakeST_ItemStack (.item (Variables|Default|GetItem)) (- (.amount (Variables|Default|GetItem)) 1)))
        (else
          (goto _label Break))))
    (:Completed
      (if (== (.amount (Variables|Default|GetItem)) 0)
        (Actor|DestroyActor)))))

(fn ConstructionScript)

(fn GetSaveData
  (return (Utilities|Struct|MakeST_PickableItemData (Variables|Default|GetItem) (Transformation|GetActorTransform))))

(fn InPlayerRange
  (bind _asbp_player_character (Utilities|Casting|CastToBP_PlayerCharacter (Game|GetPlayerCharacter 0)))
  (return (>= (Variables|/Game/Actors/Characters/BP_GameCharacter.BP_GameCharacter_C|GetInteractionRange _asbp_player_character) (Math|Vector|Distance(Vector) (Transformation|GetActorLocation _asbp_player_character) (Transformation|GetActorLocation)))))