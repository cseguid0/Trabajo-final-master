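; BP_Container is a recipient actor that holds loot in an Inventory and persists its contents through the game instance.
; GetSaveData returns the current inventory as the container's save data.
; LoadData runs from the Construction Script, looks up the actor's GUID in BP_GameInstance's RecipientData map, and restores the stored Loot into the Inventory when an entry exists.
; The event graph holds only disabled default events.
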(event EventBeginPlay
  (|CallParentFunction) ; This node is disabled and will not be called.\nDrag off pins to build functionality.
)

(event Collision|EventActorBeginOverlap
  (params (OtherActor :type Actor%20Object%20Reference))
  (|CallParentFunction OtherActor) ; This node is disabled and will not be called.\nDrag off pins to build functionality.
)

(event EventTick
  (params (DeltaSeconds :type Float%20%28single-precision%29))
  (|CallParentFunction DeltaSeconds) ; This node is disabled and will not be called.\nDrag off pins to build functionality.
)

(fn ConstructionScript
  (|CallParentFunction)
  (CallFunction|LoadData))

(fn GetSaveData
  (return (Utilities|Struct|MakeST_RecipientData (Default|GetInventory (Variables|Default|GetInventory)))))

(fn LoadData
  (bind _asbp_game_instance (Utilities|Casting|CastToBP_GameInstance (Game|GetGameInstance)))
  (if (.ReturnValue (Utilities|Map|Find (Variables|/Game/GameInstance/BP_GameInstance.BP_GameInstance_C|GetRecipientData _asbp_game_instance) (Variables|Default|GetActorGuid)))
    (Default|SetInventory (Variables|Default|GetInventory) (Utilities|Struct|BreakST_RecipientData (.Value (Utilities|Map|Find (Variables|/Game/GameInstance/BP_GameInstance.BP_GameInstance_C|GetRecipientData _asbp_game_instance) (Variables|Default|GetActorGuid)))))))