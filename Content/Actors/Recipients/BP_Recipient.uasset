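; BP_Recipient is a clickable loot container that shows a loot UI when interacted with while open.
; Clicking its Sphere asks BP_PlayerController to schedule an interaction, and Interact creates a UI_Loot widget owned by the container if IsOpen is set.
; Any end overlap on Sphere1 closes that widget.
; InPlayerRange reports whether the player is within the character's InteractionRange.
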(event OnClicked(Sphere)
  (params (TouchedComponent :type Primitive%20Component%20Object%20Reference) (ButtonPressed :type Key%20Structure :default "None"))
  (bind _asbp_player_controller (Utilities|Casting|CastToBP_PlayerController (Game|GetPlayerController 0)))
  (Default|ScheduleInteraction _asbp_player_controller self))

(event OnComponentEndOverlap(Sphere1)
  (params (OverlappedComponent :type Primitive%20Component%20Object%20Reference) (OtherActor :type Actor%20Object%20Reference) (OtherComp :type Primitive%20Component%20Object%20Reference) (OtherBodyIndex :type Integer))
  (bind _lootui (Variables|Default|GetLootUI))
  (Utilities|IsValid _lootui
    (:Is%20Valid
      (Default|Close _lootui))))

(event EventBeginPlay)

(event Collision|EventActorBeginOverlap
  (params (OtherActor :type Actor%20Object%20Reference)))

(event EventTick
  (params (DeltaSeconds :type Float%20%28single-precision%29)))

(event EventInteract
  (if (Variables|Default|GetisOpen)
    (bind _returnvalue (UserInterface|CreateWidget "/Game/UI/Loot/UI_Loot.UI_Loot_C" 0 self))
    (bind _output_get (Variables|Default|SetLootUI _returnvalue))
    (UserInterface|Viewport|AddtoViewport _output_get 0)))

(fn ConstructionScript)

(fn InPlayerRange
  (bind _returnvalue (Game|GetPlayerCharacter 0))
  (bind _asbp_player_character (Utilities|Casting|CastToBP_PlayerCharacter _returnvalue))
  (return (>= (Variables|/Game/Actors/Characters/BP_GameCharacter.BP_GameCharacter_C|GetInteractionRange _asbp_player_character) (Transformation|GetDistanceTo _returnvalue self))))