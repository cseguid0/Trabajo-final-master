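; Clickable door actor that saves the game and moves the player to another map at a given spawn point.
; Clicking its Cube waits a frame, then asks the player controller to schedule an interaction with the door.
; Interact fires a GoTo event for the map name on the GameInstance's event dispatch manager, then calls SaveAndLoadMap.
; InPlayerRange reports whether the player character is within a short distance of the door.
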(event OnClicked(Cube)
  (params (TouchedComponent :type Primitive%20Component%20Object%20Reference) (ButtonPressed :type Key%20Structure :default "None"))
  (Utilities|FlowControl|DelayUntilNextFrame)
  (bind _asbp_player_controller (Utilities|Casting|CastToBP_PlayerController (Game|GetPlayerController 0)))
  (Default|ScheduleInteraction _asbp_player_controller self))

(event EventBeginPlay)

(event Collision|EventActorBeginOverlap
  (params (OtherActor :type Actor%20Object%20Reference)))

(event EventTick
  (params (DeltaSeconds :type Float%20%28single-precision%29)))

(event EventInteract
  (bind _mapname (Variables|Default|GetMapName))
  (bind _asbp_game_instance (Utilities|Casting|CastToBP_GameInstance (Game|GetGameInstance)))
  (Default|CallGotoEvent (Variables|/Game/GameInstance/BP_GameInstance.BP_GameInstance_C|GetEventDispatchManager _asbp_game_instance) _mapname)
  (Default|SaveandLoadMap _asbp_game_instance _mapname (Variables|Default|GetSpawnPoint)))

(fn ConstructionScript)

(fn InPlayerRange
  (return (<= (Math|Vector|Distance(Vector) (Transformation|GetActorLocation (Game|GetPlayerCharacter 0)) (Transformation|GetActorLocation)) 1e+02)))