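; BP_InventoryComp is an inventory component storing slots of item and amount pairs, with getters, setters and counting.
; AddItem fills a partial stack or empty slot, then refreshes UI_Character grids.
; AddItemStack records candidate slots first and writes only when the remainder reaches exactly zero.
; RemoveItem drains slots matching hard-coded DA_Supply, ignoring its Item input, and updates the HUD's character screen.
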(event EventBeginPlay)

(event EventTick
  (params (DeltaSeconds :type Float%20%28single-precision%29)))

(fn AddItem
  (params (Item :type BP%20Item%20Object%20Reference))
  (LocalVariables|SetItemREF Item)
  (bind (_array_element _array_index) (Utilities|Array|ForEachLoopwithBreak (Variables|Default|GetInventory) :!label _label)
    (:LoopBody
      (LocalVariables|SetIndex _array_index)
      (if (> (.amount _array_element) 0)
        (if (and (== (.item _array_element) (LocalVariables|GetItemREF)) (< (.amount _array_element) (Variables|/Game/Data/Items/BP_Item.BP_Item_C|GetMaxAmount (.item _array_element))))
          (LocalVariables|SetFound true)
          (goto _label Break))))
    (:Completed
      (if (LocalVariables|GetFound)
        (Utilities|Array|SetArrayElem (Variables|Default|GetInventory) (LocalVariables|GetIndex) (Utilities|Struct|MakeST_ItemStack (.item (Utilities|Array|Get(acopy) (Variables|Default|GetInventory) (LocalVariables|GetIndex))) (+ (.amount (Utilities|Array|Get(acopy) (Variables|Default|GetInventory) (LocalVariables|GetIndex))) 1)))
        (bind _foundwidgets (Widget|GetAllWidgetsOfClass "/Game/UI/CharacterScreen/UI_Character.UI_Character_C" true))
        (for _array_element_2 _foundwidgets
          (Default|SetGrid _array_element_2))
        (return true)
        (else
          (bind (_array_element_3 _array_index_2) (Utilities|Array|ForEachLoopwithBreak (Variables|Default|GetInventory) :!label _label_2)
            (:LoopBody
              (LocalVariables|SetIndex _array_index_2)
              (if (== (.amount _array_element_3) 0)
                (LocalVariables|SetFound true)
                (goto _label_2 Break)))
            (:Completed
              (if (LocalVariables|GetFound)
                (Utilities|Array|SetArrayElem (Variables|Default|GetInventory) (LocalVariables|GetIndex) (Utilities|Struct|MakeST_ItemStack (LocalVariables|GetItemREF) 1))
                (bind _foundwidgets_2 (Widget|GetAllWidgetsOfClass "/Game/UI/CharacterScreen/UI_Character.UI_Character_C" true))
                (for _array_element_4 _foundwidgets_2
                  (Default|SetGrid _array_element_4))
                (return true)
                (else
                  (return false))))))))))

(fn SetInventory
  (params (Inventory :type Array%20of%20ST%20Item%20Stack%20Structures))
  (Variables|Default|SetInventory Inventory))

(fn GetInventory
  (return (Variables|Default|GetInventory)))

(fn RemoveItem
  (params (Item :type BP%20Item%20Object%20Reference) (Amount :type Integer))
  (bind _inventory (Variables|Default|GetInventory))
  (bind _index (LocalVariables|GetIndex))
  (bind _output (Utilities|Array|Get(acopy) _inventory _index))
  (LocalVariables|SetItemREF Item)
  (bind _output_get (LocalVariables|SetAmountREF Amount))
  (while (and (> _output_get 0) (< (LocalVariables|GetIndex) (Utilities|Array|Length (Variables|Default|GetInventory))))
    (if (== (.item _output) "/Game/Data/Items/Supply/DA_Supply.DA_Supply")
      (if (> (.amount _output) (LocalVariables|GetAmountREF))
        (Utilities|Array|SetArrayElem (Variables|Default|GetInventory) (LocalVariables|GetIndex) (Utilities|Struct|MakeST_ItemStack (.item _output) (- (.amount _output) (LocalVariables|GetAmountREF))))
        (LocalVariables|SetAmountREF 0)
        (else
          (LocalVariables|SetAmountREF (- (LocalVariables|GetAmountREF) (.amount _output)))
          (Utilities|Array|SetArrayElem (Variables|Default|GetInventory) (LocalVariables|GetIndex) (Utilities|Struct|MakeST_ItemStack 0 0)))))
    (Math|Integer|IncrementInt (LocalVariables|GetIndex)))
  (bind _asbp_player_hud (Utilities|Casting|CastToBP_PlayerHUD (HUD|GetHUD (Game|GetPlayerController 0))))
  (Utilities|IsValid (Variables|/Game/UI/PlayerHUD/BP_PlayerHUD.BP_PlayerHUD_C|GetCharacterScreen _asbp_player_hud)
    (:Is%20Valid
      (Default|UpdateUI (Variables|/Game/UI/PlayerHUD/BP_PlayerHUD.BP_PlayerHUD_C|GetCharacterScreen _asbp_player_hud))
      (return (- Amount (LocalVariables|GetAmountREF))))))

(fn CountItem
  (params (Item :type BP%20Item%20Object%20Reference))
  (for _array_element (Variables|Default|GetInventory)
    (if (== (.item _array_element) Item)
      (LocalVariables|SetTotal (+ (.amount _array_element) (LocalVariables|GetTotal)))))
  (return (LocalVariables|GetTotal)))

(fn AddItemStack
  (params (Items :type ST%20Item%20Stack%20Structure))
  (LocalVariables|SetItemREF (.item Items))
  (LocalVariables|SetAmountREF (.amount Items))
  (bind (_array_element _array_index) (Utilities|Array|ForEachLoopwithBreak (Variables|Default|GetInventory) :!label _label)
    (:LoopBody
      (Utilities|IsValid (.item _array_element)
        (:Is%20Valid
          (if (|(((amount<maxAmount)&&(itemInSlot==item))||(amount==0)) (.item _array_element) (.amount _array_element) (Variables|/Game/Data/Items/BP_Item.BP_Item_C|GetMaxAmount (.item _array_element)) (LocalVariables|GetItemREF))
            (Utilities|Array|Add (LocalVariables|GetIndexToAdd) _array_index :!label _label_2)
            (Utilities|Array|Add (LocalVariables|GetAmountToIndex) (- (Variables|/Game/Data/Items/BP_Item.BP_Item_C|GetMaxAmount (LocalVariables|GetItemREF)) (.amount _array_element)))
            (bind _output_get (LocalVariables|SetAmountREF (- (LocalVariables|GetAmountREF) (- (Variables|/Game/Data/Items/BP_Item.BP_Item_C|GetMaxAmount (LocalVariables|GetItemREF)) (.amount _array_element)))))
            (if (== _output_get 0)
              (LocalVariables|SetFoundAll true)
              (goto _label Break))))
        (:Is%20Not%20Valid
          (goto _label_2))))
    (:Completed
      (if (LocalVariables|GetFoundAll)
        (for (_array_element_2 _array_index_2) (LocalVariables|GetIndexToAdd)
          (Utilities|Array|SetArrayElem (Variables|Default|GetInventory) _array_element_2 (Utilities|Struct|MakeST_ItemStack (LocalVariables|GetItemREF) (+ (.amount (Utilities|Array|Get(acopy) (Variables|Default|GetInventory) _array_element_2)) (Utilities|Array|Get(acopy) (LocalVariables|GetAmountToIndex) _array_index_2)))))
        (return true)
        (else
          (return false))))))