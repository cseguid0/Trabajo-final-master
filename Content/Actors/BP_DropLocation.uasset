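; BP_DropLocation is a temporary interaction target marking where the player drops an item from the inventory or an equipment slot.
; On BeginPlay it walks the player toward itself and schedules an interaction with the player controller, with a range check for reach.
; Interact removes the item by source and spawns a BP_PickableActor at its location, then refreshes the character screen.
; Cancelling the interaction also refreshes that screen and destroys the actor.
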(event EventBeginPlay
  (bind _self self)
  (bind _asbp_player_controller (Utilities|Casting|CastToBP_PlayerController (Game|GetPlayerController 0)))
  (AI|Navigation|SimpleMovetoActor _asbp_player_controller _self)
  (Default|ScheduleInteraction _asbp_player_controller _self))

(event Collision|EventActorBeginOverlap
  (params (OtherActor :type Actor%20Object%20Reference)))

(event EventTick
  (params (DeltaSeconds :type Float%20%28single-precision%29)))

(event EventOnInteractionCancelled
  (bind _asbp_player_hud (Utilities|Casting|CastToBP_PlayerHUD (HUD|GetHUD (Game|GetPlayerController 0))))
  (Utilities|IsValid (Variables|/Game/UI/PlayerHUD/BP_PlayerHUD.BP_PlayerHUD_C|GetCharacterScreen _asbp_player_hud)
    (:Is%20Valid
      (Default|UpdateUI (Variables|/Game/UI/PlayerHUD/BP_PlayerHUD.BP_PlayerHUD_C|GetCharacterScreen _asbp_player_hud))
      (Actor|DestroyActor))))

(event EventInteract
  (bind _asbp_player_character (Utilities|Casting|CastToBP_PlayerCharacter (Game|GetPlayerCharacter 0)))
  (switch Utilities|FlowControl|Switch|SwitchonEnum_InventorySlotType (Variables|Default|GetItemSource)
    (:NewEnumerator0
      (if (> (.amount (Utilities|Array|Get(acopy) (Variables|/Game/Actors/Components/BP_InventoryComp.BP_InventoryComp_C|GetInventory (Variables|/Game/Actors/Characters/PlayerCharacter/BP_PlayerCharacter.BP_PlayerCharacter_C|GetInventory _asbp_player_character)) (Variables|Default|GetSlotNumber))) 0)
        (Game|SpawnActorfromClass "/Game/Actors/BP_PickableActor.BP_PickableActor_C" (Math|Transform|MakeTransform (Transformation|GetActorLocation) "0, 0, 0" "1.000000,1.000000,1.000000") "Undefined" "MultiplyWithRoot" 0 (Utilities|Struct|MakeST_ItemStack (.item (Utilities|Array|Get(acopy) (Variables|/Game/Actors/Components/BP_InventoryComp.BP_InventoryComp_C|GetInventory (Variables|/Game/Actors/Characters/PlayerCharacter/BP_PlayerCharacter.BP_PlayerCharacter_C|GetInventory _asbp_player_character)) (Variables|Default|GetSlotNumber))) (.amount (Utilities|Array|Get(acopy) (Variables|/Game/Actors/Components/BP_InventoryComp.BP_InventoryComp_C|GetInventory (Variables|/Game/Actors/Characters/PlayerCharacter/BP_PlayerCharacter.BP_PlayerCharacter_C|GetInventory _asbp_player_character)) (Variables|Default|GetSlotNumber)))) 0)
        (Utilities|Array|SetArrayElem (Variables|/Game/Actors/Components/BP_InventoryComp.BP_InventoryComp_C|GetInventory (Variables|/Game/Actors/Characters/PlayerCharacter/BP_PlayerCharacter.BP_PlayerCharacter_C|GetInventory _asbp_player_character)) (Variables|Default|GetSlotNumber) (Utilities|Struct|MakeST_ItemStack 0 0))
        (bind _asbp_player_hud (Utilities|Casting|CastToBP_PlayerHUD (HUD|GetHUD (Game|GetPlayerController 0)) :!label _label))
        (Utilities|IsValid (Variables|/Game/UI/PlayerHUD/BP_PlayerHUD.BP_PlayerHUD_C|GetCharacterScreen _asbp_player_hud)
          (:Is%20Valid
            (Default|UpdateUI (Variables|/Game/UI/PlayerHUD/BP_PlayerHUD.BP_PlayerHUD_C|GetCharacterScreen _asbp_player_hud))))))
    (:NewEnumerator1
      (bind _equipedarmor (Default|RemoveArmor _asbp_player_character))
      (Game|SpawnActorfromClass "/Game/Actors/BP_PickableActor.BP_PickableActor_C" (Math|Transform|MakeTransform (Transformation|GetActorLocation) "0, 0, 0" "1.000000,1.000000,1.000000") "Undefined" "MultiplyWithRoot" 0 (Utilities|Struct|MakeST_ItemStack _equipedarmor 1) 0)
      (goto _label))
    (:NewEnumerator2
      (bind _equipedweapon (Default|RemoveRightHand _asbp_player_character))
      (Game|SpawnActorfromClass "/Game/Actors/BP_PickableActor.BP_PickableActor_C" (Math|Transform|MakeTransform (Transformation|GetActorLocation) "0, 0, 0" "1.000000,1.000000,1.000000") "Undefined" "MultiplyWithRoot" 0 (Utilities|Struct|MakeST_ItemStack _equipedweapon 1) 0)
      (goto _label))
    (:NewEnumerator3
      (bind _equipedweapon_2 (Default|RemoveLeftHand _asbp_player_character))
      (Game|SpawnActorfromClass "/Game/Actors/BP_PickableActor.BP_PickableActor_C" (Math|Transform|MakeTransform (Transformation|GetActorLocation) "0, 0, 0" "1.000000,1.000000,1.000000") "Undefined" "MultiplyWithRoot" 0 (Utilities|Struct|MakeST_ItemStack _equipedweapon_2 1) 0)
      (goto _label))
    (:NewEnumerator4
      (bind _equipedweapon_3 (Default|RemoveRanged _asbp_player_character))
      (Game|SpawnActorfromClass "/Game/Actors/BP_PickableActor.BP_PickableActor_C" (Math|Transform|MakeTransform (Transformation|GetActorLocation) "0, 0, 0" "1.000000,1.000000,1.000000") "Undefined" "MultiplyWithRoot" 0 (Utilities|Struct|MakeST_ItemStack _equipedweapon_3 1) 0)
      (goto _label))))

(fn ConstructionScript)

(fn InPlayerRange
  (bind _asbp_player_character (Utilities|Casting|CastToBP_PlayerCharacter (Game|GetPlayerCharacter 0)))
  (return (or (>= (Variables|/Game/Actors/Characters/BP_GameCharacter.BP_GameCharacter_C|GetInteractionRange _asbp_player_character) (Math|Vector|Distance(Vector) (Transformation|GetActorLocation _asbp_player_character) (Transformation|GetActorLocation))) (< (Math|Vector|Distance(Vector) (Transformation|GetActorLocation _asbp_player_character) (Transformation|GetActorLocation)) (Variables|Default|GetInteractRange)))))