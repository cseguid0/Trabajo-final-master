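; BP_Chest is a loot container actor whose inventory and opened state can be saved and restored.
; GetSaveData exposes both values, and LoadData restores them from the BP_GameInstance ContainerData map, keyed by ActorGuid.
; LoadData runs from the Construction Script rather than BeginPlay.
; Highlight and Unhighlight events set and clear an outline overlay material on the mesh.
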(event EventBeginPlay
  (|CallParentFunction) ; This node is disabled and will not be called.\nDrag off pins to build functionality.
)

(event Collision|EventActorBeginOverlap
  (params (OtherActor :type Actor%20Object%20Reference))
  (|CallParentFunction OtherActor) ; This node is disabled and will not be called.\nDrag off pins to build functionality.
)

(event EventTick
  (params (DeltaSeconds :type Float%20%28single-precision%29))
  (|CallParentFunction DeltaSeconds) ; This node is disabled and will not be called.\nDrag off pins to build functionality.
)

(event EventHighlight
  (Rendering|Material|SetOverlayMaterial (Variables|Character|GetMesh) "/Game/Media/Materials/Outlines/MatIns_Outline.MatIns_Outline" :!class /Script/Engine.MeshComponent))

(event EventUnhighlight
  (Rendering|Material|SetOverlayMaterial (Variables|Character|GetMesh) 0 :!class /Script/Engine.MeshComponent))

(fn ConstructionScript
  (|CallParentFunction)
  (CallFunction|LoadData))

(fn GetSaveData
  (return (Utilities|Struct|MakeST_ContainerData (Default|GetInventory (Variables|Default|GetInventory)) (Variables|Default|GetisOpen))))

(fn LoadData
  (bind _asbp_game_instance (Utilities|Casting|CastToBP_GameInstance (Game|GetGameInstance)))
  (if (.ReturnValue (Utilities|Map|Find (Variables|/Game/GameInstance/BP_GameInstance.BP_GameInstance_C|GetContainerData _asbp_game_instance) (Variables|Default|GetActorGuid)))
    (Default|SetInventory (Variables|Default|GetInventory) (.Loot (Utilities|Struct|BreakST_ContainerData (.Value (Utilities|Map|Find (Variables|/Game/GameInstance/BP_GameInstance.BP_GameInstance_C|GetContainerData _asbp_game_instance) (Variables|Default|GetActorGuid))))))
    (Variables|Default|SetisOpen (.isOpened (Utilities|Struct|BreakST_ContainerData (.Value (Utilities|Map|Find (Variables|/Game/GameInstance/BP_GameInstance.BP_GameInstance_C|GetContainerData _asbp_game_instance) (Variables|Default|GetActorGuid))))))))