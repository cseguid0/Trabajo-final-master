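; Secret chest actor that stays hidden in game until every key in its Keys array is open.
; The construction script sets the initial visibility from IsOpen.
; The KeyInteracted event recomputes IsOpen as the AND of every key's IsOpen, then shows or hides the chest to match.
; An empty Keys array counts as open when that event runs.
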(event Custom|KeyInteracted
  (Variables|Default|SetisOpen true)
  (for _array_element (Variables|Default|GetKeys)
    (Variables|Default|SetisOpen (and (Variables|/Game/Actors/Containers/BP_Container.BP_Container_C|GetisOpen _array_element) (Variables|Default|GetisOpen))))
  (Rendering|SetActorHiddenInGame (not (Variables|Default|GetisOpen))))

(event EventBeginPlay
  (|CallParentFunction) ; This node is disabled and will not be called.\nDrag off pins to build functionality.
)

(event Collision|EventActorBeginOverlap
  (params (OtherActor :type Actor%20Object%20Reference))
  (|CallParentFunction OtherActor) ; This node is disabled and will not be called.\nDrag off pins to build functionality.
)

(event EventTick
  (params (DeltaSeconds :type Float%20%28single-precision%29))
  (|CallParentFunction DeltaSeconds) ; This node is disabled and will not be called.\nDrag off pins to build functionality.
)

(fn ConstructionScript
  (|CallParentFunction)
  (Rendering|SetActorHiddenInGame (not (Variables|Default|GetisOpen))))