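; BP_SecretChestKey is an interactable key actor tied to a secret chest, which also hands out the puzzle quest.
; On its first Interact it sets IsOpen, notifies the linked SecretChest through KeyInteracted, then calls GiveQuest.
; GiveQuest scans the game instance's QuestData and, unless a BP_SolveThePuzzleQuest in one of two particular statuses exists, constructs one and passes it to AcceptQuest.
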(event EventBeginPlay
  (|CallParentFunction) ; This node is disabled and will not be called.\nDrag off pins to build functionality.
)

(event Collision|EventActorBeginOverlap
  (params (OtherActor :type Actor%20Object%20Reference))
  (|CallParentFunction OtherActor) ; This node is disabled and will not be called.\nDrag off pins to build functionality.
)

(event EventTick
  (params (DeltaSeconds :type Float%20%28single-precision%29))
  (|CallParentFunction DeltaSeconds) ; This node is disabled and will not be called.\nDrag off pins to build functionality.
)

(event EventInteract
  (if (not (Variables|Default|GetisOpen))
    (Variables|Default|SetisOpen true)
    (Default|KeyInteracted (Variables|Default|GetSecretChest))
    (CallFunction|GiveQuest)))

(fn ConstructionScript
  (|CallParentFunction))

(fn GiveQuest
  (bind _returnvalue (Game|GetGameInstance))
  (bind _asbp_game_instance (Utilities|Casting|CastToBP_GameInstance _returnvalue))
  (LocalVariables|SetFoundQuest false)
  (bind _array_element (Utilities|Array|ForEachLoopwithBreak (Variables|/Game/GameInstance/BP_GameInstance.BP_GameInstance_C|GetQuestData _asbp_game_instance) :!label _label)
    (:LoopBody
      (if (and (Class|GameplayStatics|ObjectIsA _array_element "/Game/Data/Quests/SecondaryQuests/SolveThePuzzle/BP_SolveThePuzzleQuest.BP_SolveThePuzzleQuest_C") (or (Utilities|Enum|Equal(Enum) (Variables|/Game/Data/Quests/BP_Quest.BP_Quest_C|GetStatus _array_element) "NewEnumerator1") (Utilities|Enum|Equal(Enum) (Variables|/Game/Data/Quests/BP_Quest.BP_Quest_C|GetStatus _array_element) "NewEnumerator2")))
        (LocalVariables|SetFoundQuest true)
        (goto _label Break)))
    (:Completed
      (if (not (LocalVariables|GetFoundQuest))
        (bind _returnvalue_2 (Game|ConstructObjectfromClass "/Game/Data/Quests/SecondaryQuests/SolveThePuzzle/BP_SolveThePuzzleQuest.BP_SolveThePuzzleQuest_C" _returnvalue))
        (Default|AcceptQuest _asbp_game_instance _returnvalue_2)))))