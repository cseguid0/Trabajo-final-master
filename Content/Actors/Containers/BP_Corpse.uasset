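; BP_Corpse is a corpse actor, filed among the game's containers, whose appearance comes from a CorpseMesh variable.
; The construction script calls the parent's, assigns CorpseMesh to the Mesh component, and applies a world scale only if that assignment returns true.
; The event graph holds only disabled default events, so this Blueprint adds no runtime logic of its own.
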(event EventBeginPlay
  (|CallParentFunction) ; This node is disabled and will not be called.\nDrag off pins to build functionality.
)

(event Collision|EventActorBeginOverlap
  (params (OtherActor :type Actor%20Object%20Reference))
  (|CallParentFunction OtherActor) ; This node is disabled and will not be called.\nDrag off pins to build functionality.
)

(event EventTick
  (params (DeltaSeconds :type Float%20%28single-precision%29))
  (|CallParentFunction DeltaSeconds) ; This node is disabled and will not be called.\nDrag off pins to build functionality.
)

(fn ConstructionScript
  (|CallParentFunction)
  (bind _returnvalue (Components|StaticMesh|SetStaticMesh (Variables|Character|GetMesh) (Variables|Settings|GetCorpseMesh)))
  (if _returnvalue
    (Transformation|SetWorldScale3D (Variables|Character|GetMesh) (Variables|Settings|GetNew%20Scale))))