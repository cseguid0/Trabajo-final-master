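; BP_BuriedChest is a chest actor that stays hidden in game until the player detects it.
; The construction script hides the actor unless IsOpen is set.
; When a BP_PlayerCharacter overlaps Sphere2, it rolls a single-d20 ability check with a stat and a proficiency modifier.
; A successful check sets IsOpen and reveals the chest.
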(event OnComponentBeginOverlap(Sphere2)
  (params (OverlappedComponent :type Primitive%20Component%20Object%20Reference) (OtherActor :type Actor%20Object%20Reference) (OtherComp :type Primitive%20Component%20Object%20Reference) (OtherBodyIndex :type Integer) (bFromSweep :type Boolean) (SweepResult :type Hit%20Result%20Structure%20%28by%20ref%29))
  (bind _asbp_player_character (Utilities|Casting|CastToBP_PlayerCharacter OtherActor))
  (bind _success (Utilities|AbilityCheck _asbp_player_character 0 0 0 0 0 0 1 0 (Utilities|Array|MakeArray "NewEnumerator4") (Utilities|Array|MakeArray "NewEnumerator11") 0 1))
  (if _success
    (Variables|Default|SetisOpen _success)
    (Rendering|SetActorHiddenInGame false)))

(event EventBeginPlay
  (|CallParentFunction) ; This node is disabled and will not be called.\nDrag off pins to build functionality.
)

(event Collision|EventActorBeginOverlap
  (params (OtherActor :type Actor%20Object%20Reference))
  (|CallParentFunction OtherActor) ; This node is disabled and will not be called.\nDrag off pins to build functionality.
)

(event EventTick
  (params (DeltaSeconds :type Float%20%28single-precision%29))
  (|CallParentFunction DeltaSeconds) ; This node is disabled and will not be called.\nDrag off pins to build functionality.
)

(fn ConstructionScript
  (|CallParentFunction)
  (Rendering|SetActorHiddenInGame (not (Variables|Default|GetisOpen))))