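; Base weapon Blueprint for a d20-style dice system, providing attack rolls and formatted description text.
; RollAttack rolls one d20 with the stat modifier from GetStatMod and optional advantage, returning total, dice result and critical.
; GetDescription fills DescriptionFormat with the attack formula, built from the character's stat value, and the damage text.
; RollDamage, GetDamageDescription and GetStatMod are stubs, apparently meant for child weapons to override.
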(fn RollDamage
  (params (Character :type BP%20Game%20Character%20Object%20Reference) (Critical :type Boolean))
  (return 0))

(fn RollAttack
  (params (Character :type BP%20Game%20Character%20Object%20Reference) (Advantage :type Integer))
  (bind (_roll _diceresult _critical) (Default|Roll (Utilities|GetDice) Character 0 0 0 0 0 0 1 0 (Utilities|Array|MakeArray (CallFunction|GetStatMod Character)) "NewEnumerator0" Advantage))
  (return _roll _diceresult _critical))

(fn GetDamageDescription
  (params (Character :type BP%20Game%20Character%20Object%20Reference))
  (return ""))

(fn GetAttackDescription
  (params (Character :type BP%20Game%20Character%20Object%20Reference))
  (bind _statmodifier (CallFunction|GetStatMod Character))
  (bind _stats (Variables|/Game/Actors/Characters/BP_GameCharacter.BP_GameCharacter_C|GetStats Character))
  (bind (_value _returnvalue) (Utilities|Map|Find _stats _statmodifier))
  (return (Utilities|Text|FormatText "1d20 + {0}" (Math|Integer|SelectInt _value 0 _returnvalue))))

(fn GetStatMod
  (params (Character :type BP%20Game%20Character%20Object%20Reference)))

(fn GetDescription
  (params (OwnerCharacter :type BP%20Game%20Character%20Object%20Reference))
  (return (Utilities|Text|FormatText (Variables|Default|GetDescriptionFormat) (CallFunction|GetAttackDescription OwnerCharacter) (CallFunction|GetDamageDescription OwnerCharacter))))