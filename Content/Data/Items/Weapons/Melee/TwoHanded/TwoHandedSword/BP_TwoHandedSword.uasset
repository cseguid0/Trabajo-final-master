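; Two-handed sword melee weapon Blueprint that defines its damage roll and damage description text.
; RollDamage rolls a d8 through the dice object, adding DamageBonus and the stat from GetStatMod, which the description labels STR.
; The two-dice option is fixed off, so the Critical input has no effect on the roll.
; The description shows the die, the character's calculated stat modifier (defaulting a missing stat to zero) and the bonus.
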(fn GetDamageDescription
  (params (Character :type BP%20Game%20Character%20Object%20Reference))
  (bind _statmodifier (CallFunction|GetStatMod Character))
  (bind _stats (Variables|/Game/Actors/Characters/BP_GameCharacter.BP_GameCharacter_C|GetStats Character))
  (bind (_value _returnvalue) (Utilities|Map|Find _stats _statmodifier))
  (return (Utilities|Text|FormatText "1d8 + {STR} + {mod}" (Variables|Default|GetDamageBonus) (Utilities|CalculateStatModifier (Math|Integer|SelectInt _value 0 _returnvalue)))))

(fn RollDamage
  (params (Character :type BP%20Game%20Character%20Object%20Reference) (Critical :type Boolean))
  (bind _roll (Default|Roll (Utilities|GetDice) Character (Variables|Default|GetDamageBonus) 0 0 (Math|Integer|SelectInt 2 1 false) 0 0 0 0 (Utilities|Array|MakeArray (CallFunction|GetStatMod)) "NewEnumerator0"))
  (return _roll))

(fn GetStatMod
  (params (Character :type BP%20Game%20Character%20Object%20Reference))
  (return "NewEnumerator0"))