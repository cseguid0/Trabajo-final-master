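; One-handed sword weapon item that defines its damage roll and damage text using tabletop-style dice rules.
; GetStatMod picks the higher of the character's first two Enum_Stat values, finesse-style, favoring the first on a tie.
; RollDamage rolls 1d6, or 2d6 on a critical, adding that stat's modifier and DamageBonus.
; GetDamageDescription shows the same formula with the computed modifier, or a generic DEX label without a valid character.
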(fn GetDamageDescription
  (params (Character :type BP%20Game%20Character%20Object%20Reference))
  (bind _statmodifier (CallFunction|GetStatMod Character))
  (bind _stats (Variables|/Game/Actors/Characters/BP_GameCharacter.BP_GameCharacter_C|GetStats Character))
  (bind _damagebonus (Variables|Default|GetDamageBonus))
  (bind (_value _returnvalue) (Utilities|Map|Find _stats _statmodifier))
  (Utilities|IsValid Character
    (:Is%20Valid
      (return (Utilities|Text|FormatText "1d6 + {DEX} + {mod}" (Utilities|CalculateStatModifier (Math|Integer|SelectInt _value 0 _returnvalue)) _damagebonus)))
    (:Is%20Not%20Valid
      (return (Utilities|Text|FormatText "1d6 + DEX + {number}" _damagebonus)))))

(fn RollDamage
  (params (Character :type BP%20Game%20Character%20Object%20Reference) (Critical :type Boolean))
  (bind _roll (Default|Roll (Utilities|GetDice) Character (Variables|Default|GetDamageBonus) 0 (Math|Integer|SelectInt 2 1 Critical) 0 0 0 0 0 (Utilities|Array|MakeArray (CallFunction|GetStatMod Character)) "NewEnumerator0"))
  (return _roll))

(fn GetStatMod
  (params (Character :type BP%20Game%20Character%20Object%20Reference))
  (bind _returnvalue (Utilities|Enum|LiteralenumEnum_Stat "NewEnumerator1"))
  (bind _returnvalue_2 (Utilities|Enum|LiteralenumEnum_Stat "NewEnumerator0"))
  (bind _stats (Variables|/Game/Actors/Characters/BP_GameCharacter.BP_GameCharacter_C|GetStats Character))
  (bind (_value _returnvalue_3) (Utilities|Map|Find _stats _returnvalue))
  (bind (_value_2 _returnvalue_4) (Utilities|Map|Find _stats _returnvalue_2))
  (return (select (< (Math|Integer|SelectInt _value_2 0 _returnvalue_4) (Math|Integer|SelectInt _value 0 _returnvalue_3)) _returnvalue _returnvalue_2)))