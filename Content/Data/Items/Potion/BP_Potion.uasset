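; BP_Potion is a usable healing potion item whose strength scales with the character's level.
; On use it rolls one d4 per level plus one extra and applies the total as healing to the user.
; It is available only to a player character holding at least one in their inventory.
; Its tooltip shows the scaled dice amount, or generic text without a valid character.
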(event EventUse
  (params (SourceCharacter :type BP%20Game%20Character%20Object%20Reference))
  (bind _roll (Default|Roll (Utilities|GetDice) 0 0 (+ (Variables|/Game/Actors/Characters/BP_GameCharacter.BP_GameCharacter_C|GetLevel SourceCharacter) 1) 0 0 0 0 0 0 "NewEnumerator0" "NewEnumerator0"))
  (Default|ReceiveHealing SourceCharacter _roll))

(fn CheckAvailability
  (params (SourceCharacter :type BP%20Game%20Character%20Object%20Reference))
  (bind _asbp_player_character (Utilities|Casting|CastToBP_PlayerCharacter SourceCharacter)
    (:then
      (bind _count (Default|CountItem (Variables|/Game/Actors/Characters/PlayerCharacter/BP_PlayerCharacter.BP_PlayerCharacter_C|GetInventory _asbp_player_character) self))
      (return (> _count 0)))
    (:CastFailed
      (return false))))

(fn GetTooltipData
  (params (Character :type BP%20Game%20Character%20Object%20Reference))
  (Utilities|IsValid Character
    (:Is%20Valid
      (return (Variables|Default|GetName) (Utilities|Text|FormatText "Heals {number}d4" (+ (Variables|/Game/Actors/Characters/BP_GameCharacter.BP_GameCharacter_C|GetLevel Character) 1)) (Variables|Default|GetIcon)))
    (:Is%20Not%20Valid
      (return (Variables|Default|GetName) (Utilities|Text|FormatText "Heals the character when used") (Variables|Default|GetIcon)))))