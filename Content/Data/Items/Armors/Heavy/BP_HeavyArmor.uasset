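; Heavy armor item that gives its wearer a Stealth disadvantage and a strength bonus while equipped.
; On equip it runs the parent logic, adds the heavy-armor disadvantage gameplay tag and raises the first Enum_Stat entry in the character's Stats map by BonusSTR.
; Removal mirrors this, dropping the tag and subtracting the same bonus, with a missing stat entry treated as zero.
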(event EventOnEquip
  (params (Character :type BP%20Game%20Character%20Object%20Reference))
  (bind _returnvalue (Utilities|Enum|LiteralenumEnum_Stat "NewEnumerator0"))
  (bind _stats (Variables|/Game/Actors/Characters/BP_GameCharacter.BP_GameCharacter_C|GetStats Character))
  (bind (_value _returnvalue_2) (Utilities|Map|Find _stats _returnvalue))
  (|CallParentFunction Character)
  (GameplayTags|AddGameplayTag (Variables|/Game/Actors/Characters/BP_GameCharacter.BP_GameCharacter_C|GetGameplayTags Character) "(TagName=\"Disadvantage.Stealth.HeavyArmor\")" :!class /Script/GameplayTags.BlueprintGameplayTagLibrary)
  (Utilities|Map|Add _stats _returnvalue (+ (Math|Integer|SelectInt _value 0 _returnvalue_2) (Variables|Default|GetBonusSTR))))

(event EventOnRemove
  (params (Character :type BP%20Game%20Character%20Object%20Reference))
  (bind _returnvalue (Utilities|Enum|LiteralenumEnum_Stat "NewEnumerator0"))
  (bind _stats (Variables|/Game/Actors/Characters/BP_GameCharacter.BP_GameCharacter_C|GetStats Character))
  (bind (_value _returnvalue_2) (Utilities|Map|Find _stats _returnvalue))
  (|CallParentFunction Character)
  (GameplayTags|RemoveGameplayTag (Variables|/Game/Actors/Characters/BP_GameCharacter.BP_GameCharacter_C|GetGameplayTags Character) "(TagName=\"Disadvantage.Stealth.HeavyArmor\")" :!class /Script/GameplayTags.BlueprintGameplayTagLibrary)
  (Utilities|Map|Add _stats _returnvalue (- (Math|Integer|SelectInt _value 0 _returnvalue_2) (Variables|Default|GetBonusSTR))))