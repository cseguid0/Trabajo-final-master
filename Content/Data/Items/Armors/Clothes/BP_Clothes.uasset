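; BP_Clothes is a clothing armor item that grants Intelligence and Wisdom bonuses to the character wearing it.
; OnEquip calls the parent logic, then adds BonusINT and BonusWIS to two entries in the character's Stats map, keyed by Enum_Stat.
; OnRemove calls the parent logic and subtracts the same bonuses.
; Both events treat a missing stat entry as zero before writing the new value.
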(event EventOnEquip
  (params (Character :type BP%20Game%20Character%20Object%20Reference))
  (bind _returnvalue (Utilities|Enum|LiteralenumEnum_Stat "NewEnumerator4"))
  (bind _returnvalue_2 (Utilities|Enum|LiteralenumEnum_Stat "NewEnumerator3"))
  (bind _stats (Variables|/Game/Actors/Characters/BP_GameCharacter.BP_GameCharacter_C|GetStats Character))
  (bind _stats_2 (Variables|/Game/Actors/Characters/BP_GameCharacter.BP_GameCharacter_C|GetStats Character))
  (bind (_value _returnvalue_3) (Utilities|Map|Find _stats _returnvalue_2))
  (bind (_value_2 _returnvalue_4) (Utilities|Map|Find _stats_2 _returnvalue))
  (|CallParentFunction Character)
  (Utilities|Map|Add _stats _returnvalue_2 (+ (Math|Integer|SelectInt _value 0 _returnvalue_3) (Variables|Default|GetBonusINT)))
  (Utilities|Map|Add _stats_2 _returnvalue (+ (Math|Integer|SelectInt _value_2 0 _returnvalue_4) (Variables|Default|GetBonusWIS))))

(event EventOnRemove
  (params (Character :type BP%20Game%20Character%20Object%20Reference))
  (bind _returnvalue (Utilities|Enum|LiteralenumEnum_Stat "NewEnumerator4"))
  (bind _returnvalue_2 (Utilities|Enum|LiteralenumEnum_Stat "NewEnumerator3"))
  (bind _stats (Variables|/Game/Actors/Characters/BP_GameCharacter.BP_GameCharacter_C|GetStats Character))
  (bind _stats_2 (Variables|/Game/Actors/Characters/BP_GameCharacter.BP_GameCharacter_C|GetStats Character))
  (bind (_value _returnvalue_3) (Utilities|Map|Find _stats _returnvalue_2))
  (bind (_value_2 _returnvalue_4) (Utilities|Map|Find _stats_2 _returnvalue))
  (|CallParentFunction Character)
  (Utilities|Map|Add _stats _returnvalue_2 (- (Math|Integer|SelectInt _value 0 _returnvalue_3) (Variables|Default|GetBonusINT)))
  (Utilities|Map|Add _stats_2 _returnvalue (- (Math|Integer|SelectInt _value_2 0 _returnvalue_4) (Variables|Default|GetBonusWIS))))