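; BP_Shield is a shield item that raises the wearer's AC and also supplies a damage value.
; Equipping adds its Armor value to the character's AC, and removal subtracts it.
; Damage is one plus the character stat chosen by GetStatMod, treating a missing stat as zero and never dropping below zero.
; RollDamage uses no randomness and ignores criticals, so GetDamageDescription shows the same number as text.
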(event EventOnEquip
  (params (Character :type BP%20Game%20Character%20Object%20Reference))
  (Variables|/Game/Actors/Characters/BP_GameCharacter.BP_GameCharacter_C|SetAC Character (+ (Variables|/Game/Actors/Characters/BP_GameCharacter.BP_GameCharacter_C|GetAC Character) (Variables|Default|GetArmor))))

(event EventOnRemove
  (params (Character :type BP%20Game%20Character%20Object%20Reference))
  (Variables|/Game/Actors/Characters/BP_GameCharacter.BP_GameCharacter_C|SetAC Character (- (Variables|/Game/Actors/Characters/BP_GameCharacter.BP_GameCharacter_C|GetAC Character) (Variables|Default|GetArmor))))

(fn GetStatMod
  (params (Character :type BP%20Game%20Character%20Object%20Reference))
  (return "NewEnumerator0"))

(fn RollDamage
  (params (Character :type BP%20Game%20Character%20Object%20Reference) (Critical :type Boolean))
  (bind _statmodifier (CallFunction|GetStatMod Character))
  (bind _stats (Variables|/Game/Actors/Characters/BP_GameCharacter.BP_GameCharacter_C|GetStats Character))
  (bind (_value _returnvalue) (Utilities|Map|Find _stats _statmodifier))
  (return (Math|Integer|Max(Integer) (+ 1 (Math|Integer|SelectInt _value 0 _returnvalue)))))

(fn GetDamageDescription
  (params (Character :type BP%20Game%20Character%20Object%20Reference))
  (bind _statmodifier (CallFunction|GetStatMod Character))
  (bind _stats (Variables|/Game/Actors/Characters/BP_GameCharacter.BP_GameCharacter_C|GetStats Character))
  (bind (_value _returnvalue) (Utilities|Map|Find _stats _statmodifier))
  (return (Utilities|Text|ToText(Integer) (Math|Integer|Max(Integer) (+ 1 (Math|Integer|SelectInt _value 0 _returnvalue))))))