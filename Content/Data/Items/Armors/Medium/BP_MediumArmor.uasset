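; Medium armor item Blueprint that adjusts a character's Dexterity and Armor Class when equipped or removed, extending parent equip logic.
; OnEquip adds BonusDEX to the stat map, then adds the resulting stat modifier, capped at three, to AC.
; OnRemove subtracts the bonus first, then deducts the capped modifier recomputed from the reduced stat, so the AC deduction can differ from what was added.
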(event EventOnEquip
  (params (Character :type BP%20Game%20Character%20Object%20Reference))
  (bind _returnvalue (Utilities|Enum|LiteralenumEnum_Stat "NewEnumerator1"))
  (bind _stats (Variables|/Game/Actors/Characters/BP_GameCharacter.BP_GameCharacter_C|GetStats Character))
  (bind (_value _returnvalue_2) (Utilities|Map|Find _stats _returnvalue))
  (bind _returnvalue_3 (Math|Integer|SelectInt _value 0 _returnvalue_2))
  (|CallParentFunction Character)
  (Utilities|Map|Add _stats _returnvalue (+ _returnvalue_3 (Variables|Default|GetBonusDEX)))
  (Variables|/Game/Actors/Characters/BP_GameCharacter.BP_GameCharacter_C|SetAC Character (+ (Variables|/Game/Actors/Characters/BP_GameCharacter.BP_GameCharacter_C|GetAC Character) (Math|Integer|Min(Integer) (Utilities|CalculateStatModifier _returnvalue_3) 3))))

(event EventOnRemove
  (params (Character :type BP%20Game%20Character%20Object%20Reference))
  (bind _returnvalue (Utilities|Enum|LiteralenumEnum_Stat "NewEnumerator1"))
  (bind _stats (Variables|/Game/Actors/Characters/BP_GameCharacter.BP_GameCharacter_C|GetStats Character))
  (bind (_value _returnvalue_2) (Utilities|Map|Find _stats _returnvalue))
  (bind _returnvalue_3 (Math|Integer|SelectInt _value 0 _returnvalue_2))
  (|CallParentFunction Character)
  (Utilities|Map|Add _stats _returnvalue (- _returnvalue_3 (Variables|Default|GetBonusDEX)))
  (Variables|/Game/Actors/Characters/BP_GameCharacter.BP_GameCharacter_C|SetAC Character (- (Variables|/Game/Actors/Characters/BP_GameCharacter.BP_GameCharacter_C|GetAC Character) (Math|Integer|Min(Integer) (Utilities|CalculateStatModifier _returnvalue_3) 3))))