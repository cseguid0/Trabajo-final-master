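; Dialogue option Blueprint that gives the player a quest when selected.
; On selection it constructs an object from its Quest class and passes it to AcceptQuest on BP_GameInstance.
; IsVisible hides the option once the game instance's QuestData holds an object of that exact class; it calls the parent check but ignores the result.
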(event EventOnSelected
  (params (WorldContextObject :type Object%20Object%20Reference) (Window :type UI%20Dialogue%20Window%20Object%20Reference))
  (bind _asbp_game_instance (Utilities|Casting|CastToBP_GameInstance (Game|GetGameInstance WorldContextObject)))
  (bind _returnvalue (Game|ConstructObjectfromClass (Variables|Default|GetQuest) WorldContextObject))
  (Default|AcceptQuest _asbp_game_instance _returnvalue))

(fn IsVisible
  (params (WorldContextObject :type Object%20Object%20Reference))
  (|CallParentFunction WorldContextObject)
  (bind _asbp_game_instance (Utilities|Casting|CastToBP_GameInstance (Game|GetGameInstance WorldContextObject)))
  (for _array_element (Variables|/Game/GameInstance/BP_GameInstance.BP_GameInstance_C|GetQuestData _asbp_game_instance)
    (if (== (Utilities|GetClass _array_element) (Variables|Default|GetQuest))
      (return false)))
  (return true))