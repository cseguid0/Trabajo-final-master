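; Dialogue node that opens a trade window with the NPC of the current dialogue.
; On selection it stores the dialogue window, then creates UI_TradeWindow with that NPC as trader and itself as origin, and adds it to the viewport.
; When trade closes, it switches the dialogue window to the OnLeaveTree, refreshes its UI and selects that tree, using the game instance as world context.
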(event Custom|onTradeClosed
  (bind _window (Variables|Default|GetWindow))
  (bind _output_get (Variables|/Game/UI/DialogueWindow/UI_DialogueWindow.UI_DialogueWindow_C|SetDialogueTree _window (Variables|Default|GetOnLeaveTree)))
  (Default|UpdateUI _window)
  (Default|OnSelected _output_get (Game|GetGameInstance _window) (Variables|Default|GetWindow)))

(event EventOnSelected
  (params (WorldContextObject :type Object%20Object%20Reference) (Window :type UI%20Dialogue%20Window%20Object%20Reference))
  (Variables|Default|SetWindow Window)
  (bind _returnvalue (UserInterface|CreateWidget WorldContextObject "/Game/UI/TradeWindow/UI_TradeWindow.UI_TradeWindow_C" 0 (Variables|/Game/UI/DialogueWindow/UI_DialogueWindow.UI_DialogueWindow_C|GetNPC Window) self))
  (UserInterface|Viewport|AddtoViewport _returnvalue 0))