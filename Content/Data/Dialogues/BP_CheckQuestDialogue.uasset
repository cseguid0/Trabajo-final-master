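; BP_CheckQuestDialogue is a dialogue visibility condition that depends on the state of a quest.
; IsVisible reads the QuestData list from BP_GameInstance and looks for an entry whose class matches Quest and whose Status equals QuestState.
; It returns true on the first match and false when none is found.
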(fn IsVisible
  (params (WorldContextObject :type Object%20Object%20Reference))
  (bind _asbp_game_instance (Utilities|Casting|CastToBP_GameInstance (Game|GetGameInstance WorldContextObject)))
  (for _array_element (Variables|/Game/GameInstance/BP_GameInstance.BP_GameInstance_C|GetQuestData _asbp_game_instance)
    (if (and (== (Utilities|GetClass _array_element) (Variables|Default|GetQuest)) (Utilities|Enum|Equal(Enum) (Variables|/Game/Data/Quests/BP_Quest.BP_Quest_C|GetStatus _array_element) (Variables|Default|GetQuestState)))
      (return true)))
  (return false))