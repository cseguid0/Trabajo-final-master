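; Dialogue option that completes the current objective of a configured quest when the player selects it.
; On selection, it finds entries in the game instance's QuestData matching the Quest class, sets their remaining progress to 1 and advances the objective.
; The option is visible only while a matching quest has a specific status.
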(event EventOnSelected
  (params (WorldContextObject :type Object%20Object%20Reference) (Window :type UI%20Dialogue%20Window%20Object%20Reference))
  (bind _asbp_game_instance (Utilities|Casting|CastToBP_GameInstance (Game|GetGameInstance WorldContextObject)))
  (for _array_element (Variables|/Game/GameInstance/BP_GameInstance.BP_GameInstance_C|GetQuestData _asbp_game_instance)
    (if (== (Utilities|GetClass _array_element) (Variables|Default|GetQuest))
      (Variables|/Game/Data/Quests/BP_Quest.BP_Quest_C|SetRemainingProgress _array_element 1)
      (Default|AdvanceObjetive _array_element))))

(fn IsVisible
  (params (WorldContextObject :type Object%20Object%20Reference))
  (bind _asbp_game_instance (Utilities|Casting|CastToBP_GameInstance (Game|GetGameInstance WorldContextObject)))
  (for _array_element (Variables|/Game/GameInstance/BP_GameInstance.BP_GameInstance_C|GetQuestData _asbp_game_instance)
    (if (and (== (Utilities|GetClass _array_element) (Variables|Default|GetQuest)) (Utilities|Enum|Equal(Enum) (Variables|/Game/Data/Quests/BP_Quest.BP_Quest_C|GetStatus _array_element) "NewEnumerator1"))
      (return true)))
  (return false))