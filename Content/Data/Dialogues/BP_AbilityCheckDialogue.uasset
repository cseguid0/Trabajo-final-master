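; Dialogue node that resolves a player ability check against an NPC when selected.
; The difficulty is itself a dice roll by the window's NPC using its own dice and modifiers.
; The player's check applies configured dice, modifiers and counted advantages or disadvantages against that roll.
; The critical, success or failure result swaps the window's dialogue tree to that option, refreshes the UI and immediately triggers it.
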(event Custom|OnSuccess
  (bind _window (Variables|Default|GetWindow))
  (bind _output_get (Variables|/Game/UI/DialogueWindow/UI_DialogueWindow.UI_DialogueWindow_C|SetDialogueTree _window (Variables|Default|GetSuccessOption)))
  (Default|UpdateUI _window)
  (Default|OnSelected _output_get (Game|GetGameInstance _window) _window))

(event Custom|OnFailure
  (bind _window (Variables|Default|GetWindow))
  (bind _output_get (Variables|/Game/UI/DialogueWindow/UI_DialogueWindow.UI_DialogueWindow_C|SetDialogueTree _window (Variables|Default|GetFailureOption)))
  (Default|UpdateUI _window)
  (Default|OnSelected _output_get (Game|GetGameInstance _window) _window))

(event Custom|OnCriticalSuccess
  (bind _window (Variables|Default|GetWindow))
  (bind _output_get (Variables|/Game/UI/DialogueWindow/UI_DialogueWindow.UI_DialogueWindow_C|SetDialogueTree _window (Variables|Default|GetCriticalSuccessOption)))
  (Default|UpdateUI _window)
  (Default|OnSelected _output_get (Game|GetGameInstance _window) _window))

(event EventOnSelected
  (params (WorldContextObject :type Object%20Object%20Reference) (Window :type UI%20Dialogue%20Window%20Object%20Reference))
  (Variables|Default|SetWindow Window)
  (bind _asbp_player_character (Utilities|Casting|CastToBP_PlayerCharacter (Game|GetPlayerCharacter WorldContextObject)))
  (bind _roll (Default|Roll (Utilities|GetDice) (Variables|/Game/UI/DialogueWindow/UI_DialogueWindow.UI_DialogueWindow_C|GetNPC Window) (Variables|AbilityCheckDifficulty|GetDifficulty%20Static%20Modifier) (Variables|AbilityCheckDifficulty|GetDifficulty%20Amount%20D4) (Variables|AbilityCheckDifficulty|GetDifficulty%20Amount%20D6) (Variables|AbilityCheckDifficulty|GetDifficulty%20Amount%20D8) (Variables|AbilityCheckDifficulty|GetDifficulty%20Amount%20D10) (Variables|AbilityCheckDifficulty|GetDifficulty%20Amount%20D12) (Variables|AbilityCheckDifficulty|GetDifficulty%20Amount%20D20) (Variables|AbilityCheckDifficulty|GetDifficulty%20Amount%20D100) (Variables|AbilityCheckDifficulty|GetDifficulty%20Stat%20Modifiers) (Variables|AbilityCheckDifficulty|GetDifficulty%20Proficiency%20Modifiers)))
  (bind (_success _critical) (Utilities|AbilityCheck _asbp_player_character (Variables|AbilityCheckRoll|GetStatic%20Modifier) (Variables|AbilityCheckRoll|GetAmount%20D4) (Variables|AbilityCheckRoll|GetAmount%20D6) (Variables|AbilityCheckRoll|GetAmount%20D8) (Variables|AbilityCheckRoll|GetAmount%20D10) (Variables|AbilityCheckRoll|GetAmount%20D12) (Variables|AbilityCheckRoll|GetAmount%20D20) (Variables|AbilityCheckRoll|GetAmount%20D100) (Variables|AbilityCheckRoll|GetStat%20Modifiers) (Variables|AbilityCheckRoll|GetProficiency%20Modifiers) (Utilities|CountAdvantage _asbp_player_character (Variables|AbilityCheckRoll|GetAdvantages) (Variables|AbilityCheckRoll|GetDisadvantages)) _roll))
  (if _critical
    (CallFunction|OnCriticalSuccess)
    (elif _success
      (CallFunction|OnSuccess)
      (else
        (CallFunction|OnFailure)))))