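; Base quest Blueprint that tracks objective progress and completion, with empty hooks that appear intended for child quests to override.
; AdvanceObjetive decrements RemainingProgress and calls Complete at zero, which changes Status, then calls GiveRewards and OnComplete.
; OnLoad re-runs OnAccept, while OnAccept, GiveRewards and OnComplete are empty stubs and GetObjetiveText returns an empty string.
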(event Custom|AdvanceObjetive
  (Math|Integer|DecrementInt (Variables|Default|GetRemainingProgress)
    (:%20%20
      (if (== (Variables|Default|GetRemainingProgress) 0)
        (CallFunction|Complete)))))

(event Custom|Complete
  (Variables|Default|SetStatus "NewEnumerator2")
  (CallFunction|GiveRewards)
  (CallFunction|OnComplete))

(event Custom|OnAccept)

(event Custom|GiveRewards)

(event Custom|OnComplete)

(fn GetObjetiveText
  (return ""))

(fn OnLoad
  (CallFunction|OnAccept))