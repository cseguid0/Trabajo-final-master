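; Secondary quest in which the player must find and solve the secret puzzle.
; On accept it binds to the game instance's EventDispatchManager puzzle-solved event, advances its objective when the secret puzzle is reported, and unbinds on completion.
; Rewards grant experience, money and a heavy armor item, which is spawned at the player's transform if adding it to the inventory fails.
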(event Custom|PuzzleSolved
  (params (Puzzle :type Name))
  (if (== Puzzle "SecretPuzzle")
    (CallFunction|AdvanceObjetive)))

(event EventGiveRewards
  (bind _world_context_object (Variables|Default|GetWorld%20Context%20Object))
  (bind _returnvalue (Game|GetPlayerCharacter _world_context_object))
  (bind _asbp_player_character (Utilities|Casting|CastToBP_PlayerCharacter _returnvalue))
  (Default|AddExp _asbp_player_character 250)
  (Default|AddMoney _asbp_player_character 500)
  (bind _added (Default|AddItem (Variables|/Game/Actors/Characters/PlayerCharacter/BP_PlayerCharacter.BP_PlayerCharacter_C|GetInventory _asbp_player_character) "/Game/Data/Items/Armors/Heavy/DA_+3HeavyArmor.DA_+3HeavyArmor"))
  (if (not _added)
    (bind _asbp_game_instance (Utilities|Casting|CastToBP_GameInstance (Game|GetGameInstance (Variables|Default|GetWorld%20Context%20Object))))
    (Default|SpawnItem _asbp_game_instance (Transformation|GetActorTransform _returnvalue) (Utilities|Struct|MakeST_ItemStack "/Game/Data/Items/Armors/Heavy/DA_+3HeavyArmor.DA_+3HeavyArmor" 1))))

(event EventOnAccept
  (bind _asbp_game_instance (Utilities|Casting|CastToBP_GameInstance (Game|GetGameInstance (Variables|Default|GetWorld%20Context%20Object))))
  (EventDispatchers|BindEventtoPuzzleSolved (Variables|/Game/GameInstance/BP_GameInstance.BP_GameInstance_C|GetEventDispatchManager _asbp_game_instance) (delegate Custom|PuzzleSolved)))

(event EventOnComplete
  (bind _asbp_game_instance (Utilities|Casting|CastToBP_GameInstance (Game|GetGameInstance (Variables|Default|GetWorld%20Context%20Object))))
  (EventDispatchers|UnbindEventfromPuzzleSolved (Variables|/Game/GameInstance/BP_GameInstance.BP_GameInstance_C|GetEventDispatchManager _asbp_game_instance) (delegate Custom|PuzzleSolved)))

(fn GetObjetiveText
  (return "Find where the puzzle is and solve it"))