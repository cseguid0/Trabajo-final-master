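; Quest Blueprint for the principal quest to defeat the bandit boss.
; On accept it binds to the game instance's event dispatch manager for the bandit boss kill, advancing its objective when that fires, and unbinds on completion.
; Its rewards grant the player experience and money, then chain the story by constructing and accepting the Return the Stolen Shipment quest.
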(event Custom|KillBanditBoss
  (CallFunction|AdvanceObjetive))

(event EventGiveRewards
  (bind _asbp_game_instance (Utilities|Casting|CastToBP_GameInstance (Game|GetGameInstance (Variables|Default|GetWorld%20Context%20Object))))
  (bind _returnvalue (Game|ConstructObjectfromClass _asbp_game_instance "/Game/Data/Quests/PrincipalQuests/ReturnTheStolenShipment/BP_ReturnTheStolenShipmentQuest.BP_ReturnTheStolenShipmentQuest_C" _asbp_game_instance))
  (Default|AcceptQuest _asbp_game_instance _returnvalue)
  (bind _asbp_player_character (Utilities|Casting|CastToBP_PlayerCharacter (Game|GetPlayerCharacter (Variables|Default|GetWorld%20Context%20Object))))
  (Default|AddExp _asbp_player_character 300)
  (Default|AddMoney _asbp_player_character 500))

(event EventOnAccept
  (bind _asbp_game_instance (Utilities|Casting|CastToBP_GameInstance (Game|GetGameInstance (Variables|Default|GetWorld%20Context%20Object))))
  (EventDispatchers|BindEventtoBanditBossKill (Variables|/Game/GameInstance/BP_GameInstance.BP_GameInstance_C|GetEventDispatchManager _asbp_game_instance) (delegate Custom|KillBanditBoss)))

(event EventOnComplete
  (bind _asbp_game_instance (Utilities|Casting|CastToBP_GameInstance (Game|GetGameInstance (Variables|Default|GetWorld%20Context%20Object))))
  (EventDispatchers|UnbindEventfromBanditBossKill (Variables|/Game/GameInstance/BP_GameInstance.BP_GameInstance_C|GetEventDispatchManager _asbp_game_instance) (delegate Custom|KillBanditBoss)))

(fn GetObjetiveText
  (return "Defeat the bandit boss"))