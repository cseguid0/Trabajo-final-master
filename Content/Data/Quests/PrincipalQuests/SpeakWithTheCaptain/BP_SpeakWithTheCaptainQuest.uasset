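; Main-story quest object that tasks the player with speaking to the captain in the city.
; On accept it binds to the game instance's EventDispatchManager, advances its objective when the speak event fires, and unbinds on completion.
; Its rewards grant the player money and experience, then construct and accept the follow-up Find The Stolen Shipment quest, chaining the questline.
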(event Custom|SpeakWithTheCaptain
  (CallFunction|AdvanceObjetive))

(event EventGiveRewards
  (bind _world_context_object (Variables|Default|GetWorld%20Context%20Object))
  (bind _asbp_player_character (Utilities|Casting|CastToBP_PlayerCharacter (Game|GetPlayerCharacter _world_context_object)))
  (Default|AddMoney _asbp_player_character 100)
  (Default|AddExp _asbp_player_character 200)
  (bind _asbp_game_instance (Utilities|Casting|CastToBP_GameInstance (Game|GetGameInstance _world_context_object)))
  (bind _returnvalue (Game|ConstructObjectfromClass _asbp_game_instance "/Game/Data/Quests/PrincipalQuests/FindTheStolenShipment/BP_FindTheStolenShipmentQuest.BP_FindTheStolenShipmentQuest_C" _asbp_game_instance))
  (Default|AcceptQuest _asbp_game_instance _returnvalue))

(event EventOnAccept
  (bind _asbp_game_instance (Utilities|Casting|CastToBP_GameInstance (Game|GetGameInstance (Variables|Default|GetWorld%20Context%20Object))))
  (EventDispatchers|BindEventtoSpeakwiththeCaptain (Variables|/Game/GameInstance/BP_GameInstance.BP_GameInstance_C|GetEventDispatchManager _asbp_game_instance) (delegate Custom|SpeakWithTheCaptain)))

(event EventOnComplete
  (bind _asbp_game_instance (Utilities|Casting|CastToBP_GameInstance (Game|GetGameInstance (Variables|Default|GetWorld%20Context%20Object))))
  (EventDispatchers|UnbindEventfromSpeakwiththeCaptain (Variables|/Game/GameInstance/BP_GameInstance.BP_GameInstance_C|GetEventDispatchManager _asbp_game_instance) (delegate Custom|SpeakWithTheCaptain)))

(fn GetObjetiveText
  (return "Speak with the captain in the city"))