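; Quest Blueprint for "Return the Stolen Shipment", a principal quest whose objective is to speak with the captain in the city.
; Accepting the quest binds to the SpeakWithTheCaptain event on the game instance's EventDispatchManager, and completing it unbinds.
; That event advances the objective, while GiveRewards grants money and experience to the player character.
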(event Custom|SpeakWithTheCaptain
  (CallFunction|AdvanceObjetive))

(event EventOnAccept
  (bind _asbp_game_instance (Utilities|Casting|CastToBP_GameInstance (Game|GetGameInstance (Variables|Default|GetWorld%20Context%20Object))))
  (EventDispatchers|BindEventtoSpeakwiththeCaptain (Variables|/Game/GameInstance/BP_GameInstance.BP_GameInstance_C|GetEventDispatchManager _asbp_game_instance) (delegate Custom|SpeakWithTheCaptain)))

(event EventOnComplete
  (bind _asbp_game_instance (Utilities|Casting|CastToBP_GameInstance (Game|GetGameInstance (Variables|Default|GetWorld%20Context%20Object))))
  (EventDispatchers|UnbindEventfromSpeakwiththeCaptain (Variables|/Game/GameInstance/BP_GameInstance.BP_GameInstance_C|GetEventDispatchManager _asbp_game_instance) (delegate Custom|SpeakWithTheCaptain)))

(event EventGiveRewards
  (bind _asbp_player_character (Utilities|Casting|CastToBP_PlayerCharacter (Game|GetPlayerCharacter (Variables|Default|GetWorld%20Context%20Object))))
  (Default|AddMoney _asbp_player_character 1500)
  (Default|AddExp _asbp_player_character 400))

(fn GetObjetiveText
  (return "Speak with the captain in the city"))