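; Quest object for the main quest to find the stolen shipment.
; On accept it binds to the game instance's EventDispatchManager find-location event, advances the objective when the "StolenShipment" location is reported, and unbinds on completion.
; Its reward step grants the player experience and chains the story by constructing and accepting the End The Bandit Boss quest.
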(event Custom|FindStolenShipment
  (params (Location :type Name))
  (if (== Location "StolenShipment")
    (CallFunction|AdvanceObjetive)))

(event EventGiveRewards
  (bind _asbp_game_instance (Utilities|Casting|CastToBP_GameInstance (Game|GetGameInstance (Variables|Default|GetWorld%20Context%20Object))))
  (bind _returnvalue (Game|ConstructObjectfromClass _asbp_game_instance "/Game/Data/Quests/PrincipalQuests/EndTheBanditBoss/BP_EndTheBanditBossQuest.BP_EndTheBanditBossQuest_C" _asbp_game_instance))
  (Default|AcceptQuest _asbp_game_instance _returnvalue)
  (bind _asbp_player_character (Utilities|Casting|CastToBP_PlayerCharacter (Game|GetPlayerCharacter (Variables|Default|GetWorld%20Context%20Object))))
  (Default|AddExp _asbp_player_character 300))

(event EventOnAccept
  (bind _asbp_game_instance (Utilities|Casting|CastToBP_GameInstance (Game|GetGameInstance (Variables|Default|GetWorld%20Context%20Object))))
  (EventDispatchers|BindEventtoFindLocation (Variables|/Game/GameInstance/BP_GameInstance.BP_GameInstance_C|GetEventDispatchManager _asbp_game_instance) (delegate Custom|FindStolenShipment)))

(event EventOnComplete
  (bind _asbp_game_instance (Utilities|Casting|CastToBP_GameInstance (Game|GetGameInstance (Variables|Default|GetWorld%20Context%20Object))))
  (EventDispatchers|UnbindEventfromFindLocation (Variables|/Game/GameInstance/BP_GameInstance.BP_GameInstance_C|GetEventDispatchManager _asbp_game_instance) (delegate Custom|FindStolenShipment)))

(fn GetObjetiveText
  (return "Find where the stolen shipment is"))