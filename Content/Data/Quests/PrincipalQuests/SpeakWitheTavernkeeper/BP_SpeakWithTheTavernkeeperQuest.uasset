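; Principal quest asset that asks the player to speak with the tavernkeeper.
; On accept it binds its objective handler to the tavernkeeper dialogue event on the game instance's EventDispatchManager, and unbinds it on completion.
; That event advances the objective.
; Rewards grant money to the player character and chain the story by constructing and accepting the Speak With The Captain quest.
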(event Custom|SpeakWithTheTavernkeeper
  (CallFunction|AdvanceObjetive))

(event EventGiveRewards
  (bind _asbp_player_character (Utilities|Casting|CastToBP_PlayerCharacter (Game|GetPlayerCharacter (Variables|Default|GetWorld%20Context%20Object))))
  (Default|AddMoney _asbp_player_character 150)
  (bind _asbp_game_instance (Utilities|Casting|CastToBP_GameInstance (Game|GetGameInstance (Variables|Default|GetWorld%20Context%20Object))))
  (bind _returnvalue (Game|ConstructObjectfromClass _asbp_game_instance "/Game/Data/Quests/PrincipalQuests/SpeakWithTheCaptain/BP_SpeakWithTheCaptainQuest.BP_SpeakWithTheCaptainQuest_C" _asbp_game_instance))
  (Default|AcceptQuest _asbp_game_instance _returnvalue))

(event EventOnAccept
  (bind _asbp_game_instance (Utilities|Casting|CastToBP_GameInstance (Game|GetGameInstance (Variables|Default|GetWorld%20Context%20Object))))
  (EventDispatchers|BindEventtoSpeakwiththeTavernkeeper (Variables|/Game/GameInstance/BP_GameInstance.BP_GameInstance_C|GetEventDispatchManager _asbp_game_instance) (delegate Custom|SpeakWithTheTavernkeeper)))

(event EventOnComplete
  (bind _asbp_game_instance (Utilities|Casting|CastToBP_GameInstance (Game|GetGameInstance (Variables|Default|GetWorld%20Context%20Object))))
  (EventDispatchers|UnbindEventfromSpeakwiththeTavernkeeper (Variables|/Game/GameInstance/BP_GameInstance.BP_GameInstance_C|GetEventDispatchManager _asbp_game_instance) (delegate Custom|SpeakWithTheTavernkeeper)))

(fn GetObjetiveText
  (return "Speak with the tavernkeeper"))