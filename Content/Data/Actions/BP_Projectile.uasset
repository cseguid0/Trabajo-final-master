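; Projectile actor for actions that travels from a Source toward a Target and reports when it reaches it.
; Construction applies speed, gravity and optional homing to the movement component; BeginPlay ignores the Source and points velocity at the Target.
; A hit on the Target calls OnTargetReached with the critical flag, then plays impact effect and sound and destroys the actor.
; Other hits are ignored unless the Target is invalid, which triggers only impact and destruction.
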(event OnComponentHit(CollisionSphere)
  (params (HitComponent :type Primitive%20Component%20Object%20Reference) (OtherActor :type Actor%20Object%20Reference) (OtherComp :type Primitive%20Component%20Object%20Reference) (NormalImpulse :type Vector :default "0, 0, 0") (Hit :type Hit%20Result%20Structure%20%28by%20ref%29))
  (bind _location (Collision|BreakHitResult Hit))
  (bind _target (Variables|Target|GetTarget)
    (:then
      (if (== _target OtherActor)
        (Default|CallOnTargetReached (Variables|Default|GetSource) (Variables|Target|GetTarget) (Variables|Default|GetCritical))
        (bind _impacteffect (Variables|Effects|GetImpactEffect :!label _label)
          (:then
            (Niagara|SpawnSystematLocation _impacteffect _location))
          (:else
            _))
        (bind _impactsound (Variables|Effects|GetImpactSound)
          (:then
            (Audio|PlaySoundatLocation _impactsound _location "0, 0, 0" 1.0 1.0 0.0 0 0 0 0))
          (:else
            _))
        (Actor|DestroyActor)))
    (:else
      (goto _label))))

(event EventBeginPlay
  (Collision|IgnoreActorwhenMoving (Variables|Default|GetCollisionSphere) (Variables|Default|GetSource) true)
  (bind _target (Variables|Target|GetTarget)
    (:then
      (Variables|/Script/Engine.MovementComponent|SetVelocity (Variables|Default|GetProjectileMovement) (Math|Vector|GetUnitDirection(Vector) (Transformation|GetActorLocation) (Transformation|GetActorLocation _target))))
    (:else)))

(fn ConstructionScript
  (bind _projectilemovement (Variables|Default|GetProjectileMovement))
  (bind _speed (Variables|ProjectileSettings|GetSpeed))
  (Variables|/Script/Engine.ProjectileMovementComponent|SetInitialSpeed _projectilemovement _speed)
  (Variables|/Script/Engine.ProjectileMovementComponent|SetMaxSpeed _projectilemovement _speed)
  (Variables|/Script/Engine.ProjectileMovementComponent|SetProjectileGravityScale _projectilemovement (Variables|ProjectileSettings|GetGravityScale))
  (Variables|Target|GetTarget
    (:then
      (bind _output_get (Variables|/Script/Engine.ProjectileMovementComponent|SetbIsHomingProjectile _projectilemovement (Variables|Target|GetisHoming)))
      (if _output_get
        (Variables|/Script/Engine.ProjectileMovementComponent|SetHomingTargetComponent _projectilemovement (Variables|/Script/Engine.Actor|GetRootComponent (Variables|Target|GetTarget)))))
    (:else)))