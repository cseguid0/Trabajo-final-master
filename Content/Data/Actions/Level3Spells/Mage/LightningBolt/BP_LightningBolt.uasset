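; Lightning Bolt, a level 3 Mage spell action that damages the target and characters in the line between it and the caster.
; DoAction spawns a projectile through the game instance and binds an event to its target-reached callback.
; DealDamage multi-line traces on Visibility from caster to target, then handles the target separately.
; Each victim gets its own 8d6 roll and DEX save against the caster's spell difficulty, halving damage on success.
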(event Custom|DealDamage
  (params (ProjectileSource :type BP%20Game%20Character%20Object%20Reference) (ProjectileTarget :type BP%20Game%20Character%20Object%20Reference) (Critical :type Boolean))
  (bind _difficulty (Utilities|GetSpellSaveThrowDifficulty ProjectileSource "NewEnumerator3"))
  (bind _self self)
  (bind _self_2 self)
  (bind _outhits (Collision|MultiLineTraceByChannel ProjectileSource (Transformation|GetActorLocation ProjectileSource) (Transformation|GetActorLocation ProjectileTarget) "TraceTypeQuery1" false (Utilities|Array|MakeArray ProjectileSource ProjectileTarget) "None"))
  (for _array_element _outhits
    (bind _asbp_game_character (Utilities|Casting|CastToBP_GameCharacter (.HitActor (Collision|BreakHitResult _array_element))))
    (bind _success (Utilities|AbilitySave _asbp_game_character "NewEnumerator1" _difficulty))
    (bind _roll (Default|Roll (Utilities|GetDice) 0 0 0 8 0 0 0 0 0 "NewEnumerator0" "NewEnumerator0"))
    (if _success
      (Default|ReceiveDamage _asbp_game_character (/ _roll 2) _self_2 ProjectileSource)
      (else
        (Default|ReceiveDamage _asbp_game_character _roll _self_2 ProjectileSource))))
  (bind _success_2 (Utilities|AbilitySave ProjectileTarget "NewEnumerator1" _difficulty))
  (bind _roll_2 (Default|Roll (Utilities|GetDice) 0 0 0 8 0 0 0 0 0 "NewEnumerator0" "NewEnumerator0"))
  (if _success_2
    (Default|ReceiveDamage ProjectileTarget (/ _roll_2 2) _self ProjectileSource)
    (else
      (Default|ReceiveDamage ProjectileTarget _roll_2 _self ProjectileSource))))

(fn DoAction
  (params (SourceCharacter :type BP%20Game%20Character%20Object%20Reference) (TargetCharacter :type BP%20Game%20Character%20Object%20Reference) (TargetLocation :type Vector :default "0, 0, 0") (AttackRollSuccess :type Boolean) (AttackRollCritical :type Boolean))
  (bind _asbp_game_instance (Utilities|Casting|CastToBP_GameInstance (Game|GetGameInstance SourceCharacter)))
  (bind _returnvalue (Default|SpawnProjectile _asbp_game_instance "/Game/Data/Actions/Level3Spells/Mage/LightningBolt/BP_LightningBoltProjectile.BP_LightningBoltProjectile_C" (Transformation|GetActorLocation SourceCharacter) SourceCharacter TargetCharacter SourceCharacter AttackRollCritical SourceCharacter))
  (EventDispatchers|BindEventtoOnTargetReached _returnvalue (EventDispatchers|CreateEvent :!event Custom|DealDamage)))

(fn GetDescription
  (params (Caster :type BP%20Game%20Character%20Object%20Reference) (PlayerData :type ST%20Player%20Data%20Structure))
  (return "All characters between you and your target receive 8d6 points of damage. If they succed a DEX save they receive half damage"))