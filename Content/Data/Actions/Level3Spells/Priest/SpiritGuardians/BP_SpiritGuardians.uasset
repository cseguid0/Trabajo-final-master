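; Spirit Guardians spell action, a level 3 Priest spell that surrounds the caster with spirits that damage enemies.
; DoAction spawns a persistent AoE through the game instance, attaches it to the caster and binds its area-entered event.
; DealDamage rolls d8s, adds a stat modifier when the source has the WIS spell damage tag, and applies the result as DoT damage.
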(event Custom|DealDamage
  (params (Character :type BP%20Game%20Character%20Object%20Reference) (Source :type BP%20Game%20Character%20Object%20Reference))
  (bind _roll (Default|Roll (Utilities|GetDice) Source 0 0 0 3 0 0 0 0 (select (GameplayTags|HasTag (Variables|/Game/Actors/Characters/BP_GameCharacter.BP_GameCharacter_C|GetGameplayTags Source) "(TagName=\"Modifier.DamageRoll.WISSpellDamage\")") (Utilities|Array|MakeArray "NewEnumerator4") "NewEnumerator0") "NewEnumerator0"))
  (Default|ReceiveDoTDamage Character _roll))

(fn DoAction
  (params (SourceCharacter :type BP%20Game%20Character%20Object%20Reference) (TargetCharacter :type BP%20Game%20Character%20Object%20Reference) (TargetLocation :type Vector :default "0, 0, 0") (AttackRollSuccess :type Boolean) (AttackRollCritical :type Boolean))
  (bind _asbp_game_instance (Utilities|Casting|CastToBP_GameInstance (Game|GetGameInstance SourceCharacter)))
  (bind _returnvalue (Default|SpawnPersistentAoE _asbp_game_instance "/Game/Data/Actions/Level3Spells/Priest/SpiritGuardians/BP_SpiritGuardiansAoE.BP_SpiritGuardiansAoE_C" (Transformation|GetActorLocation SourceCharacter) SourceCharacter))
  (Transformation|AttachActorToActor _returnvalue SourceCharacter "center_of_mass" "KeepRelative" "KeepRelative" "KeepRelative" false)
  (EventDispatchers|BindEventtoOnAreaEntered _returnvalue (EventDispatchers|CreateEvent :!event Custom|DealDamage)))

(fn GetDescription
  (params (Caster :type BP%20Game%20Character%20Object%20Reference) (PlayerData :type ST%20Player%20Data%20Structure))
  (return "Summon spirit guardians that fly around you dealing damage to any enemy"))