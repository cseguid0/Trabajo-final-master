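; Vampiric Touch is a level 3 spell action that damages a target and heals the caster.
; AttackRoll makes a d20 ability check with a stat modifier and the supplied roll modifier against the target's AC.
; On a hit, DoAction rolls 3d6, doubling the dice on a critical, then deals that total as damage and passes the same amount to the caster as healing.
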(fn AttackRoll
  (params (Character :type BP%20Game%20Character%20Object%20Reference) (Target :type BP%20Game%20Character%20Object%20Reference) (RollMod :type Integer) (AdvantageModifier :type Integer))
  (bind _ac (Variables|/Game/Actors/Characters/BP_GameCharacter.BP_GameCharacter_C|GetAC Target))
  (bind (_success _critical _result _diceresult) (Utilities|AbilityCheck Character RollMod 0 0 0 0 0 1 0 (Utilities|Array|MakeArray "NewEnumerator3") "NewEnumerator0" 0 _ac))
  (return _success _critical _result _diceresult _ac AdvantageModifier))

(fn DoAction
  (params (SourceCharacter :type BP%20Game%20Character%20Object%20Reference) (TargetCharacter :type BP%20Game%20Character%20Object%20Reference) (TargetLocation :type Vector :default "0, 0, 0") (AttackRollSuccess :type Boolean) (AttackRollCritical :type Boolean))
  (if AttackRollSuccess
    (bind _roll (Default|Roll (Utilities|GetDice) SourceCharacter 0 0 (Math|Integer|SelectInt 6 3 AttackRollCritical) 0 0 0 0 0 "NewEnumerator0" "NewEnumerator0"))
    (Default|ReceiveDamage TargetCharacter _roll self SourceCharacter)
    (Default|ReceiveHealing SourceCharacter _roll)))

(fn GetDescription
  (params (Caster :type BP%20Game%20Character%20Object%20Reference) (PlayerData :type ST%20Player%20Data%20Structure))
  (return "Deals 3d6 points of damage. Heal yourself the same amount"))