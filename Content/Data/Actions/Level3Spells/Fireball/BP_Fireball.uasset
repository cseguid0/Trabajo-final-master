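; Level 3 Fireball spell action: throws a projectile at a location that explodes into an area of effect.
; DoAction spawns a fake target actor at the location and launches the projectile at it, binding to its target-reached event.
; On arrival, the fake target is destroyed and a spawned AoE triggers DealDamage.
; Each character hit takes 8d6 damage, halved on a successful save against the caster's spell DC.
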(event Custom|TargetReached
  (params (ProjectileSource :type BP%20Game%20Character%20Object%20Reference) (ProjectileTarget :type BP%20Game%20Character%20Object%20Reference) (Critical :type Boolean))
  (bind _asbp_game_instance (Utilities|Casting|CastToBP_GameInstance (Game|GetGameInstance ProjectileSource)))
  (bind _returnvalue (Default|SpawnAoE _asbp_game_instance "/Game/Data/Actions/Level3Spells/Fireball/BP_FireballAoE.BP_FireballAoE_C" (Transformation|GetActorLocation ProjectileTarget) ProjectileSource))
  (Actor|DestroyActor ProjectileTarget)
  (Default|Trigger _returnvalue (delegate Custom|DealDamage)))

(event Custom|DealDamage
  (params (Source :type BP%20Game%20Character%20Object%20Reference) (GameCharacter :type BP%20Game%20Character%20Object%20Reference))
  (bind _self self)
  (bind _success (Utilities|AbilitySave GameCharacter "NewEnumerator1" (Utilities|GetSpellSaveThrowDifficulty Source "NewEnumerator3")))
  (bind _roll (Default|Roll (Utilities|GetDice) 0 0 0 8 0 0 0 0 0 "NewEnumerator0" "NewEnumerator0"))
  (if _success
    (Default|ReceiveDamage GameCharacter (/ _roll 2) _self Source)
    (else
      (Default|ReceiveDamage GameCharacter _roll _self Source))))

(fn GetDescription
  (params (Caster :type BP%20Game%20Character%20Object%20Reference) (PlayerData :type ST%20Player%20Data%20Structure))
  (return "Throw a fireball that explodes over its target. Characters in the area receive 8d6 points of damage. If they succed a DEX save, they recibe half damage"))

(fn DoAction
  (params (SourceCharacter :type BP%20Game%20Character%20Object%20Reference) (TargetCharacter :type BP%20Game%20Character%20Object%20Reference) (TargetLocation :type Vector :default "0, 0, 0") (AttackRollSuccess :type Boolean) (AttackRollCritical :type Boolean))
  (bind _asbp_game_instance (Utilities|Casting|CastToBP_GameInstance (Game|GetGameInstance SourceCharacter)))
  (bind _character (Default|SpawnFakeTarget _asbp_game_instance TargetLocation))
  (bind _returnvalue (Default|SpawnProjectile _asbp_game_instance "/Game/Data/Actions/Level3Spells/Fireball/BP_FireballProjectile.BP_FireballProjectile_C" (Transformation|GetActorLocation SourceCharacter) SourceCharacter _character SourceCharacter false SourceCharacter))
  (EventDispatchers|BindEventtoOnTargetReached _returnvalue (EventDispatchers|CreateEvent :!event Custom|TargetReached)))