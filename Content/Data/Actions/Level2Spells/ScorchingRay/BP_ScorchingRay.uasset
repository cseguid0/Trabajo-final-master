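; Scorching Ray is a level 2 spell action that launches three fire beams at one target, each resolving its own hit and damage.
; The first beam uses the attack result passed into DoAction, while the other two call AttackRoll, a d20 ability check against target AC.
; Each hit deals 2d6 damage, doubled to 4d6 on a critical.
; AttackRoll returns its advantage modifier without applying it to the check.
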(fn DoAction
  (params (SourceCharacter :type BP%20Game%20Character%20Object%20Reference) (TargetCharacter :type BP%20Game%20Character%20Object%20Reference) (TargetLocation :type Vector :default "0, 0, 0") (AttackRollSuccess :type Boolean) (AttackRollCritical :type Boolean))
  (Utilities|FlowControl|Sequence
    (:then_0
      (if AttackRollSuccess
        (bind _roll (Default|Roll (Utilities|GetDice) 0 0 0 (Math|Integer|SelectInt 4 2 AttackRollCritical) 0 0 0 0 0 "NewEnumerator0" "NewEnumerator0"))
        (Default|ReceiveDamage TargetCharacter _roll self SourceCharacter)))
    (:then_1
      (bind (_success _critical) (CallFunction|AttackRoll SourceCharacter TargetCharacter))
      (if _success
        (bind _roll_2 (Default|Roll (Utilities|GetDice) 0 0 0 (Math|Integer|SelectInt 4 2 _critical) 0 0 0 0 0 "NewEnumerator0" "NewEnumerator0"))
        (Default|ReceiveDamage TargetCharacter _roll_2 self SourceCharacter)))
    (:then_2
      (bind (_success_2 _critical_2) (CallFunction|AttackRoll SourceCharacter TargetCharacter))
      (if _success_2
        (bind _roll_3 (Default|Roll (Utilities|GetDice) 0 0 0 (Math|Integer|SelectInt 4 2 _critical_2) 0 0 0 0 0 "NewEnumerator0" "NewEnumerator0"))
        (Default|ReceiveDamage TargetCharacter _roll_3 self SourceCharacter)))))

(fn GetDescription
  (params (Caster :type BP%20Game%20Character%20Object%20Reference) (PlayerData :type ST%20Player%20Data%20Structure))
  (return "Launch 3 fire beams at the target"))

(fn AttackRoll
  (params (Character :type BP%20Game%20Character%20Object%20Reference) (Target :type BP%20Game%20Character%20Object%20Reference) (RollMod :type Integer) (AdvantageModifier :type Integer))
  (bind _ac (Variables|/Game/Actors/Characters/BP_GameCharacter.BP_GameCharacter_C|GetAC Target))
  (bind (_success _critical _result _diceresult) (Utilities|AbilityCheck Character RollMod 0 0 0 0 0 1 0 (Utilities|Array|MakeArray "NewEnumerator3") "NewEnumerator0" 0 _ac))
  (return _success _critical _result _diceresult _ac AdvantageModifier))