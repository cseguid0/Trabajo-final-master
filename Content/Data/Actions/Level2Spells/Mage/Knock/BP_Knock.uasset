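; Knock is a level 2 Mage spell action that opens a locked chest.
; Targeting sphere-traces around the caster on the Visibility channel, accepting only BP_Chest actors within the spell's Range, or the caster's InteractionRange when Range is zero.
; Casting notifies the caster's passives in reverse order, pays the cost, then sets the chest's IsOpen flag directly.
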(event EventCast
  (params (SourceCharacter :type BP%20Game%20Character%20Object%20Reference) (TargetCharacter :type Actor%20Object%20Reference) (TargetLocation :type Vector :default "0, 0, 0"))
  (bind _arrayelement (Utilities|Array|ReverseforEachLoop (Variables|/Game/Actors/Characters/BP_GameCharacter.BP_GameCharacter_C|GetPassives SourceCharacter))
    (:LoopBody
      (Class|BPIonCastingTrigger|OnCasting(Message) _arrayelement SourceCharacter self))
    (:Completed
      (CallFunction|PayCost SourceCharacter)
      (bind _asbp_chest (Utilities|Casting|CastToBP_Chest TargetCharacter))
      (Variables|/Game/Actors/Containers/BP_Container.BP_Container_C|SetisOpen _asbp_chest true))))

(fn GetValidTargets
  (params (SourceCharacter :type BP%20Game%20Character%20Object%20Reference))
  (bind _returnvalue (Transformation|GetActorLocation SourceCharacter))
  (bind _range (Variables|Default|GetRange))
  (bind _range_2 (Variables|Default|GetRange))
  (bind _outhits (Collision|MultiSphereTraceByChannel SourceCharacter _returnvalue (+ _returnvalue "0.000000,0.000000,0.010000") (Math|Float|SelectFloat (Variables|/Game/Actors/Characters/BP_GameCharacter.BP_GameCharacter_C|GetInteractionRange SourceCharacter) (Math|Conversions|ToFloat(Integer) _range) (== _range 0)) "TraceTypeQuery1" false 0 "None" false))
  (for _array_element _outhits
    (bind _asbp_chest (Utilities|Casting|CastToBP_Chest (.HitActor (Collision|BreakHitResult _array_element))))
    (if (<= (Transformation|GetDistanceTo SourceCharacter _asbp_chest) (Math|Float|SelectFloat (Variables|/Game/Actors/Characters/BP_GameCharacter.BP_GameCharacter_C|GetInteractionRange SourceCharacter) (Math|Conversions|ToFloat(Integer) _range_2) (== _range_2 0)))
      (Utilities|Array|Add (LocalVariables|GetValidTargets) _asbp_chest)))
  (return (LocalVariables|GetValidTargets)))

(fn CheckTargetIsValid
  (params (SourceCharacter :type BP%20Game%20Character%20Object%20Reference) (Target :type Actor%20Object%20Reference) (TargetLocation :type Vector :default "0, 0, 0"))
  (bind _range (Variables|Default|GetRange))
  (bind _asbp_chest (Utilities|Casting|CastToBP_Chest Target)
    (:then
      (return (<= (Transformation|GetDistanceTo SourceCharacter _asbp_chest) (Math|Float|SelectFloat (Variables|/Game/Actors/Characters/BP_GameCharacter.BP_GameCharacter_C|GetInteractionRange SourceCharacter) (Math|Conversions|ToFloat(Integer) _range) (== _range 0)))))
    (:CastFailed
      (return false))))

(fn GetDescription
  (params (Caster :type BP%20Game%20Character%20Object%20Reference) (PlayerData :type ST%20Player%20Data%20Structure))
  (return "Open a locked chest"))