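; Level 2 spell action Cloud of Daggers, which creates a persistent damage area at the target location.
; DoAction has the game instance spawn a BP_CloudOfDaggersAoE with the caster as source, then binds an event to its area-entered callback.
; DealDamage rolls d4 dice and applies the result to a character as damage from this spell.
; The five-turn duration appears here only in the description text.
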(event Custom|DealDamage
  (params (Character :type BP%20Game%20Character%20Object%20Reference) (Source :type BP%20Game%20Character%20Object%20Reference))
  (bind _roll (Default|Roll (Utilities|GetDice) 0 0 4 0 0 0 0 0 0 "NewEnumerator0" "NewEnumerator0"))
  (Default|ReceiveDamage Character _roll self Source))

(fn DoAction
  (params (SourceCharacter :type BP%20Game%20Character%20Object%20Reference) (TargetCharacter :type BP%20Game%20Character%20Object%20Reference) (TargetLocation :type Vector :default "0, 0, 0") (AttackRollSuccess :type Boolean) (AttackRollCritical :type Boolean))
  (bind _asbp_game_instance (Utilities|Casting|CastToBP_GameInstance (Game|GetGameInstance SourceCharacter)))
  (bind _returnvalue (Default|SpawnPersistentAoE _asbp_game_instance "/Game/Data/Actions/Level2Spells/CloudOfDaggers/BP_CloudOfDaggersAoE.BP_CloudOfDaggersAoE_C" TargetLocation SourceCharacter))
  (EventDispatchers|BindEventtoOnAreaEntered _returnvalue (EventDispatchers|CreateEvent :!event Custom|DealDamage)))

(fn GetDescription
  (params (Caster :type BP%20Game%20Character%20Object%20Reference) (PlayerData :type ST%20Player%20Data%20Structure))
  (return "Generate a cloud of daggers that deals 4d4 to any character inside. It lasts 5 turns"))