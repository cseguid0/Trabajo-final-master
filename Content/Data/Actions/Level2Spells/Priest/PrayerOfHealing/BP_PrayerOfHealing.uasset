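; Priest level 2 spell action Prayer of Healing, which heals allies around the caster.
; DoAction runs a sphere overlap at the caster for game character pawns, skipping any BP_HostileNPC.
; Each remaining character receives its own dice roll of 2d8 plus a stat modifier, described as WIS, through ReceiveHealing.
; The target and attack roll inputs are unused.
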(fn DoAction
  (params (SourceCharacter :type BP%20Game%20Character%20Object%20Reference) (TargetCharacter :type BP%20Game%20Character%20Object%20Reference) (TargetLocation :type Vector :default "0, 0, 0") (AttackRollSuccess :type Boolean) (AttackRollCritical :type Boolean))
  (bind _outactors (Collision|SphereOverlapActors SourceCharacter (Transformation|GetActorLocation SourceCharacter) 9e+02 (Utilities|Array|MakeArray "ObjectTypeQuery3") "/Game/Actors/Characters/BP_GameCharacter.BP_GameCharacter_C"))
  (for _array_element _outactors
    (Utilities|Casting|CastToBP_HostileNPC _array_element
      (:CastFailed
        (bind _asbp_game_character (Utilities|Casting|CastToBP_GameCharacter _array_element))
        (bind _roll (Default|Roll (Utilities|GetDice) SourceCharacter 0 0 0 2 0 0 0 0 (Utilities|Array|MakeArray "NewEnumerator4") "NewEnumerator0"))
        (Default|ReceiveHealing _asbp_game_character _roll)))))

(fn GetDescription
  (params (Caster :type BP%20Game%20Character%20Object%20Reference) (PlayerData :type ST%20Player%20Data%20Structure))
  (return "Heals 2d8 + {WIS} to your close allies around you"))