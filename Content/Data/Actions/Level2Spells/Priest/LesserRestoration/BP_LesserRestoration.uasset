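; Lesser Restoration is a level 2 Priest spell action that restores two Level 1 Spell Points to its caster.
; DoAction reads the caster's current and maximum values from the resource maps, treating missing entries as zero, and writes back the increased value capped at the maximum.
; The target, location and attack roll inputs are unused, and GetDescription returns fixed text.
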(fn DoAction
  (params (SourceCharacter :type BP%20Game%20Character%20Object%20Reference) (TargetCharacter :type BP%20Game%20Character%20Object%20Reference) (TargetLocation :type Vector :default "0, 0, 0") (AttackRollSuccess :type Boolean) (AttackRollCritical :type Boolean))
  (bind _resources (Variables|/Game/Actors/Characters/BP_GameCharacter.BP_GameCharacter_C|GetResources SourceCharacter))
  (bind _maxresources (Variables|/Game/Actors/Characters/BP_GameCharacter.BP_GameCharacter_C|GetMaxResources SourceCharacter))
  (bind (_value _returnvalue) (Utilities|Map|Find _resources "NewEnumerator3"))
  (bind (_value_2 _returnvalue_2) (Utilities|Map|Find _maxresources "NewEnumerator3"))
  (Utilities|Map|Add _resources "NewEnumerator3" (Math|Integer|Min(Integer) (+ (Math|Integer|SelectInt _value 0 _returnvalue) 2) (Math|Integer|SelectInt _value_2 0 _returnvalue_2))))

(fn GetDescription
  (params (Caster :type BP%20Game%20Character%20Object%20Reference) (PlayerData :type ST%20Player%20Data%20Structure))
  (return "Restores 2 Level 1 Spell Points"))