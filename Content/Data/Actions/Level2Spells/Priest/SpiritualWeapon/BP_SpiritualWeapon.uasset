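; Spiritual Weapon, a level 2 Priest spell action that summons a weapon to boost the caster's melee damage.
; DoAction applies the DA_SpiritualWeaponEffect passive to the source character, ignoring target and attack roll inputs.
; GetDescription builds tooltip text showing 1d8 plus the Wisdom modifier, read from the caster's stats, or from PlayerData when no valid caster exists.
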(fn DoAction
  (params (SourceCharacter :type BP%20Game%20Character%20Object%20Reference) (TargetCharacter :type BP%20Game%20Character%20Object%20Reference) (TargetLocation :type Vector :default "0, 0, 0") (AttackRollSuccess :type Boolean) (AttackRollCritical :type Boolean))
  (Default|AddPassive SourceCharacter "/Game/Data/Effects/SpiritualWeaponEffect/DA_SpiritualWeaponEffect.DA_SpiritualWeaponEffect"))

(fn GetDescription
  (params (Caster :type BP%20Game%20Character%20Object%20Reference) (PlayerData :type ST%20Player%20Data%20Structure))
  (bind _stats (Utilities|Struct|BreakST_PlayerData PlayerData))
  (bind _stats_2 (Variables|/Game/Actors/Characters/BP_GameCharacter.BP_GameCharacter_C|GetStats Caster))
  (bind (_value _returnvalue) (Utilities|Map|Find _stats "NewEnumerator4"))
  (bind (_value_2 _returnvalue_2) (Utilities|Map|Find _stats_2 "NewEnumerator4"))
  (Utilities|IsValid Caster
    (:Is%20Valid
      (return (Utilities|Text|FormatText "Summon a weapon that adds 1d8 + {WIS} to your melee damage" (Utilities|CalculateStatModifier (Math|Integer|SelectInt _value_2 0 _returnvalue_2)))))
    (:Is%20Not%20Valid
      (return (Utilities|Text|FormatText "Summon a weapon that adds 1d8 + {WIS} to your melee damage" (Utilities|CalculateStatModifier (Math|Integer|SelectInt _value 0 _returnvalue)))))))