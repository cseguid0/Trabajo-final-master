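; Basic attack action for a D&D-style combat system, striking with the right-hand weapon or unarmed when that slot is empty.
; AttackRoll tests against target AC using the weapon's roll or a d20 ability check, with advantage from gameplay tags.
; DoAction applies weapon or unarmed damage plus stat modifier, accounting for criticals.
; An AdditionalAttack passive entry bypasses the parent's cost and availability check.
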(fn GetDescription
  (params (Caster :type BP%20Game%20Character%20Object%20Reference) (PlayerData :type ST%20Player%20Data%20Structure))
  (bind (_maxhp _hp _ac _stats _proficiencies _passives _resources _armorslot _rightweaponslot) (Utilities|Struct|BreakST_PlayerData PlayerData))
  (bind _returnvalue (Utilities|IsValid Caster))
  (bind _rightweaponslot_2 (Variables|/Game/Actors/Characters/BP_GameCharacter.BP_GameCharacter_C|GetRightWeaponSlot Caster))
  (bind _stats_2 (Variables|/Game/Actors/Characters/BP_GameCharacter.BP_GameCharacter_C|GetStats Caster))
  (bind _returnvalue_2 (Utilities|SelectObject _rightweaponslot_2 _rightweaponslot _returnvalue))
  (bind (_value _returnvalue_3) (Utilities|Map|Find _stats_2 "NewEnumerator0"))
  (bind (_value_2 _returnvalue_4) (Utilities|Map|Find _stats "NewEnumerator0"))
  (Utilities|IsValid _returnvalue_2
    (:Is%20Valid
      (bind _asbp_weapon (Utilities|Casting|CastToBP_Weapon _returnvalue_2))
      (bind _description (Default|GetDamageDescription _asbp_weapon))
      (return (Utilities|Text|FormatText "Attack with your right hand weapon dealing {dmg} damage. If you dont have a weapon it is an unarmed strike" _description)))
    (:Is%20Not%20Valid
      (return (Utilities|Text|FormatText "Attack with your right hand weapon dealing {dmg} damage. If you dont have a weapon it is an unarmed strike" (+ (Math|Integer|SelectInt (Math|Integer|SelectInt _value 0 _returnvalue_3) (Math|Integer|SelectInt _value_2 0 _returnvalue_4) _returnvalue) 1))))))

(fn DoAction
  (params (SourceCharacter :type BP%20Game%20Character%20Object%20Reference) (TargetCharacter :type BP%20Game%20Character%20Object%20Reference) (TargetLocation :type Vector :default "0, 0, 0") (AttackRollSuccess :type Boolean) (AttackRollCritical :type Boolean))
  (bind _rightweaponslot (Variables|/Game/Actors/Characters/BP_GameCharacter.BP_GameCharacter_C|GetRightWeaponSlot SourceCharacter))
  (bind _stats (Variables|/Game/Actors/Characters/BP_GameCharacter.BP_GameCharacter_C|GetStats SourceCharacter))
  (bind (_value _returnvalue) (Utilities|Map|Find _stats "NewEnumerator0"))
  (bind _returnvalue_2 (Math|Integer|SelectInt _value 0 _returnvalue))
  (bind _modifier (Utilities|CalculateStatModifier _returnvalue_2))
  (bind _returnvalue_3 (+ _modifier 1))
  (if AttackRollSuccess
    (Utilities|IsValid _rightweaponslot
      (:Is%20Valid
        (bind _statmodifier (Default|GetStatMod _rightweaponslot SourceCharacter))
        (bind _damage (Default|RollDamage _rightweaponslot AttackRollCritical))
        (Default|ReceiveDamage TargetCharacter (+ _damage (Utilities|CalculateStatModifier (Math|Integer|SelectInt (.Value (Utilities|Map|Find (Variables|/Game/Actors/Characters/BP_GameCharacter.BP_GameCharacter_C|GetStats SourceCharacter) _statmodifier)) 0 (.ReturnValue (Utilities|Map|Find (Variables|/Game/Actors/Characters/BP_GameCharacter.BP_GameCharacter_C|GetStats SourceCharacter) _statmodifier))))) self SourceCharacter))
      (:Is%20Not%20Valid
        (Default|ReceiveDamage TargetCharacter (Math|Integer|SelectInt (* _returnvalue_3 2) _returnvalue_3 AttackRollCritical) self SourceCharacter)))))

(fn AttackRoll
  (params (Character :type BP%20Game%20Character%20Object%20Reference) (Target :type BP%20Game%20Character%20Object%20Reference) (RollMod :type Integer) (AdvantageModifier :type Integer))
  (bind _returnvalue (GameplayTags|MakeLiteralGameplayTagContainer "(GameplayTags=((TagName=\"Disadvantage.ReceiveAttack\")))"))
  (bind _returnvalue_2 (GameplayTags|MakeLiteralGameplayTagContainer "(GameplayTags=((TagName=\"Advantage.ReceiveAttack\")))"))
  (bind _returnvalue_3 (GameplayTags|MakeLiteralGameplayTagContainer "(GameplayTags=((TagName=\"Advantage.Attack\")))"))
  (bind _returnvalue_4 (GameplayTags|MakeLiteralGameplayTagContainer "(GameplayTags=((TagName=\"Disadvantage.Attack\")))"))
  (bind _rightweaponslot (Variables|/Game/Actors/Characters/BP_GameCharacter.BP_GameCharacter_C|GetRightWeaponSlot Character))
  (bind _ac (Variables|/Game/Actors/Characters/BP_GameCharacter.BP_GameCharacter_C|GetAC Target))
  (bind _ac_2 (Variables|/Game/Actors/Characters/BP_GameCharacter.BP_GameCharacter_C|GetAC Target))
  (bind _advantage (Utilities|GetAdvantage Character _returnvalue_3 _returnvalue_4 Target _returnvalue_2 _returnvalue))
  (bind _returnvalue_5 (+ AdvantageModifier _advantage))
  (Utilities|IsValid _rightweaponslot
    (:Is%20Valid
      (bind (_attack _diceresult _critical) (Default|RollAttack _rightweaponslot Character _returnvalue_5))
      (return (>= (+ _attack RollMod) _ac) _critical (+ _attack RollMod) _diceresult _ac _returnvalue_5))
    (:Is%20Not%20Valid
      (bind (_success _critical_2 _result _diceresult_2) (Utilities|AbilityCheck Character RollMod 0 0 0 0 0 1 0 (Utilities|Array|MakeArray "NewEnumerator0") "NewEnumerator0" _returnvalue_5 _ac_2))
      (return _success _critical_2 _result _diceresult_2 _ac_2 _returnvalue_5))))

(fn PayCost
  (params (Character :type BP%20Game%20Character%20Object%20Reference))
  (if (not (.ReturnValue (Utilities|Map|Find (Variables|/Game/Actors/Characters/BP_GameCharacter.BP_GameCharacter_C|GetPassivesData Character) "AdditionalAttack")))
    (|CallParentFunction Character)))

(fn CheckAvailability
  (params (SourceCharacter :type BP%20Game%20Character%20Object%20Reference))
  (if (.ReturnValue (Utilities|Map|Find (Variables|/Game/Actors/Characters/BP_GameCharacter.BP_GameCharacter_C|GetPassivesData SourceCharacter) "AdditionalAttack"))
    (return true)
    (else
      (bind _availability (|CallParentFunction SourceCharacter))
      (return _availability))))