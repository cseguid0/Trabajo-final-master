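; Action Blueprint for Action Surge, an ability that gives the character back one action point and can be used once per rest.
; DoAction sets an ActionSurge_Spent flag in the character's passive data, increments the first resource type and adds the Action Surge Recovery passive.
; CheckAvailability extends the parent check by requiring that spent flag to be absent or zero.
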(fn DoAction
  (params (SourceCharacter :type BP%20Game%20Character%20Object%20Reference) (TargetCharacter :type BP%20Game%20Character%20Object%20Reference) (TargetLocation :type Vector :default "0, 0, 0") (AttackRollSuccess :type Boolean) (AttackRollCritical :type Boolean))
  (bind _resources (Variables|/Game/Actors/Characters/BP_GameCharacter.BP_GameCharacter_C|GetResources SourceCharacter))
  (bind (_value _returnvalue) (Utilities|Map|Find _resources "NewEnumerator0"))
  (Utilities|Map|Add (Variables|/Game/Actors/Characters/BP_GameCharacter.BP_GameCharacter_C|GetPassivesData SourceCharacter) "ActionSurge_Spent" 1)
  (Utilities|Map|Add _resources "NewEnumerator0" (+ (Math|Integer|SelectInt _value 0 _returnvalue) 1))
  (Default|AddPassive SourceCharacter "/Game/Data/Effects/ActionSurgeRecovery/DA_ActionSurgeRecovery.DA_ActionSurgeRecovery"))

(fn GetDescription
  (params (Caster :type BP%20Game%20Character%20Object%20Reference) (PlayerData :type ST%20Player%20Data%20Structure))
  (return "Recover 1 action point. Can only be used once per rest"))

(fn CheckAvailability
  (params (SourceCharacter :type BP%20Game%20Character%20Object%20Reference))
  (bind _passivesdata (Variables|/Game/Actors/Characters/BP_GameCharacter.BP_GameCharacter_C|GetPassivesData SourceCharacter))
  (bind (_value _returnvalue) (Utilities|Map|Find _passivesdata "ActionSurge_Spent"))
  (bind _availability (|CallParentFunction SourceCharacter))
  (return (and _availability (== (Math|Integer|SelectInt _value 0 _returnvalue) 0))))