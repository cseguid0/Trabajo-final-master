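; Ranged attack action for a tabletop-style combat system, using the character's equipped ranged weapon.
; The attack roll adds advantage from gameplay tags on caster and target and succeeds on meeting the target's AC or rolling a critical.
; On a hit it deals weapon damage plus the weapon's stat modifier.
; It requires a ranged weapon, and an AdditionalAttack passive bypasses the parent's availability check and cost.
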(fn DoAction
  (params (SourceCharacter :type BP%20Game%20Character%20Object%20Reference) (TargetCharacter :type BP%20Game%20Character%20Object%20Reference) (TargetLocation :type Vector :default "0, 0, 0") (AttackRollSuccess :type Boolean) (AttackRollCritical :type Boolean))
  (bind _rangedweaponslot (Variables|/Game/Actors/Characters/BP_GameCharacter.BP_GameCharacter_C|GetRangedWeaponSlot SourceCharacter))
  (bind _stats (Variables|/Game/Actors/Characters/BP_GameCharacter.BP_GameCharacter_C|GetStats SourceCharacter))
  (bind _statmodifier (Default|GetStatMod _rangedweaponslot SourceCharacter))
  (bind (_value _returnvalue) (Utilities|Map|Find _stats _statmodifier))
  (if AttackRollSuccess
    (bind _damage (Default|RollDamage _rangedweaponslot SourceCharacter AttackRollCritical))
    (Default|ReceiveDamage TargetCharacter (+ _damage (Utilities|CalculateStatModifier (Math|Integer|SelectInt _value 0 _returnvalue))) self SourceCharacter)))

(fn GetDescription
  (params (Caster :type BP%20Game%20Character%20Object%20Reference) (PlayerData :type ST%20Player%20Data%20Structure))
  (bind _rangedweaponslot (Utilities|Struct|BreakST_PlayerData PlayerData))
  (bind _rangedweaponslot_2 (Variables|/Game/Actors/Characters/BP_GameCharacter.BP_GameCharacter_C|GetRangedWeaponSlot Caster))
  (Utilities|IsValid Caster
    (:Is%20Valid
      (Utilities|IsValid _rangedweaponslot_2
        (:Is%20Valid
          (return (Utilities|Text|FormatText "Attack with your ranged weapon dealing {dmg} points of damage" (Default|GetDamageDescription _rangedweaponslot_2))))
        (:Is%20Not%20Valid
          _)))
    (:Is%20Not%20Valid
      (Utilities|IsValid _rangedweaponslot
        (:Is%20Valid
          (return (Utilities|Text|FormatText "Attack with your ranged weapon dealing {dmg} points of damage" (Default|GetDamageDescription _rangedweaponslot))))
        (:Is%20Not%20Valid
          _))))
  (return "Attack with your ranged weapon"))

(fn CheckAvailability
  (params (SourceCharacter :type BP%20Game%20Character%20Object%20Reference))
  (bind _rangedweaponslot (Variables|/Game/Actors/Characters/BP_GameCharacter.BP_GameCharacter_C|GetRangedWeaponSlot SourceCharacter))
  (bind _returnvalue (Utilities|IsValid _rangedweaponslot))
  (if (.ReturnValue (Utilities|Map|Find (Variables|/Game/Actors/Characters/BP_GameCharacter.BP_GameCharacter_C|GetPassivesData SourceCharacter) "AdditionalAttack"))
    (return _returnvalue)
    (else
      (bind _availability (|CallParentFunction SourceCharacter))
      (return (and _availability _returnvalue)))))

(fn AttackRoll
  (params (Character :type BP%20Game%20Character%20Object%20Reference) (Target :type BP%20Game%20Character%20Object%20Reference) (RollMod :type Integer) (AdvantageModifier :type Integer))
  (bind _returnvalue (GameplayTags|MakeLiteralGameplayTagContainer "(GameplayTags=((TagName=\"Disadvantage.ReceiveAttack\")))"))
  (bind _returnvalue_2 (GameplayTags|MakeLiteralGameplayTagContainer "(GameplayTags=((TagName=\"Advantage.ReceiveAttack\")))"))
  (bind _returnvalue_3 (GameplayTags|MakeLiteralGameplayTagContainer "(GameplayTags=((TagName=\"Advantage.Attack\")))"))
  (bind _returnvalue_4 (GameplayTags|MakeLiteralGameplayTagContainer "(GameplayTags=((TagName=\"Disadvantage.Attack\")))"))
  (bind _ac (Variables|/Game/Actors/Characters/BP_GameCharacter.BP_GameCharacter_C|GetAC Target))
  (bind _advantage (Utilities|GetAdvantage Character _returnvalue_3 _returnvalue_4 Target _returnvalue_2 _returnvalue))
  (bind _returnvalue_5 (+ AdvantageModifier _advantage))
  (bind (_attack _diceresult _critical) (Default|RollAttack (Variables|/Game/Actors/Characters/BP_GameCharacter.BP_GameCharacter_C|GetRangedWeaponSlot Character) Character _returnvalue_5))
  (return (or (>= (+ _attack RollMod) _ac) _critical) _critical (+ _attack RollMod) _diceresult _ac _returnvalue_5))

(fn PayCost
  (params (Character :type BP%20Game%20Character%20Object%20Reference))
  (if (not (.ReturnValue (Utilities|Map|Find (Variables|/Game/Actors/Characters/BP_GameCharacter.BP_GameCharacter_C|GetPassivesData Character) "AdditionalAttack")))
    (|CallParentFunction Character)))