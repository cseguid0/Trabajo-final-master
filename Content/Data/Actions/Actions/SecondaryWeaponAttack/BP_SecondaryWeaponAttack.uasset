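; Action asset for an off-hand attack or shield bash, available only when the character has a valid left weapon slot.
; The attack roll uses the left weapon plus tag-derived advantage from attacker and target, succeeding against target AC or on a critical.
; On a hit it applies the weapon's damage, plus optional 1d8 and stat-modifier bonuses gated by gameplay tags.
; The description shows the weapon's damage, using either the caster or player data.
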(fn CheckAvailability
  (params (SourceCharacter :type BP%20Game%20Character%20Object%20Reference))
  (bind _availability (|CallParentFunction SourceCharacter))
  (return (and _availability (Utilities|IsValid (Variables|/Game/Actors/Characters/BP_GameCharacter.BP_GameCharacter_C|GetLeftWeaponSlot SourceCharacter)))))

(fn DoAction
  (params (SourceCharacter :type BP%20Game%20Character%20Object%20Reference) (TargetCharacter :type BP%20Game%20Character%20Object%20Reference) (TargetLocation :type Vector :default "0, 0, 0") (AttackRollSuccess :type Boolean) (AttackRollCritical :type Boolean))
  (bind _gameplaytags (Variables|/Game/Actors/Characters/BP_GameCharacter.BP_GameCharacter_C|GetGameplayTags SourceCharacter))
  (bind _stats (Variables|/Game/Actors/Characters/BP_GameCharacter.BP_GameCharacter_C|GetStats SourceCharacter))
  (bind (_value _returnvalue) (Utilities|Map|Find _stats "NewEnumerator4"))
  (if AttackRollSuccess
    (bind _damage (Default|RollDamage (Variables|/Game/Actors/Characters/BP_GameCharacter.BP_GameCharacter_C|GetLeftWeaponSlot SourceCharacter) SourceCharacter AttackRollCritical))
    (Default|ReceiveDamage TargetCharacter (+ _damage (+ (Math|Integer|SelectInt (+ (Math|Random|RandomInteger 8) 1) 0 (GameplayTags|HasTag _gameplaytags "(TagName=\"Modifier.DamageRoll.+1d8\")")) (Math|Integer|SelectInt (Utilities|CalculateStatModifier (Math|Integer|SelectInt _value 0 _returnvalue)) 0 (GameplayTags|HasTag _gameplaytags "(TagName=\"Modifier.DamageRoll.WIS\")")))) self SourceCharacter)))

(fn GetDescription
  (params (Caster :type BP%20Game%20Character%20Object%20Reference) (PlayerData :type ST%20Player%20Data%20Structure))
  (bind _leftweaponslot (Utilities|Struct|BreakST_PlayerData PlayerData))
  (bind _leftweaponslot_2 (Variables|/Game/Actors/Characters/BP_GameCharacter.BP_GameCharacter_C|GetLeftWeaponSlot Caster))
  (Utilities|IsValid Caster
    (:Is%20Valid
      (Utilities|IsValid _leftweaponslot_2
        (:Is%20Valid
          (return (Utilities|Text|FormatText "Attack with your left hand weapon or do a shield bash dealing {dmg} damage" (Default|GetDamageDescription _leftweaponslot_2 Caster))))
        (:Is%20Not%20Valid
          _)))
    (:Is%20Not%20Valid
      (Utilities|IsValid _leftweaponslot
        (:Is%20Valid
          (return (Utilities|Text|FormatText "Attack with your left hand weapon or do a shield bash dealing {dmg} damage" (Default|GetDamageDescription _leftweaponslot))))
        (:Is%20Not%20Valid
          _))))
  (return "Attack with your left hand weapon or do a shield bash"))

(fn AttackRoll
  (params (Character :type BP%20Game%20Character%20Object%20Reference) (Target :type BP%20Game%20Character%20Object%20Reference) (RollMod :type Integer) (AdvantageModifier :type Integer))
  (bind _returnvalue (GameplayTags|MakeLiteralGameplayTagContainer "(GameplayTags=((TagName=\"Disadvantage.ReceiveAttack\")))"))
  (bind _returnvalue_2 (GameplayTags|MakeLiteralGameplayTagContainer "(GameplayTags=((TagName=\"Advantage.ReceiveAttack\")))"))
  (bind _returnvalue_3 (GameplayTags|MakeLiteralGameplayTagContainer "(GameplayTags=((TagName=\"Advantage.Attack\")))"))
  (bind _returnvalue_4 (GameplayTags|MakeLiteralGameplayTagContainer "(GameplayTags=((TagName=\"Disadvantage.Attack\")))"))
  (bind _ac (Variables|/Game/Actors/Characters/BP_GameCharacter.BP_GameCharacter_C|GetAC Target))
  (bind _advantage (Utilities|GetAdvantage Character _returnvalue_3 _returnvalue_4 Target _returnvalue_2 _returnvalue))
  (bind _returnvalue_5 (+ AdvantageModifier _advantage))
  (bind (_attack _diceresult _critical) (Default|RollAttack (Variables|/Game/Actors/Characters/BP_GameCharacter.BP_GameCharacter_C|GetLeftWeaponSlot Character) Character _returnvalue_5))
  (return (or (>= (+ _attack RollMod) _ac) _critical) _critical (+ _attack RollMod) _diceresult _ac _returnvalue_5))