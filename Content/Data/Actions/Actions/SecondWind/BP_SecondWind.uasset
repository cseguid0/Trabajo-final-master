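; Second Wind action that heals the caster for 1d10 plus level, usable once per rest.
; DoAction sets a SecondWind_Spent entry in the character's PassivesData, rolls and applies the healing, then adds the DA_SecondWindRecovery passive.
; CheckAvailability requires the parent check to pass and that spent entry to be absent or zero.
; GetDescription takes the level from the caster, or from PlayerData when no caster is valid.
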(fn GetDescription
  (params (Caster :type BP%20Game%20Character%20Object%20Reference) (PlayerData :type ST%20Player%20Data%20Structure))
  (bind _returnvalue (Utilities|Text|MakeLiteralText "Heals 1d10 + {0}. Can only be used once per rest"))
  (Utilities|IsValid Caster
    (:Is%20Valid
      (return (Utilities|Text|FormatText _returnvalue (Variables|/Game/Actors/Characters/BP_GameCharacter.BP_GameCharacter_C|GetLevel Caster))))
    (:Is%20Not%20Valid
      (return (Utilities|Text|FormatText _returnvalue (.Level (Utilities|Struct|BreakST_PlayerData PlayerData)))))))

(fn DoAction
  (params (SourceCharacter :type BP%20Game%20Character%20Object%20Reference) (TargetCharacter :type BP%20Game%20Character%20Object%20Reference) (TargetLocation :type Vector :default "0, 0, 0") (AttackRollSuccess :type Boolean) (AttackRollCritical :type Boolean))
  (Utilities|Map|Add (Variables|/Game/Actors/Characters/BP_GameCharacter.BP_GameCharacter_C|GetPassivesData SourceCharacter) "SecondWind_Spent" 1)
  (bind _roll (Default|Roll (Utilities|GetDice) SourceCharacter (Variables|/Game/Actors/Characters/BP_GameCharacter.BP_GameCharacter_C|GetLevel SourceCharacter) 0 0 0 1 0 0 0 "NewEnumerator0" "NewEnumerator0"))
  (Default|ReceiveHealing SourceCharacter _roll)
  (Default|AddPassive SourceCharacter "/Game/Data/Effects/SecondWindRecovery/DA_SecondWindRecovery.DA_SecondWindRecovery"))

(fn CheckAvailability
  (params (SourceCharacter :type BP%20Game%20Character%20Object%20Reference))
  (bind _passivesdata (Variables|/Game/Actors/Characters/BP_GameCharacter.BP_GameCharacter_C|GetPassivesData SourceCharacter))
  (bind (_value _returnvalue) (Utilities|Map|Find _passivesdata "SecondWind_Spent"))
  (bind _availability (|CallParentFunction SourceCharacter))
  (return (and _availability (== (Math|Integer|SelectInt _value 0 _returnvalue) 0))))