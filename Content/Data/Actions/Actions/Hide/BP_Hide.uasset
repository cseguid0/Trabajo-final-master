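; Hide action that lets a character toggle stealth on or off.
; Leaving stealth, or hiding with no observers, succeeds automatically.
; Otherwise each observer's d20 proficiency roll sets the difficulty for a separate ability check by the character, with advantage or disadvantage from DEX and Perception tags.
; Stealth toggles on only if the combined result across all observers is a success.
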(fn DoAction
  (params (SourceCharacter :type BP%20Game%20Character%20Object%20Reference) (TargetCharacter :type BP%20Game%20Character%20Object%20Reference) (TargetLocation :type Vector :default "0, 0, 0") (AttackRollSuccess :type Boolean) (AttackRollCritical :type Boolean))
  (bind _observers (Variables|/Game/Actors/Characters/BP_GameCharacter.BP_GameCharacter_C|GetObservers SourceCharacter))
  (if (GameplayTags|HasTag (Variables|/Game/Actors/Characters/BP_GameCharacter.BP_GameCharacter_C|GetGameplayTags SourceCharacter) "(TagName=\"Status.Stealth\")" true)
    (Default|ToggleStealth SourceCharacter :!label _label)
    (elif (> (Utilities|Array|Length _observers) 0)
      (for _array_element _observers
        (bind _roll (Default|Roll (Utilities|GetDice) _array_element 0 0 0 0 0 0 1 0 "NewEnumerator0" (Utilities|Array|MakeArray "NewEnumerator11")))
        (bind _success (Utilities|AbilityCheck SourceCharacter 0 0 0 0 0 0 0 0 (Utilities|Array|MakeArray "NewEnumerator1") (Utilities|Array|MakeArray "NewEnumerator16") (Utilities|GetAdvantage SourceCharacter (GameplayTags|MakeLiteralGameplayTagContainer "(GameplayTags=((TagName=\"Advantage.DEX\"),(TagName=\"Advantage.Stealth\")))") (GameplayTags|MakeLiteralGameplayTagContainer "(GameplayTags=((TagName=\"Disadvantage.DEX\"),(TagName=\"Disadvantage.Stealth\")))") _array_element (GameplayTags|MakeLiteralGameplayTagContainer "(GameplayTags=((TagName=\"Advantage.Perception\")))") (GameplayTags|MakeLiteralGameplayTagContainer "(GameplayTags=((TagName=\"Disadvantage.Perception\")))")) _roll))
        (LocalVariables|SetSuccess (and _success (LocalVariables|GetSuccess))))
      (if (LocalVariables|GetSuccess)
        (goto _label))
      (else
        (goto _label)))))

(fn GetDescription
  (params (Caster :type BP%20Game%20Character%20Object%20Reference) (PlayerData :type ST%20Player%20Data%20Structure))
  (return "Hide yourself from sight"))