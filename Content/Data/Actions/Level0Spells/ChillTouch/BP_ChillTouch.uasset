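; Chill Touch level 0 spell action that deals d8 damage and applies a healing negation passive on a hit.
; AttackRoll makes a d20 ability check against the target's AC, returning the advantage modifier without passing it into the check.
; DoAction rolls more dice above caster level 4, doubles them on a critical, then damages the target.
; GetDescription builds level-scaled tooltip text from the caster, falling back to player data.
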(fn DoAction
  (params (SourceCharacter :type BP%20Game%20Character%20Object%20Reference) (TargetCharacter :type BP%20Game%20Character%20Object%20Reference) (TargetLocation :type Vector :default "0, 0, 0") (AttackRollSuccess :type Boolean) (AttackRollCritical :type Boolean))
  (bind _level (Variables|/Game/Actors/Characters/BP_GameCharacter.BP_GameCharacter_C|GetLevel SourceCharacter))
  (bind _returnvalue (<= _level 4))
  (if AttackRollSuccess
    (bind _roll (Default|Roll (Utilities|GetDice) SourceCharacter 0 0 0 (Math|Integer|SelectInt (Math|Integer|SelectInt 2 4 _returnvalue) (Math|Integer|SelectInt 1 2 _returnvalue) AttackRollCritical) 0 0 0 0 "NewEnumerator0" "NewEnumerator0"))
    (Default|ReceiveDamage TargetCharacter _roll self SourceCharacter)
    (Default|AddPassive TargetCharacter "/Game/Data/Effects/HealingNegation/DA_HealingNegation.DA_HealingNegation")))

(fn GetDescription
  (params (Caster :type BP%20Game%20Character%20Object%20Reference) (PlayerData :type ST%20Player%20Data%20Structure))
  (bind _returnvalue (Utilities|Text|MakeLiteralText "Deal {0} points of damage and stops healing on the target for the next 2 turns"))
  (Utilities|IsValid Caster
    (:Is%20Valid
      (return (Utilities|Text|FormatText _returnvalue (Utilities|String|SelectText "1d8" "2d8" (<= (Variables|/Game/Actors/Characters/BP_GameCharacter.BP_GameCharacter_C|GetLevel Caster) 4)))))
    (:Is%20Not%20Valid
      (return (Utilities|Text|FormatText _returnvalue (Utilities|String|SelectText "1d8" "2d8" (<= (.Level (Utilities|Struct|BreakST_PlayerData PlayerData)) 4)))))))

(fn AttackRoll
  (params (Character :type BP%20Game%20Character%20Object%20Reference) (Target :type BP%20Game%20Character%20Object%20Reference) (RollMod :type Integer) (AdvantageModifier :type Integer))
  (bind _ac (Variables|/Game/Actors/Characters/BP_GameCharacter.BP_GameCharacter_C|GetAC Target))
  (bind (_success _critical _result _diceresult) (Utilities|AbilityCheck Character RollMod 0 0 0 0 0 1 0 (Utilities|Array|MakeArray "NewEnumerator3") "NewEnumerator0" 0 _ac))
  (return (or _success _critical) _critical _result _diceresult _ac AdvantageModifier))