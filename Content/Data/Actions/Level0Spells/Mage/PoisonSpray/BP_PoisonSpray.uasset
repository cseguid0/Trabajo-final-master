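; Level 0 Mage spell action Poison Spray, a single-target ranged attack that deals d12 damage.
; AttackRoll makes a d20 ability check against the target's AC, returning AdvantageModifier without applying it to the roll.
; On a hit, DoAction spawns a projectile through the game instance and binds its target-reached event for damage.
; Damage dice double above caster level 4 and again on a critical, and the description text reflects the level scaling.
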(event Custom|DealDamage
  (params (ProjectileSource :type BP%20Game%20Character%20Object%20Reference) (ProjectileTarget :type BP%20Game%20Character%20Object%20Reference) (Critical :type Boolean))
  (bind _level (Variables|/Game/Actors/Characters/BP_GameCharacter.BP_GameCharacter_C|GetLevel ProjectileSource))
  (bind _returnvalue (<= _level 4))
  (bind _roll (Default|Roll (Utilities|GetDice) ProjectileSource 0 0 0 0 0 (Math|Integer|SelectInt (Math|Integer|SelectInt 1 2 _returnvalue) (Math|Integer|SelectInt 2 4 _returnvalue) Critical) 0 0 "NewEnumerator0" "NewEnumerator0"))
  (Default|ReceiveDamage ProjectileTarget _roll self ProjectileSource))

(fn DoAction
  (params (SourceCharacter :type BP%20Game%20Character%20Object%20Reference) (TargetCharacter :type BP%20Game%20Character%20Object%20Reference) (TargetLocation :type Vector :default "0, 0, 0") (AttackRollSuccess :type Boolean) (AttackRollCritical :type Boolean))
  (if AttackRollSuccess
    (bind _asbp_game_instance (Utilities|Casting|CastToBP_GameInstance (Game|GetGameInstance SourceCharacter)))
    (bind _returnvalue (Default|SpawnProjectile _asbp_game_instance "/Game/Data/Actions/Level0Spells/Mage/PoisonSpray/BP_PoisonSprayProjectile.BP_PoisonSprayProjectile_C" (Transformation|GetActorLocation SourceCharacter) SourceCharacter TargetCharacter SourceCharacter AttackRollCritical SourceCharacter))
    (EventDispatchers|BindEventtoOnTargetReached _returnvalue (EventDispatchers|CreateEvent :!event Custom|DealDamage))))

(fn GetDescription
  (params (Caster :type BP%20Game%20Character%20Object%20Reference) (PlayerData :type ST%20Player%20Data%20Structure))
  (bind _returnvalue (Utilities|Text|MakeLiteralText "Spray an enemy with a jet of poison. Deals {0} points of damage"))
  (Utilities|IsValid Caster
    (:Is%20Valid
      (return (Utilities|Text|FormatText _returnvalue (Utilities|String|SelectText "1d12" "2d12" (<= (Variables|/Game/Actors/Characters/BP_GameCharacter.BP_GameCharacter_C|GetLevel Caster) 4)))))
    (:Is%20Not%20Valid
      (return (Utilities|Text|FormatText _returnvalue (Utilities|String|SelectText "1d12" "2d12" (<= (.Level (Utilities|Struct|BreakST_PlayerData PlayerData)) 4)))))))

(fn AttackRoll
  (params (Character :type BP%20Game%20Character%20Object%20Reference) (Target :type BP%20Game%20Character%20Object%20Reference) (RollMod :type Integer) (AdvantageModifier :type Integer))
  (bind _ac (Variables|/Game/Actors/Characters/BP_GameCharacter.BP_GameCharacter_C|GetAC Target))
  (bind (_success _critical _result _diceresult) (Utilities|AbilityCheck Character RollMod 0 0 0 0 0 1 0 (Utilities|Array|MakeArray "NewEnumerator3") "NewEnumerator0" 0 _ac))
  (return (or _success _critical) _critical _result _diceresult _ac AdvantageModifier))