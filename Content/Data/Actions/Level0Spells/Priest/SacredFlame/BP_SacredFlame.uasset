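; Sacred Flame, a level 0 Priest spell action that deals holy light damage to a target.
; The target rolls an ability save against the caster's spell save difficulty and takes damage only on a failure, with the attack roll inputs unused.
; Damage is a d8 roll that gains a second die at higher caster level, plus the Wisdom modifier if the caster has the matching gameplay tag.
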(fn GetDescription
  (params (Caster :type BP%20Game%20Character%20Object%20Reference) (PlayerData :type ST%20Player%20Data%20Structure))
  (Utilities|IsValid Caster
    (:Is%20Valid
      (return (Utilities|Text|FormatText "Throws holy light to the target and deals {dmg} of damage" (Utilities|String|SelectText "2d8" "1d8" (>= (Variables|/Game/Actors/Characters/BP_GameCharacter.BP_GameCharacter_C|GetLevel Caster) 4)))))
    (:Is%20Not%20Valid
      (return (Utilities|Text|FormatText "Throws holy light to the target and deals {dmg} of damage" (Utilities|String|SelectText "2d8" "1d8" (>= (.Level (Utilities|Struct|BreakST_PlayerData PlayerData)) 4)))))))

(fn DoAction
  (params (SourceCharacter :type BP%20Game%20Character%20Object%20Reference) (TargetCharacter :type BP%20Game%20Character%20Object%20Reference) (TargetLocation :type Vector :default "0, 0, 0") (AttackRollSuccess :type Boolean) (AttackRollCritical :type Boolean))
  (bind _success (Utilities|AbilitySave TargetCharacter "NewEnumerator1" (Utilities|GetSpellSaveThrowDifficulty SourceCharacter "NewEnumerator4")))
  (if (not _success)
    (bind _roll (Default|Roll (Utilities|GetDice) SourceCharacter 0 0 0 (Math|Integer|SelectInt 2 1 (>= (Variables|/Game/Actors/Characters/BP_GameCharacter.BP_GameCharacter_C|GetLevel SourceCharacter) 4)) 0 0 0 0 (select (GameplayTags|HasTag (Variables|/Game/Actors/Characters/BP_GameCharacter.BP_GameCharacter_C|GetGameplayTags SourceCharacter) "(TagName=\"Modifier.DamageRoll.WISSpellDamage\")") (Utilities|Array|MakeArray "NewEnumerator4") "NewEnumerator0") "NewEnumerator0"))
    (Default|ReceiveDamage TargetCharacter _roll self SourceCharacter)))