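; BP_Reaction is a reaction action for game characters, built on two passives: a trigger and an effect.
; Use toggles the ReactionTrigger passive on the source character, and availability always returns true.
; Cast pays the cost, then calls DoAction with a forced successful attack roll.
; DoAction adds the ReactionEffect passive to the source character, ignoring the target and roll.
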(event EventUse
  (params (SourceCharacter :type BP%20Game%20Character%20Object%20Reference))
  (bind _reactiontrigger (Variables|Default|GetReactionTrigger))
  (if (Utilities|Array|ContainsItem (Variables|/Game/Actors/Characters/BP_GameCharacter.BP_GameCharacter_C|GetPassives SourceCharacter) (Variables|Default|GetReactionTrigger))
    (Default|RemovePassive SourceCharacter _reactiontrigger)
    (else
      (Default|AddPassive SourceCharacter _reactiontrigger))))

(event EventCast
  (params (SourceCharacter :type BP%20Game%20Character%20Object%20Reference) (TargetCharacter :type Actor%20Object%20Reference) (TargetLocation :type Vector :default "0, 0, 0"))
  (CallFunction|PayCost SourceCharacter)
  (bind _asbp_game_character (Utilities|Casting|CastToBP_GameCharacter TargetCharacter)
    (:then
      _)
    (:CastFailed
      _))
  (CallFunction|DoAction SourceCharacter _asbp_game_character TargetLocation true false))

(fn CheckAvailability
  (params (SourceCharacter :type BP%20Game%20Character%20Object%20Reference))
  (return true))

(fn DoAction
  (params (SourceCharacter :type BP%20Game%20Character%20Object%20Reference) (TargetCharacter :type BP%20Game%20Character%20Object%20Reference) (TargetLocation :type Vector :default "0, 0, 0") (AttackRollSuccess :type Boolean) (AttackRollCritical :type Boolean))
  (Default|AddPassive SourceCharacter (Variables|Default|GetReactionEffect)))