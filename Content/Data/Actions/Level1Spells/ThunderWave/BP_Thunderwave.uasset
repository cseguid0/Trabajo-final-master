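; BP_Thunderwave is the action for the level 1 Thunderwave spell, a sound explosion around the caster.
; DoAction spawns a BP_ThunderwaveAoE at the caster's location through the game instance and triggers it with an event delegate.
; DealDamage skips the caster, rolls an ability save against the caster's spell DC, and applies 2d8 damage, halved on a successful save.
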(event Custom|DealDamage
  (params (Source :type BP%20Game%20Character%20Object%20Reference) (GameCharacter :type BP%20Game%20Character%20Object%20Reference))
  (if (!= Source GameCharacter)
    (bind _success (Utilities|AbilitySave GameCharacter "NewEnumerator2" (Utilities|GetSpellSaveThrowDifficulty Source "NewEnumerator3")))
    (bind _roll (Default|Roll (Utilities|GetDice) 0 0 0 0 2 0 0 0 0 "NewEnumerator0" "NewEnumerator0"))
    (if _success
      (Default|ReceiveDamage GameCharacter (/ _roll 2) self Source)
      (else
        (Default|ReceiveDamage GameCharacter _roll self Source)))))

(fn DoAction
  (params (SourceCharacter :type BP%20Game%20Character%20Object%20Reference) (TargetCharacter :type BP%20Game%20Character%20Object%20Reference) (TargetLocation :type Vector :default "0, 0, 0") (AttackRollSuccess :type Boolean) (AttackRollCritical :type Boolean))
  (bind _asbp_game_instance (Utilities|Casting|CastToBP_GameInstance (Game|GetGameInstance SourceCharacter)))
  (bind _returnvalue (Default|SpawnAoE _asbp_game_instance "/Game/Data/Actions/Level1Spells/ThunderWave/BP_ThunderwaveAoE.BP_ThunderwaveAoE_C" (Transformation|GetActorLocation SourceCharacter) SourceCharacter))
  (Default|Trigger _returnvalue (EventDispatchers|CreateEvent :!event Custom|DealDamage)))

(fn GetDescription
  (params (Caster :type BP%20Game%20Character%20Object%20Reference) (PlayerData :type ST%20Player%20Data%20Structure))
  (return "Makes a sound explosion around the caster"))