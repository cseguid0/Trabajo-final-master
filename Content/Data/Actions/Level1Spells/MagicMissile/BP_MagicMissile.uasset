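; Magic Missile level 1 spell action that fires three homing-style darts from the caster at a chosen target.
; DoAction starts ThrowDarts, which spawns three BP_MagicMissileProjectile actors through the game instance, spaced by a short delay.
; Each projectile's OnTargetReached event triggers DealDamage, which rolls 1d4+1 and applies it to the target with no attack roll or critical handling.
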(event Custom|ThrowDarts
  (params (Source :type BP%20Game%20Character%20Object%20Reference) (Target :type BP%20Game%20Character%20Object%20Reference))
  (bind _asbp_game_instance (Utilities|Casting|CastToBP_GameInstance (Game|GetGameInstance Target)))
  (for _index (range 1 3)
    (bind _returnvalue (Default|SpawnProjectile _asbp_game_instance "/Game/Data/Actions/Level1Spells/MagicMissile/BP_MagicMissileProjectile.BP_MagicMissileProjectile_C" (Transformation|GetActorLocation Source) Source Target Source false Source))
    (EventDispatchers|BindEventtoOnTargetReached _returnvalue (delegate Custom|DealDamage))
    (Utilities|FlowControl|Delay Source)))

(event Custom|DealDamage
  (params (ProjectileSource :type BP%20Game%20Character%20Object%20Reference) (ProjectileTarget :type BP%20Game%20Character%20Object%20Reference) (Critical :type Boolean))
  (bind _roll (Default|Roll (Utilities|GetDice) 0 1 1 0 0 0 0 0 0 "NewEnumerator0" "NewEnumerator0"))
  (Default|ReceiveDamage ProjectileTarget _roll self ProjectileSource))

(fn DoAction
  (params (SourceCharacter :type BP%20Game%20Character%20Object%20Reference) (TargetCharacter :type BP%20Game%20Character%20Object%20Reference) (TargetLocation :type Vector :default "0, 0, 0") (AttackRollSuccess :type Boolean) (AttackRollCritical :type Boolean))
  (CallFunction|ThrowDarts SourceCharacter TargetCharacter))

(fn GetDescription
  (params (Caster :type BP%20Game%20Character%20Object%20Reference) (PlayerData :type ST%20Player%20Data%20Structure))
  (return "Throw 3 darts that deal 1d4 + 1 points of damage each one"))