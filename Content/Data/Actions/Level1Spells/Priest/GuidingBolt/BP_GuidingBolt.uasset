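; Guiding Bolt, a level 1 Priest spell action that makes an attack against a target character.
; AttackRoll runs a d20 ability check with a stat modifier, roll modifier and advantage against the target's AC.
; DoAction rolls 4d6, adding a stat modifier only if the caster has the WIS spell damage tag, then deals damage and applies the Guiding Bolt passive, without reading the hit or critical inputs.
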(fn GetDescription
  (params (Caster :type BP%20Game%20Character%20Object%20Reference) (PlayerData :type ST%20Player%20Data%20Structure))
  (bind _description (|CallParentFunction Caster PlayerData))
  (return _description))

(fn DoAction
  (params (SourceCharacter :type BP%20Game%20Character%20Object%20Reference) (TargetCharacter :type BP%20Game%20Character%20Object%20Reference) (TargetLocation :type Vector :default "0, 0, 0") (AttackRollSuccess :type Boolean) (AttackRollCritical :type Boolean))
  (bind _roll (Default|Roll (Utilities|GetDice) SourceCharacter 0 0 4 0 0 0 0 0 (select (GameplayTags|HasTag (Variables|/Game/Actors/Characters/BP_GameCharacter.BP_GameCharacter_C|GetGameplayTags SourceCharacter) "(TagName=\"Modifier.DamageRoll.WISSpellDamage\")") (Utilities|Array|MakeArray "NewEnumerator4") "NewEnumerator0") "NewEnumerator0"))
  (Default|ReceiveDamage TargetCharacter _roll self SourceCharacter)
  (Default|AddPassive TargetCharacter "/Game/Data/Effects/GuidingBoltEffect/DA_GuidingBoltEffect.DA_GuidingBoltEffect"))

(fn AttackRoll
  (params (Character :type BP%20Game%20Character%20Object%20Reference) (Target :type BP%20Game%20Character%20Object%20Reference) (RollMod :type Integer) (AdvantageModifier :type Integer))
  (bind _ac (Variables|/Game/Actors/Characters/BP_GameCharacter.BP_GameCharacter_C|GetAC Target))
  (bind (_success _critical _result _diceresult) (Utilities|AbilityCheck Character RollMod 0 0 0 0 0 1 0 (Utilities|Array|MakeArray "NewEnumerator4") "NewEnumerator0" AdvantageModifier _ac))
  (return _success _critical _result _diceresult _ac AdvantageModifier))