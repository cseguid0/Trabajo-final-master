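; Cure Wounds, a level 1 Priest spell action that heals its target for 1d8 plus the caster's Wisdom.
; DoAction rolls through the dice object with the stat as modifier and passes the result to the target's ReceiveHealing.
; GetDescription fills the tooltip text with the Wisdom value from the caster, or from PlayerData when no valid caster exists, defaulting to 0 if the stat is missing.
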(fn GetDescription
  (params (Caster :type BP%20Game%20Character%20Object%20Reference) (PlayerData :type ST%20Player%20Data%20Structure))
  (bind _stats (Utilities|Struct|BreakST_PlayerData PlayerData))
  (bind _stats_2 (Variables|/Game/Actors/Characters/BP_GameCharacter.BP_GameCharacter_C|GetStats Caster))
  (bind (_value _returnvalue) (Utilities|Map|Find _stats "NewEnumerator4"))
  (bind (_value_2 _returnvalue_2) (Utilities|Map|Find _stats_2 "NewEnumerator4"))
  (Utilities|IsValid Caster
    (:Is%20Valid
      (return (Utilities|Text|FormatText "The target is healed 1d8 + {WIS}" (Math|Integer|SelectInt _value_2 0 _returnvalue_2))))
    (:Is%20Not%20Valid
      (return (Utilities|Text|FormatText "The target is healed 1d8 + {WIS}" (Math|Integer|SelectInt _value 0 _returnvalue))))))

(fn DoAction
  (params (SourceCharacter :type BP%20Game%20Character%20Object%20Reference) (TargetCharacter :type BP%20Game%20Character%20Object%20Reference) (TargetLocation :type Vector :default "0, 0, 0") (AttackRollSuccess :type Boolean) (AttackRollCritical :type Boolean))
  (bind _roll (Default|Roll (Utilities|GetDice) SourceCharacter 0 0 0 1 0 0 0 0 (Utilities|Array|MakeArray "NewEnumerator4") "NewEnumerator0"))
  (Default|ReceiveHealing TargetCharacter _roll))