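; Ray of Sickness is a level 1 spell action that damages a target and can poison it.
; It makes a d20 attack roll against AC, and on success spawns a projectile through the game instance, binding an event to its target-reached dispatcher.
; DealDamage rolls d8 damage, doubling the dice on a critical.
; A failed saving throw stores the caster's spell DC on the target and adds the Poisoned passive.
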(event Custom|DealDamage
  (params (ProjectileSource :type BP%20Game%20Character%20Object%20Reference) (ProjectileTarget :type BP%20Game%20Character%20Object%20Reference) (Critical :type Boolean))
  (bind _difficulty (Utilities|GetSpellSaveThrowDifficulty ProjectileSource "NewEnumerator3"))
  (bind _roll (Default|Roll (Utilities|GetDice) 0 0 0 0 (Math|Integer|SelectInt 4 2 Critical) 0 0 0 0 "NewEnumerator0" "NewEnumerator0"))
  (Default|ReceiveDamage ProjectileTarget _roll self ProjectileSource)
  (bind _success (Utilities|AbilitySave ProjectileTarget "NewEnumerator2" _difficulty))
  (if (not _success)
    (Utilities|Map|Add (Variables|/Game/Actors/Characters/BP_GameCharacter.BP_GameCharacter_C|GetPassivesData ProjectileTarget) "Poisoned_DC" _difficulty)
    (Default|AddPassive ProjectileTarget "/Game/Data/Effects/Poisoned/DA_Poisoned.DA_Poisoned")))

(fn AttackRoll
  (params (Character :type BP%20Game%20Character%20Object%20Reference) (Target :type BP%20Game%20Character%20Object%20Reference) (RollMod :type Integer) (AdvantageModifier :type Integer))
  (bind _ac (Variables|/Game/Actors/Characters/BP_GameCharacter.BP_GameCharacter_C|GetAC Target))
  (bind (_success _critical _result _diceresult) (Utilities|AbilityCheck Character RollMod 0 0 0 0 0 1 0 (Utilities|Array|MakeArray "NewEnumerator3") "NewEnumerator0" 0 _ac))
  (return (or _success _critical) _critical _result _diceresult _ac AdvantageModifier))

(fn DoAction
  (params (SourceCharacter :type BP%20Game%20Character%20Object%20Reference) (TargetCharacter :type BP%20Game%20Character%20Object%20Reference) (TargetLocation :type Vector :default "0, 0, 0") (AttackRollSuccess :type Boolean) (AttackRollCritical :type Boolean))
  (if AttackRollSuccess
    (bind _asbp_game_instance (Utilities|Casting|CastToBP_GameInstance (Game|GetGameInstance SourceCharacter)))
    (bind _returnvalue (Default|SpawnProjectile _asbp_game_instance "/Game/Data/Actions/Level1Spells/RayOfSickness/BP_RayOfSicknessProjectile.BP_RayOfSicknessProjectile_C" (Transformation|GetActorLocation SourceCharacter) SourceCharacter TargetCharacter SourceCharacter AttackRollCritical SourceCharacter))
    (EventDispatchers|BindEventtoOnTargetReached _returnvalue (EventDispatchers|CreateEvent :!event Custom|DealDamage))))

(fn GetDescription
  (params (Caster :type BP%20Game%20Character%20Object%20Reference) (PlayerData :type ST%20Player%20Data%20Structure))
  (return "Deals 2d8 poinst of damage.If the victim fails a constitution save, its poisoned and receives 1d4 damage in its turn until the saving throw is successfull"))