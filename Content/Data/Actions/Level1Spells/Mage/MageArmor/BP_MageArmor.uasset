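; Mage Armor, a level 1 Mage spell action that gives the caster an armor class bonus through a passive effect.
; DoAction adds the DA_MageArmorEffect passive to the source character, ignoring target and attack roll.
; GetDescription shows the AC gain as a stat modifier plus a flat bonus, reading the stat from the caster when valid, otherwise from PlayerData.
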(fn DoAction
  (params (SourceCharacter :type BP%20Game%20Character%20Object%20Reference) (TargetCharacter :type BP%20Game%20Character%20Object%20Reference) (TargetLocation :type Vector :default "0, 0, 0") (AttackRollSuccess :type Boolean) (AttackRollCritical :type Boolean))
  (Default|AddPassive SourceCharacter "/Game/Data/Effects/MageArmorEffect/DA_MageArmorEffect.DA_MageArmorEffect"))

(fn GetDescription
  (params (Caster :type BP%20Game%20Character%20Object%20Reference) (PlayerData :type ST%20Player%20Data%20Structure))
  (bind _stats (Utilities|Struct|BreakST_PlayerData PlayerData))
  (bind _returnvalue (Utilities|Text|MakeLiteralText "Surround yourself with a magic armor and gain {0} AC"))
  (bind _stats_2 (Variables|/Game/Actors/Characters/BP_GameCharacter.BP_GameCharacter_C|GetStats Caster))
  (bind (_value _returnvalue_2) (Utilities|Map|Find _stats "NewEnumerator1"))
  (bind (_value_2 _returnvalue_3) (Utilities|Map|Find _stats_2 "NewEnumerator1"))
  (Utilities|IsValid Caster
    (:Is%20Valid
      (return (Utilities|Text|FormatText _returnvalue (+ (Utilities|CalculateStatModifier (Math|Integer|SelectInt _value_2 0 _returnvalue_3)) 3))))
    (:Is%20Not%20Valid
      (return (Utilities|Text|FormatText _returnvalue (+ (Utilities|CalculateStatModifier (Math|Integer|SelectInt _value 0 _returnvalue_2)) 3))))))