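; Base action for spells and attacks in the turn-based RPG, with placeholder DoAction, AttackRoll and GetDescription for children to override.
; Use starts player casting; availability checks cover resources, status tags and combat turn, while targeting checks faction, range and line of sight.
; Cast pays costs, then either calls DoAction or offers the target a reaction, with ContinueCast resolving the roll.
; Caster and target passives hook each stage to modify or cancel attacks.
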(event Custom|Cast
  (params (SourceCharacter :type BP%20Game%20Character%20Object%20Reference) (TargetCharacter :type Actor%20Object%20Reference) (TargetLocation :type Vector))
  (bind _arrayelement (Utilities|Array|ReverseforEachLoop (Variables|/Game/Actors/Characters/BP_GameCharacter.BP_GameCharacter_C|GetPassives SourceCharacter))
    (:LoopBody
      (Class|BPIonCastingTrigger|OnCasting(Message) _arrayelement SourceCharacter self))
    (:Completed
      (CallFunction|PayCost SourceCharacter)
      (if (Variables|Default|GetHasAttackRoll)
        (Utilities|IsValid TargetCharacter
          (:Is%20Valid
            (bind _asbp_game_character (Utilities|Casting|CastToBP_GameCharacter TargetCharacter))
            (Default|OnReceiveAttackReaction _asbp_game_character SourceCharacter self))
          (:Is%20Not%20Valid
            (CallFunction|ContinueCast SourceCharacter 0 TargetLocation)))
        (Default|LoseStealth SourceCharacter :!label _label)
        (else
          (bind _asbp_game_character_2 (Utilities|Casting|CastToBP_GameCharacter TargetCharacter)
            (:then
              (bind _continueattack (CallFunction|OnReceivingAttackTrigger _asbp_game_character_2))
              (if _continueattack
                (CallFunction|DoAction SourceCharacter _asbp_game_character_2 TargetLocation true false)
                (goto _label)))
            (:CastFailed
              (CallFunction|DoAction SourceCharacter 0 TargetLocation true false))))))))

(event Custom|ContinueCast
  (params (SourceCharacter :type BP%20Game%20Character%20Object%20Reference) (TargetCharacter :type BP%20Game%20Character%20Object%20Reference) (TargetLocation :type Vector))
  (bind (_continueattack _attackrollmodifier) (CallFunction|OnReceivingAttackTrigger TargetCharacter))
  (if _continueattack
    (bind (_rollmodifier _advantagemodifier) (CallFunction|OnAttackTrigger SourceCharacter TargetCharacter))
    (bind (_success _critical _result _dice _difficulty _advantage) (CallFunction|AttackRoll SourceCharacter TargetCharacter (+ _rollmodifier _attackrollmodifier) _advantagemodifier))
    (bind (_success_2 _critical_2) (CallFunction|OnAfterAttackTrigger SourceCharacter _dice _result _difficulty _advantage _success _critical))
    (CallFunction|OnAfterReceivingAttackTrigger TargetCharacter SourceCharacter _success_2)
    (CallFunction|DoAction SourceCharacter TargetCharacter TargetLocation _success_2 _critical_2)))

(event EventUse
  (params (SourceCharacter :type BP%20Game%20Character%20Object%20Reference))
  (bind _asbp_player_controller (Utilities|Casting|CastToBP_PlayerController (Pawn|GetController SourceCharacter)))
  (Default|StartCasting _asbp_player_controller self))

(fn GetValidTargets
  (params (SourceCharacter :type BP%20Game%20Character%20Object%20Reference))
  (bind _returnvalue (Transformation|GetActorLocation SourceCharacter))
  (bind _range (Variables|Default|GetRange))
  (bind _outhits (Collision|MultiSphereTraceByChannel SourceCharacter _returnvalue (+ _returnvalue "0.000000,0.000000,0.010000") (Math|Float|SelectFloat (Variables|/Game/Actors/Characters/BP_GameCharacter.BP_GameCharacter_C|GetInteractionRange SourceCharacter) (Math|Conversions|ToFloat(Integer) _range) (== _range 0)) "TraceTypeQuery1" false 0 "None" false))
  (for _array_element _outhits
    (bind _asbp_game_character (Utilities|Casting|CastToBP_GameCharacter (.HitActor (Collision|BreakHitResult _array_element))))
    (bind _validtarget (CallFunction|CheckTargetIsValid SourceCharacter _asbp_game_character (.Location (Collision|BreakHitResult _array_element))))
    (if _validtarget
      (Utilities|Array|Add (LocalVariables|GetValidTargets) _asbp_game_character)))
  (return (LocalVariables|GetValidTargets)))

(fn CheckTargetIsValid
  (params (SourceCharacter :type BP%20Game%20Character%20Object%20Reference) (Target :type Actor%20Object%20Reference) (TargetLocation :type Vector))
  (bind _range (Variables|Default|GetRange))
  (bind _range_2 (Variables|Default|GetRange))
  (bind _range_3 (Variables|Default|GetRange))
  (LocalVariables|SetLSourceCharacter SourceCharacter)
  (LocalVariables|SetLTarget Target)
  (LocalVariables|SetLTargetLocation TargetLocation)
  (Utilities|Casting|CastToBP_PlayerCharacter SourceCharacter
    (:then
      (switch Utilities|FlowControl|Switch|SwitchonEnum_TargetType (Variables|Default|GetTargetType)
        (:NewEnumerator0
          (Utilities|Casting|CastToBP_HostileNPC (LocalVariables|GetLTarget)
            (:then
              (bind (_outhit _returnvalue) (Collision|LineTraceByChannel (LocalVariables|GetLSourceCharacter) (Transformation|GetActorLocation (LocalVariables|GetLSourceCharacter)) (Transformation|GetActorLocation (LocalVariables|GetLTarget)) "TraceTypeQuery1" false (Utilities|Array|MakeArray (LocalVariables|GetLSourceCharacter)) "None" false :!label _label))
              (return (Math|Boolean|ANDBoolean (== (LocalVariables|GetLTarget) (.HitActor (Collision|BreakHitResult _outhit))) _returnvalue (<= (.Distance (Collision|BreakHitResult _outhit)) (Math|Float|SelectFloat (Variables|/Game/Actors/Characters/BP_GameCharacter.BP_GameCharacter_C|GetInteractionRange (LocalVariables|GetLSourceCharacter)) (Math|Conversions|ToFloat(Integer) _range) (== _range 0))))))
            (:CastFailed
              (return false))))
        (:NewEnumerator1
          (if (== (LocalVariables|GetLSourceCharacter) (LocalVariables|GetLTarget))
            _
            (else
              (Utilities|Casting|CastToBP_FriendlyNPC (LocalVariables|GetLTarget)
                (:then
                  (goto _label))
                (:CastFailed
                  (return false))))))
        (:NewEnumerator2
          _)
        (:NewEnumerator3
          (bind (_outhit_2 _returnvalue_2) (Collision|LineTraceByChannel (LocalVariables|GetLSourceCharacter) (Transformation|GetActorLocation (LocalVariables|GetLSourceCharacter)) (LocalVariables|GetLTargetLocation) "TraceTypeQuery1" false 0 "ForDuration" :!label _label_2))
          (return (and (Math|Boolean|ORBoolean (Utilities|ClassIsChildOf (Utilities|GetClass (.HitActor (Collision|BreakHitResult _outhit_2))) "/Game/Actors/Characters/BP_GameCharacter.BP_GameCharacter_C") (not _returnvalue_2) (Utilities|Operators|EqualEqual (.Location (Collision|BreakHitResult _outhit_2)) (LocalVariables|GetLTargetLocation) 1e+01)) (<= (.Distance (Collision|BreakHitResult _outhit_2)) (Math|Float|SelectFloat (Variables|/Game/Actors/Characters/BP_GameCharacter.BP_GameCharacter_C|GetInteractionRange (LocalVariables|GetLSourceCharacter)) (Math|Conversions|ToFloat(Integer) _range_2) (== _range_2 0))))))))
    (:CastFailed
      (switch Utilities|FlowControl|Switch|SwitchonEnum_TargetType (Variables|Default|GetTargetType)
        (:NewEnumerator0
          (Utilities|Casting|CastToBP_PlayerCharacter (LocalVariables|GetLTarget)
            (:then
              (bind (_outhit_3 _returnvalue_3) (Collision|LineTraceByChannel (LocalVariables|GetLSourceCharacter) (Transformation|GetActorLocation (LocalVariables|GetLSourceCharacter)) (Transformation|GetActorLocation (LocalVariables|GetLTarget)) "TraceTypeQuery1" false 0 "None" :!label _label_3))
              (return (Math|Boolean|ANDBoolean (== (LocalVariables|GetLTarget) (.HitActor (Collision|BreakHitResult _outhit_3))) _returnvalue_3 (<= (.Distance (Collision|BreakHitResult _outhit_3)) (Math|Float|SelectFloat (Variables|/Game/Actors/Characters/BP_GameCharacter.BP_GameCharacter_C|GetInteractionRange (LocalVariables|GetLSourceCharacter)) (Math|Conversions|ToFloat(Integer) _range_3) (== _range_3 0))))))
            (:CastFailed
              (return false))))
        (:NewEnumerator1
          (if (== (LocalVariables|GetLSourceCharacter) (LocalVariables|GetLTarget))
            _
            (else
              (Utilities|Casting|CastToBP_HostileNPC (LocalVariables|GetLTarget)
                (:then
                  (goto _label_3))
                (:CastFailed
                  (return false))))))
        (:NewEnumerator2
          _)
        (:NewEnumerator3
          (goto _label_2)))))
  (return (== (LocalVariables|GetLSourceCharacter) (LocalVariables|GetLTarget))))

(fn GetDescription
  (params (Caster :type BP%20Game%20Character%20Object%20Reference) (PlayerData :type ST%20Player%20Data%20Structure))
  (return ""))

(fn DoAction
  (params (SourceCharacter :type BP%20Game%20Character%20Object%20Reference) (TargetCharacter :type BP%20Game%20Character%20Object%20Reference) (TargetLocation :type Vector) (AttackRollSuccess :type Boolean) (AttackRollCritical :type Boolean)))

(fn CanAfford
  (params (Character :type BP%20Game%20Character%20Object%20Reference))
  (bind (_keypin _valuepin) (Utilities|Map|ForEachLoop(Map) (Variables|Default|GetCost))
    (:then
      (if (.ReturnValue (Utilities|Map|Find (Variables|/Game/Actors/Characters/BP_GameCharacter.BP_GameCharacter_C|GetResources Character) _keypin))
        (if (> _valuepin (.Value (Utilities|Map|Find (Variables|/Game/Actors/Characters/BP_GameCharacter.BP_GameCharacter_C|GetResources Character) _keypin)))
          (return false))
        (else
          (return false))))
    (:CompletedPin
      (return true))))

(fn PayCost
  (params (Character :type BP%20Game%20Character%20Object%20Reference))
  (bind _resources (Variables|/Game/Actors/Characters/BP_GameCharacter.BP_GameCharacter_C|GetResources Character))
  (bind (_keypin _valuepin) (Utilities|Map|ForEachLoop(Map) (Variables|Default|GetCost))
    (:then
      (Utilities|Map|Add _resources _keypin (- (.Value (Utilities|Map|Find _resources _keypin)) _valuepin)))
    (:CompletedPin
      (return))))

(fn AttackRoll
  (params (Character :type BP%20Game%20Character%20Object%20Reference) (Target :type BP%20Game%20Character%20Object%20Reference) (RollMod :type Integer) (AdvantageModifier :type Integer))
  (return true false RollMod RollMod 0 AdvantageModifier))

(fn OnAttackTrigger
  (params (Character :type BP%20Game%20Character%20Object%20Reference) (Target :type BP%20Game%20Character%20Object%20Reference))
  (bind _arrayelement (Utilities|Array|ReverseforEachLoop (Variables|/Game/Actors/Characters/BP_GameCharacter.BP_GameCharacter_C|GetPassives Character))
    (:LoopBody
      (if (Utilities|DoesObjectImplementInterface _arrayelement "/Game/Data/Effects/BPI_OnAttackTrigger.BPI_OnAttackTrigger_C")
        (bind (_rollmodifier _advantagemodifier) (Class|BPIonAttackTrigger|OnAttack(Message) _arrayelement Character Target self))
        (LocalVariables|SetTotalRollModifier _rollmodifier)
        (LocalVariables|SetTotalAdvantageModifier _advantagemodifier)))
    (:Completed
      (return (LocalVariables|GetTotalRollModifier) (LocalVariables|GetTotalAdvantageModifier)))))

(fn OnReceivingAttackTrigger
  (params (Character :type BP%20Game%20Character%20Object%20Reference))
  (Utilities|IsValid Character
    (:Is%20Valid
      (bind _arrayelement (Utilities|Array|ReverseforEachLoop (Variables|/Game/Actors/Characters/BP_GameCharacter.BP_GameCharacter_C|GetPassives Character))
        (:LoopBody
          (if (Utilities|DoesObjectImplementInterface _arrayelement "/Game/Data/Effects/BPI_OnReceivingAttackTrigger.BPI_OnReceivingAttackTrigger_C")
            (bind (_continueattack _attackrollmodifier) (Class|BPIonReceivingAttackTrigger|OnReceivingAttack(Message) _arrayelement Character self))
            (LocalVariables|SetTotalContinueAttack (and _continueattack (LocalVariables|GetTotalContinueAttack)))
            (LocalVariables|SetTotalAttackRollModifier (+ _attackrollmodifier (LocalVariables|GetTotalAttackRollModifier)))))
        (:Completed
          (return (LocalVariables|GetTotalContinueAttack) (LocalVariables|GetTotalAttackRollModifier)))))
    (:Is%20Not%20Valid
      (return true 0))))

(fn OnAfterAttackTrigger
  (params (Character :type BP%20Game%20Character%20Object%20Reference) (OldRoll :type Integer) (OldResult :type Integer) (Difficulty :type Integer) (Advantage :type Integer) (OldSuccess :type Boolean) (OldCritical :type Boolean))
  (LocalVariables|SetLSuccess OldSuccess)
  (LocalVariables|SetLCritical OldCritical)
  (bind _arrayelement (Utilities|Array|ReverseforEachLoop (Variables|/Game/Actors/Characters/BP_GameCharacter.BP_GameCharacter_C|GetPassives Character))
    (:LoopBody
      (if (Utilities|DoesObjectImplementInterface _arrayelement "/Game/Data/Effects/BPI_OnAfterAttackTrigger.BPI_OnAfterAttackTrigger_C")
        (bind (_success _critical) (Class|BPIonAfterAttackTrigger|OnAfterAttack(Message) _arrayelement Character self OldRoll OldResult Difficulty Advantage (LocalVariables|GetLSuccess) (LocalVariables|GetLCritical)))
        (LocalVariables|SetLSuccess _success)
        (LocalVariables|SetLCritical _critical)))
    (:Completed
      (return (LocalVariables|GetLSuccess) (LocalVariables|GetLCritical)))))

(fn OnAfterReceivingAttackTrigger
  (params (Character :type BP%20Game%20Character%20Object%20Reference) (Attacker :type BP%20Game%20Character%20Object%20Reference) (AttackSuccess :type Boolean))
  (bind _arrayelement (Utilities|Array|ReverseforEachLoop (Variables|/Game/Actors/Characters/BP_GameCharacter.BP_GameCharacter_C|GetPassives Character))
    (:LoopBody
      (Class|BPIonAfterReceivingAttackTrigger|OnAfterReceivingAttack(Message) _arrayelement Character Attacker self AttackSuccess))))

(fn CheckAvailability
  (params (SourceCharacter :type BP%20Game%20Character%20Object%20Reference))
  (bind _returnvalue (Pawn|GetController SourceCharacter))
  (bind _gameplaytags (Variables|/Game/Actors/Characters/BP_GameCharacter.BP_GameCharacter_C|GetGameplayTags SourceCharacter))
  (bind _canafford (CallFunction|CanAfford SourceCharacter))
  (if (Math|Boolean|ORBoolean (not _canafford) (and (Utilities|Array|ContainsItem (LocalVariables|GetSpellTypes) (Variables|Default|GetClassification)) (GameplayTags|HasTag _gameplaytags "(TagName=\"Status.Silenced\")")) (GameplayTags|HasTag _gameplaytags "(TagName=\"Status.Pacified\")"))
    (return false)
    (else
      (bind _asbp_rol_game_mode (Utilities|Casting|CastToBP_RolGameMode (Game|GetGameMode SourceCharacter)))
      (bind _asbp_player_controller (Utilities|Casting|CastToBP_PlayerController _returnvalue)
        (:then
          (return (or (not (Variables|/Game/GameMode/BP_RolGameMode.BP_RolGameMode_C|GetisInCombat _asbp_rol_game_mode)) (Variables|/Game/Controllers/BP_PlayerController.BP_PlayerController_C|GethasTurn _asbp_player_controller))))
        (:CastFailed
          (bind _asbp_npccontroller (Utilities|Casting|CastToBP_NPCController _returnvalue))
          (return (or (not (Variables|/Game/GameMode/BP_RolGameMode.BP_RolGameMode_C|GetisInCombat _asbp_rol_game_mode)) (Variables|/Game/Controllers/BP_NPCController.BP_NPCController_C|GethasTurn _asbp_npccontroller))))))))

(fn GetTooltipData
  (params (Character :type BP%20Game%20Character%20Object%20Reference))
  (bind _asbp_game_instance (Utilities|Casting|CastToBP_GameInstance (Game|GetGameInstance Character)))
  (bind _description (CallFunction|GetDescription Character (Variables|/Game/GameInstance/BP_GameInstance.BP_GameInstance_C|GetPlayerData _asbp_game_instance)))
  (return (Variables|Default|GetName) _description (Variables|Default|GetIcon)))