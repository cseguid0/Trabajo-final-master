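; BP_AoE is an area-of-effect action actor that Trigger fires, binding the caller's effect to its overlap event.
; It sphere-overlaps pawns within Radius and broadcasts that event for each BP_GameCharacter whose passives allow it.
; Passives implementing BPI_OnEnteringAoETrigger are polled in reverse, their answers ANDed.
; It draws a debug sphere, then plays optional Niagara and sound, destroying itself when the effect finishes, or next tick without one.
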(event Custom|SpawnAoE
  (Rendering|Debug|DrawDebugSphere (Transformation|GetActorLocation) (Variables|Settings|GetRadius) 12 "(R=1.000000,G=0.000000,B=0.820733,A=1.000000)" 3.0 1.0)
  (bind _outactors (Collision|SphereOverlapActors (Transformation|GetActorLocation) (Variables|Settings|GetRadius) (Utilities|Array|MakeArray "ObjectTypeQuery3") 0))
  (for _array_element _outactors
    (bind _asbp_game_character (Utilities|Casting|CastToBP_GameCharacter _array_element))
    (bind _affected (CallFunction|CheckonEnteringAoEPassives _asbp_game_character))
    (if _affected
      (Default|CallOnAoEOverlap (Variables|Default|GetSource) _asbp_game_character)))
  (bind _effect (Variables|Effects|GetEffect)
    (:then
      (bind _returnvalue (Niagara|SpawnSystemAttached _effect (Variables|Default|GetDefaultSceneRoot) "None" "0, 0, 0" "0, 0, 0" "KeepRelativeOffset" true))
      (EventDispatchers|BindEventtoOnSystemFinished _returnvalue (delegate Custom|onSystemFinish))
      (bind _sound (Variables|Effects|GetSound)
        (:then
          (Audio|PlaySoundatLocation _sound (Transformation|GetActorLocation) "0, 0, 0" 1.0 1.0 0.0 0 0 0 0))
        (:else)))
    (:else
      (Utilities|FlowControl|DelayUntilNextTick)
      (Actor|DestroyActor))))

(event Custom|onSystemFinish
  (params (PSystem :type Niagara%20Component%20Object%20Reference))
  (Actor|DestroyActor))

(event EventBeginPlay)

(fn ConstructionScript)

(fn Trigger
  (params (OnTriggerEffect :type Delegate%20%28by%20ref%29))
  (EventDispatchers|BindEventtoOnAoEOverlap OnTriggerEffect)
  (CallFunction|SpawnAoE))

(fn CheckonEnteringAoEPassives
  (params (Character :type BP%20Game%20Character%20Object%20Reference))
  (bind _arrayelement (Utilities|Array|ReverseforEachLoop (Variables|/Game/Actors/Characters/BP_GameCharacter.BP_GameCharacter_C|GetPassives Character))
    (:LoopBody
      (if (Utilities|DoesObjectImplementInterface _arrayelement "/Game/Data/Effects/BPI_OnEnteringAoETrigger.BPI_OnEnteringAoETrigger_C")
        (bind _affected (Class|BPIonEnteringAoETrigger|OnEnteringAoE(Message) _arrayelement Character (Variables|Default|GetSource) self))
        (LocalVariables|SetAffectedL (and _affected (LocalVariables|GetAffectedL)))))
    (:Completed
      (return (LocalVariables|GetAffectedL)))))