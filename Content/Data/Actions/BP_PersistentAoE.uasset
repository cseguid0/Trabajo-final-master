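; BP_PersistentAoE is a spherical area of effect that persists for a number of turns, then destroys itself.
; It counts down via the game mode's turn-change event, gated by a math expression on combat state and turn order.
; Entering or leaving characters' passives are polled through an interface to decide whether they are affected, controlling area callbacks and adding or removing a turn-start passive.
; Enter and exit effects and sounds play regardless.
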(event OnComponentBeginOverlap(CollisionSphere)
  (params (OverlappedComponent :type Primitive%20Component%20Object%20Reference) (OtherActor :type Actor%20Object%20Reference) (OtherComp :type Primitive%20Component%20Object%20Reference) (OtherBodyIndex :type Integer) (bFromSweep :type Boolean) (SweepResult :type Hit%20Result%20Structure%20%28by%20ref%29))
  (bind _returnvalue (Transformation|GetActorLocation OtherActor))
  (bind _asbp_game_character (Utilities|Casting|CastToBP_GameCharacter OtherActor))
  (Utilities|FlowControl|Sequence
    (:then_0
      (bind _affected (CallFunction|CheckonEnteringAoEPassives _asbp_game_character))
      (if _affected
        (Default|CallOnAreaEntered _asbp_game_character (Variables|Default|GetSource))
        (bind _onbeginningturneffect (Variables|Settings|GetonBeginningTurnEffect)
          (:then
            (Default|AddPassive _asbp_game_character _onbeginningturneffect))
          (:else))))
    (:then_1
      (bind _onentereffect (Variables|Effects|GetonEnterEffect)
        (:then
          (Niagara|SpawnSystematLocation _onentereffect _returnvalue))
        (:else
          _))
      (bind _onentersound (Variables|Effects|GetonEnterSound)
        (:then
          (Audio|PlaySoundatLocation _onentersound _returnvalue "0, 0, 0" 1.0 1.0 0.0 0 0 0 0))
        (:else)))))

(event OnComponentEndOverlap(CollisionSphere)
  (params (OverlappedComponent :type Primitive%20Component%20Object%20Reference) (OtherActor :type Actor%20Object%20Reference) (OtherComp :type Primitive%20Component%20Object%20Reference) (OtherBodyIndex :type Integer))
  (bind _returnvalue (Transformation|GetActorLocation OtherActor))
  (bind _asbp_game_character (Utilities|Casting|CastToBP_GameCharacter OtherActor))
  (Utilities|FlowControl|Sequence
    (:then_0
      (bind _affected (CallFunction|CheckonEnteringAoEPassives _asbp_game_character))
      (if _affected
        (Default|CallOnAreaLeft _asbp_game_character (Variables|Default|GetSource))
        (bind _onbeginningturneffect (Variables|Settings|GetonBeginningTurnEffect)
          (:then
            (Default|RemovePassive _asbp_game_character _onbeginningturneffect))
          (:else))))
    (:then_1
      (bind _onexiteffect (Variables|Effects|GetonExitEffect)
        (:then
          (Niagara|SpawnSystematLocation _onexiteffect _returnvalue))
        (:else
          _))
      (bind _onexitsound (Variables|Effects|GetonExitSound)
        (:then
          (Audio|PlaySoundatLocation _onexitsound _returnvalue "0, 0, 0" 1.0 1.0 0.0 0 0 0 0))
        (:else)))))

(event Custom|DecreaseTTL
  (bind _asbp_rol_game_mode (Utilities|Casting|CastToBP_RolGameMode (Game|GetGameMode)))
  (if (|((notInCombat||(CurrentTurn=={8E14827A-4239-984E-EC93-928C4F4B6666}))||(({8E14827A-4239-984E-EC93-928C4F4B6666}>=CombatMembers)&&(CurrentTurn==(CombatMembers-1)))) (Variables|/Game/GameMode/BP_RolGameMode.BP_RolGameMode_C|GetcurrentTurn _asbp_rol_game_mode) (Utilities|Array|Length (Variables|/Game/GameMode/BP_RolGameMode.BP_RolGameMode_C|GetcombatOrder _asbp_rol_game_mode)) (not (Variables|/Game/GameMode/BP_RolGameMode.BP_RolGameMode_C|GetisInCombat _asbp_rol_game_mode)))
    (Variables|Settings|SetTimeToLive (- (Variables|Settings|GetTimeToLive) 1))
    (if (== (Variables|Settings|GetTimeToLive) 0)
      (Actor|DestroyActor))))

(event EventBeginPlay
  (bind _asbp_rol_game_mode (Utilities|Casting|CastToBP_RolGameMode (Game|GetGameMode)))
  (EventDispatchers|BindEventtoOnTurnChanged _asbp_rol_game_mode (delegate Custom|DecreaseTTL)))

(event EventDestroyed
  (bind _asbp_rol_game_mode (Utilities|Casting|CastToBP_RolGameMode (Game|GetGameMode)))
  (EventDispatchers|UnbindEventfromOnTurnChanged _asbp_rol_game_mode (delegate Custom|DecreaseTTL)))

(fn ConstructionScript
  (Components|Sphere|SetSphereRadius (Variables|Default|GetCollisionSphere) (Variables|Settings|GetRadius) true))

(fn CheckonEnteringAoEPassives
  (params (Character :type BP%20Game%20Character%20Object%20Reference))
  (bind _arrayelement (Utilities|Array|ReverseforEachLoop (Variables|/Game/Actors/Characters/BP_GameCharacter.BP_GameCharacter_C|GetPassives Character))
    (:LoopBody
      (if (Utilities|DoesObjectImplementInterface _arrayelement "/Game/Data/Effects/BPI_OnEnteringAoETrigger.BPI_OnEnteringAoETrigger_C")
        (bind _affected (Class|BPIonEnteringAoETrigger|OnEnteringPersistentAoE(Message) _arrayelement Character (Variables|Default|GetSource) self))
        (LocalVariables|SetAffectedL (and _affected (LocalVariables|GetAffectedL)))))
    (:Completed
      (return (LocalVariables|GetAffectedL)))))