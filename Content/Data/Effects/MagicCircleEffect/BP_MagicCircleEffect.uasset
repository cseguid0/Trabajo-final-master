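; BP_MagicCircleEffect is the Magic Circle status effect that marks a character as pacified.
; It adds the Status.Pacified.MagicCircle gameplay tag when applied and removes it when the effect ends.
; Its persistent AoE entry hook returns false only when the character owns a BP_MagicCircleAoE it is entering, while the regular AoE hook always returns true.
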(event EventOnAdded
  (params (Character :type BP%20Game%20Character%20Object%20Reference))
  (GameplayTags|AddGameplayTag (Variables|/Game/Actors/Characters/BP_GameCharacter.BP_GameCharacter_C|GetGameplayTags Character) "(TagName=\"Status.Pacified.MagicCircle\")" :!class /Script/GameplayTags.BlueprintGameplayTagLibrary))

(event EventOnRemoved
  (params (Character :type BP%20Game%20Character%20Object%20Reference))
  (GameplayTags|RemoveGameplayTag (Variables|/Game/Actors/Characters/BP_GameCharacter.BP_GameCharacter_C|GetGameplayTags Character) "(TagName=\"Status.Pacified.MagicCircle\")" :!class /Script/GameplayTags.BlueprintGameplayTagLibrary))

(fn OnEnteringAoE
  (params (Character :type BP%20Game%20Character%20Object%20Reference) (AoEOwner :type BP%20Game%20Character%20Object%20Reference) (AoE :type BP%20Ao%20E%20Object%20Reference))
  (return true))

(fn OnEnteringPersistentAoE
  (params (Character :type BP%20Game%20Character%20Object%20Reference) (AoEOwner :type BP%20Game%20Character%20Object%20Reference) (PersistentAoE :type BP%20Persistent%20Ao%20E%20Object%20Reference))
  (return (not (and (== Character AoEOwner) (Class|GameplayStatics|ObjectIsA PersistentAoE "/Game/Data/Actions/Level3Spells/Priest/MagicCircle/BP_MagicCircleAoE.BP_MagicCircleAoE_C")))))