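; Magic Weapon passive effect that temporarily grants a character a flat damage bonus and returns a bonus from its attack hook.
; It stores a turn countdown in the character's PassivesData map when added and clears it when removed.
; Each turn start decrements the counter, or removes the passive once it reads zero or is missing.
; The damage hook leaves the multiplier neutral.
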(event EventOnAdded
  (params (Character :type BP%20Game%20Character%20Object%20Reference))
  (Utilities|Map|Add (Variables|/Game/Actors/Characters/BP_GameCharacter.BP_GameCharacter_C|GetPassivesData Character) "MagicWeaponEffect_Timer" 5))

(event EventOnRemoved
  (params (Character :type BP%20Game%20Character%20Object%20Reference))
  (Utilities|Map|Remove (Variables|/Game/Actors/Characters/BP_GameCharacter.BP_GameCharacter_C|GetPassivesData Character) "MagicWeaponEffect_Timer"))

(event EventOnBegginingTurn
  (params (Triggerer :type BP%20Game%20Character%20Object%20Reference))
  (bind _passivesdata (Variables|/Game/Actors/Characters/BP_GameCharacter.BP_GameCharacter_C|GetPassivesData Triggerer))
  (bind (_value _returnvalue) (Utilities|Map|Find _passivesdata "MagicWeaponEffect_Timer"))
  (bind _returnvalue_2 (Math|Integer|SelectInt _value 0 _returnvalue))
  (if (== _returnvalue_2 0)
    (Default|RemovePassive Triggerer self)
    (else
      (Utilities|Map|Add _passivesdata "MagicWeaponEffect_Timer" (- _returnvalue_2 1)))))

(fn OnAttack
  (params (Character :type BP%20Game%20Character%20Object%20Reference))
  (return 1))

(fn OnDealingDamage
  (params (Character :type BP%20Game%20Character%20Object%20Reference) (Damage :type Integer) (AttackType :type Enum_ActionClassification%20Enum :default "NewEnumerator0"))
  (return 1 1.0))