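; Crown of Madness passive effect that can deal damage to the affected character at the start of its turns.
; It stores a turn countdown and default save DC in PassivesData, clearing both on removal.
; Each turn it expires at zero or decrements and rolls an ability save: success deals 1d4 damage, failure removes it.
; The save reads CrownOfMadness_DC, unlike the stored CrownOfMadnessEffect_DC key.
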(event EventOnAdded
  (params (Character :type BP%20Game%20Character%20Object%20Reference))
  (bind _passivesdata (Variables|/Game/Actors/Characters/BP_GameCharacter.BP_GameCharacter_C|GetPassivesData Character))
  (Utilities|Map|Add _passivesdata "CrownOfMadnessEffect_Timer" 5)
  (if (not (.ReturnValue (Utilities|Map|Find _passivesdata "CrownOfMadnessEffect_DC")))
    (Utilities|Map|Add _passivesdata "CrownOfMadnessEffect_DC" 10)))

(event EventOnRemoved
  (params (Character :type BP%20Game%20Character%20Object%20Reference))
  (bind _passivesdata (Variables|/Game/Actors/Characters/BP_GameCharacter.BP_GameCharacter_C|GetPassivesData Character))
  (Utilities|Map|Remove _passivesdata "CrownOfMadnessEffect_Timer")
  (Utilities|Map|Remove _passivesdata "CrownOfMadnessEffect_DC"))

(event EventOnBegginingTurn
  (params (Triggerer :type BP%20Game%20Character%20Object%20Reference))
  (bind _passivesdata (Variables|/Game/Actors/Characters/BP_GameCharacter.BP_GameCharacter_C|GetPassivesData Triggerer))
  (bind (_value _returnvalue) (Utilities|Map|Find _passivesdata "CrownOfMadness_DC"))
  (bind (_value_2 _returnvalue_2) (Utilities|Map|Find _passivesdata "CrownOfMadnessEffect_Timer"))
  (bind _returnvalue_3 (Math|Integer|SelectInt _value_2 0 _returnvalue_2))
  (if (== _returnvalue_3 0)
    (Default|RemovePassive Triggerer self)
    (else
      (Utilities|Map|Add _passivesdata "CrownOfMadnessEffect_Timer" (- _returnvalue_3 1))
      (bind _success (Utilities|AbilitySave Triggerer "NewEnumerator4" (Math|Integer|SelectInt _value 0 _returnvalue)))
      (if _success
        (bind _roll (Default|Roll (Utilities|GetDice) 0 0 1 0 0 0 0 0 0 "NewEnumerator0" "NewEnumerator0"))
        (Default|ReceiveDamage Triggerer _roll "/Game/Data/Actions/Level2Spells/CrownOfMadness/DA_CrownOfMadness.DA_CrownOfMadness")
        (else
          (Default|RemovePassive Triggerer self))))))