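; BP_Curse is a passive effect that curses a character, reducing every stat.
; When added, it loops over all keys in the character's Stats map and rewrites each value lowered by a fixed amount.
; Removal adds the same amount back to every stat, and the passive removes itself when the character rests.
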(event EventOnAdded
  (params (Character :type BP%20Game%20Character%20Object%20Reference))
  (bind _stats (Variables|/Game/Actors/Characters/BP_GameCharacter.BP_GameCharacter_C|GetStats Character))
  (bind _keys (Utilities|Map|Keys _stats))
  (for _array_element _keys
    (Utilities|Map|Add _stats _array_element (- (.Value (Utilities|Map|Find _stats _array_element)) 2))))

(event EventOnRemoved
  (params (Character :type BP%20Game%20Character%20Object%20Reference))
  (bind _stats (Variables|/Game/Actors/Characters/BP_GameCharacter.BP_GameCharacter_C|GetStats Character))
  (bind _keys (Utilities|Map|Keys _stats))
  (for _array_element _keys
    (Utilities|Map|Add _stats _array_element (+ (.Value (Utilities|Map|Find _stats _array_element)) 2))))

(event EventOnRest
  (params (Character :type BP%20Game%20Character%20Object%20Reference))
  (Default|RemovePassive Character self))