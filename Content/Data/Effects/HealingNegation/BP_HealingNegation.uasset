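; Passive status effect that negates healing on the affected character for a limited number of turns.
; OnReceivingHeal returns zero for both the plain and factor heal modifiers.
; A timer in the character's PassivesData map grows by two on each application and drops by one at turn start.
; The passive removes itself when the timer reaches zero and clears the entry on removal.
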(event EventOnAdded
  (params (Character :type BP%20Game%20Character%20Object%20Reference))
  (bind _passivesdata (Variables|/Game/Actors/Characters/BP_GameCharacter.BP_GameCharacter_C|GetPassivesData Character))
  (bind (_value _returnvalue) (Utilities|Map|Find _passivesdata "HealingNegation_Timer"))
  (Utilities|Map|Add _passivesdata "HealingNegation_Timer" (+ (Math|Integer|SelectInt _value 0 _returnvalue) 2)))

(event EventOnBegginingTurn
  (params (Triggerer :type BP%20Game%20Character%20Object%20Reference))
  (bind _passivesdata (Variables|/Game/Actors/Characters/BP_GameCharacter.BP_GameCharacter_C|GetPassivesData Triggerer))
  (bind (_value _returnvalue) (Utilities|Map|Find _passivesdata "HealingNegation_Timer"))
  (bind _returnvalue_2 (Math|Integer|SelectInt _value 0 _returnvalue))
  (Utilities|Map|Add _passivesdata "HealingNegation_Timer" (- _returnvalue_2 1))
  (if (== _returnvalue_2 0)
    (Default|RemovePassive Triggerer self)))

(event EventOnRemoved
  (params (Character :type BP%20Game%20Character%20Object%20Reference))
  (Utilities|Map|Remove (Variables|/Game/Actors/Characters/BP_GameCharacter.BP_GameCharacter_C|GetPassivesData Character) "HealingNegation_Timer"))

(fn OnReceivingHeal
  (params (Heal :type Integer) (Healing%20Target :type BP%20Game%20Character%20Object%20Reference))
  (return 0 0.0))