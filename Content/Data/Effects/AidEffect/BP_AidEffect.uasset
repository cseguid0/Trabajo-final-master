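; BP_AidEffect is a passive character effect that temporarily grants bonus hit points.
; When added, it raises both MaxHP and HP by a fixed amount, and when removed it subtracts the same amount from both.
; On rest, it removes itself from the character, which ends the buff.
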(event EventOnAdded
  (params (Character :type BP%20Game%20Character%20Object%20Reference))
  (Variables|/Game/Actors/Characters/BP_GameCharacter.BP_GameCharacter_C|SetMaxHP Character (+ (Variables|/Game/Actors/Characters/BP_GameCharacter.BP_GameCharacter_C|GetMaxHP Character) 5))
  (Variables|/Game/Actors/Characters/BP_GameCharacter.BP_GameCharacter_C|SetHP Character (+ (Variables|/Game/Actors/Characters/BP_GameCharacter.BP_GameCharacter_C|GetHP Character) 5)))

(event EventOnRemoved
  (params (Character :type BP%20Game%20Character%20Object%20Reference))
  (Variables|/Game/Actors/Characters/BP_GameCharacter.BP_GameCharacter_C|SetMaxHP Character (- (Variables|/Game/Actors/Characters/BP_GameCharacter.BP_GameCharacter_C|GetMaxHP Character) 5))
  (Variables|/Game/Actors/Characters/BP_GameCharacter.BP_GameCharacter_C|SetHP Character (- (Variables|/Game/Actors/Characters/BP_GameCharacter.BP_GameCharacter_C|GetHP Character) 5)))

(event EventOnRest
  (params (Character :type BP%20Game%20Character%20Object%20Reference))
  (Default|RemovePassive Character self))