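; Stealth passive effect that crouches the character and grants status, attack-advantage and receive-attack-disadvantage gameplay tags, undoing both on removal.
; When the character is seen, the watcher's d20 roll sets the difficulty for the character's ability check, with Perception and Stealth tags supplying advantage or disadvantage.
; A math expression weighs both criticals against the check's success, and the passive removes itself if the character loses.
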(event EventOnAdded
  (params (Character :type BP%20Game%20Character%20Object%20Reference))
  (bind _gameplaytags (Variables|/Game/Actors/Characters/BP_GameCharacter.BP_GameCharacter_C|GetGameplayTags Character))
  (GameplayTags|AddGameplayTag _gameplaytags "(TagName=\"Status.Stealth\")" :!class /Script/GameplayTags.BlueprintGameplayTagLibrary)
  (GameplayTags|AddGameplayTag _gameplaytags "(TagName=\"Advantage.Attack.Stealth\")" :!class /Script/GameplayTags.BlueprintGameplayTagLibrary)
  (GameplayTags|AddGameplayTag _gameplaytags "(TagName=\"Disadvantage.ReceiveAttack.Stealth\")" :!class /Script/GameplayTags.BlueprintGameplayTagLibrary)
  (Character|Crouch Character))

(event EventOnRemoved
  (params (Character :type BP%20Game%20Character%20Object%20Reference))
  (bind _gameplaytags (Variables|/Game/Actors/Characters/BP_GameCharacter.BP_GameCharacter_C|GetGameplayTags Character))
  (GameplayTags|RemoveGameplayTag _gameplaytags "(TagName=\"Status.Stealth\")" :!class /Script/GameplayTags.BlueprintGameplayTagLibrary)
  (GameplayTags|RemoveGameplayTag _gameplaytags "(TagName=\"Advantage.Attack.Stealth\")" :!class /Script/GameplayTags.BlueprintGameplayTagLibrary)
  (GameplayTags|RemoveGameplayTag _gameplaytags "(TagName=\"Disadvantage.ReceiveAttack.Stealth\")" :!class /Script/GameplayTags.BlueprintGameplayTagLibrary)
  (Character|UnCrouch Character))

(event EventOnSeen
  (params (Watcher :type BP%20Game%20Character%20Object%20Reference) (Character :type BP%20Game%20Character%20Object%20Reference))
  (bind (_roll _diceresult _critical) (Default|Roll (Utilities|GetDice) Watcher 0 0 0 0 0 0 1 0 (Utilities|Array|MakeArray "NewEnumerator4") (Utilities|Array|MakeArray "NewEnumerator11") (Utilities|CountAdvantage Watcher (GameplayTags|MakeLiteralGameplayTagContainer "(GameplayTags=((TagName=\"Advantage.Perception\")))") (GameplayTags|MakeLiteralGameplayTagContainer "(GameplayTags=((TagName=\"Disadvantage.Perception\")))"))))
  (bind (_success _critical_2) (Utilities|AbilityCheck Character 0 0 0 0 0 0 1 0 (Utilities|Array|MakeArray "NewEnumerator1") (Utilities|Array|MakeArray "NewEnumerator16") (Utilities|CountAdvantage Character (GameplayTags|MakeLiteralGameplayTagContainer "(GameplayTags=((TagName=\"Advantage.Stealth\")))") (GameplayTags|MakeLiteralGameplayTagContainer "(GameplayTags=((TagName=\"Disadvantage.Stealth\")))")) _roll))
  (if (not (|(((CriticalSuccess==CriticalDefender)&&Success)||CriticalSuccess) _critical_2 _critical _success))
    (Default|RemovePassive Character self)))