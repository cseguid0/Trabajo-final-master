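; Enfeeblement is a passive debuff that applies a 0.5 factor modifier to the damage its bearer deals.
; When added, it stores a turn timer and a default save difficulty, unless one is already set, in the character's PassivesData map.
; Each turn start decrements the timer and rolls an ability save, removing the passive on success or when time runs out.
; Removal clears both stored entries.
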(event EventOnAdded
  (params (Character :type BP%20Game%20Character%20Object%20Reference))
  (bind _passivesdata (Variables|/Game/Actors/Characters/BP_GameCharacter.BP_GameCharacter_C|GetPassivesData Character))
  (Utilities|Map|Add _passivesdata "Enfeeblement_Timer" 5)
  (if (not (.ReturnValue (Utilities|Map|Find _passivesdata "Enfeeblement_DC")))
    (Utilities|Map|Add _passivesdata "Enfeeblement_DC" 10)))

(event EventOnRemoved
  (params (Character :type BP%20Game%20Character%20Object%20Reference))
  (bind _passivesdata (Variables|/Game/Actors/Characters/BP_GameCharacter.BP_GameCharacter_C|GetPassivesData Character))
  (Utilities|Map|Remove _passivesdata "Enfeeblement_Timer")
  (Utilities|Map|Remove _passivesdata "Enfeeblement_DC"))

(event EventOnBegginingTurn
  (params (Triggerer :type BP%20Game%20Character%20Object%20Reference))
  (bind _passivesdata (Variables|/Game/Actors/Characters/BP_GameCharacter.BP_GameCharacter_C|GetPassivesData Triggerer))
  (bind (_value _returnvalue) (Utilities|Map|Find _passivesdata "Enfeeblement_Timer"))
  (bind (_value_2 _returnvalue_2) (Utilities|Map|Find _passivesdata "Enfeeblement_DC"))
  (bind _returnvalue_3 (Math|Integer|SelectInt _value 0 _returnvalue))
  (Utilities|Map|Add _passivesdata "Enfeeblement_Timer" (- _returnvalue_3 1))
  (bind _success (Utilities|AbilitySave Triggerer "NewEnumerator2" (Math|Integer|SelectInt _value_2 0 _returnvalue_2)))
  (if (or _success (== _returnvalue_3 0))
    (Default|RemovePassive Triggerer self)))

(fn OnDealingDamage
  (params (Character :type BP%20Game%20Character%20Object%20Reference) (Damage :type Integer) (Attack :type BP%20Action%20Object%20Reference))
  (return 0 0.5))