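; Furtive Attack effect, a sneak-attack passive that adds bonus damage once armed by an advantaged hit, re-enabled each turn.
; A FurtiveAttack entry in the character's PassivesData acts as a three-state flag: ready, armed, spent.
; Turn start readies it, and a successful attack with advantage from either of two schools arms it.
; The next damage dealt spends it, adding a d6 roll scaled to half the character's level.
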(event EventOnBegginingTurn
  (params (Triggerer :type BP%20Game%20Character%20Object%20Reference))
  (Utilities|Map|Add (Variables|/Game/Actors/Characters/BP_GameCharacter.BP_GameCharacter_C|GetPassivesData Triggerer) "FurtiveAttack" 1))

(fn OnAfterAttack
  (params (Character :type BP%20Game%20Character%20Object%20Reference) (Attack :type BP%20Action%20Object%20Reference) (OldRoll :type Integer) (OldResult :type Integer) (Difficulty :type Integer) (Advantage :type Integer) (OldSuccess :type Boolean) (OldCritical :type Boolean))
  (bind _passivesdata (Variables|/Game/Actors/Characters/BP_GameCharacter.BP_GameCharacter_C|GetPassivesData Character))
  (bind _school (Variables|/Game/Data/Actions/BP_Action.BP_Action_C|GetSchool Attack))
  (bind (_value _returnvalue) (Utilities|Map|Find _passivesdata "FurtiveAttack"))
  (if (Math|Boolean|ANDBoolean (or (Utilities|Enum|Equal(Enum) _school "NewEnumerator4") (Utilities|Enum|Equal(Enum) _school "NewEnumerator3")) (> Advantage 0) OldSuccess (> (Math|Integer|SelectInt _value 0 _returnvalue) 0))
    (Utilities|Map|Add _passivesdata "FurtiveAttack" 0))
  (return OldSuccess OldCritical))

(fn OnDealingDamage
  (params (Character :type BP%20Game%20Character%20Object%20Reference) (Damage :type Integer) (Attack :type BP%20Action%20Object%20Reference))
  (bind _passivesdata (Variables|/Game/Actors/Characters/BP_GameCharacter.BP_GameCharacter_C|GetPassivesData Character))
  (bind (_value _returnvalue) (Utilities|Map|Find _passivesdata "FurtiveAttack"))
  (if (== (Math|Integer|SelectInt _value -1 _returnvalue) 0)
    (Utilities|Map|Add _passivesdata "FurtiveAttack" -1)
    (bind _roll (Default|Roll (Utilities|GetDice) Character 0 0 (/ (Variables|/Game/Actors/Characters/BP_GameCharacter.BP_GameCharacter_C|GetLevel Character) 2) 0 0 0 0 0 "NewEnumerator0" "NewEnumerator0"))
    (return _roll 1.0)
    (else
      (return 0 1.0))))