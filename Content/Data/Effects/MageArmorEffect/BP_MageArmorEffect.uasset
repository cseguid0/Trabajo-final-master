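; Mage Armor passive effect that raises a character's AC until removed or until the character rests.
; OnAdded adds 3 plus the modifier of one looked-up stat to AC, then stores the resulting total AC in PassivesData.
; OnRemoved subtracts that stored value, which is the full total rather than just the bonus, and clears the entry.
; OnRest removes the passive from the character.
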(event EventOnAdded
  (params (Character :type BP%20Game%20Character%20Object%20Reference))
  (bind _stats (Variables|/Game/Actors/Characters/BP_GameCharacter.BP_GameCharacter_C|GetStats Character))
  (bind (_value _returnvalue) (Utilities|Map|Find _stats "NewEnumerator1"))
  (bind _output_get (Variables|/Game/Actors/Characters/BP_GameCharacter.BP_GameCharacter_C|SetAC Character (+ (Variables|/Game/Actors/Characters/BP_GameCharacter.BP_GameCharacter_C|GetAC Character) 3 (Utilities|CalculateStatModifier (Math|Integer|SelectInt _value 0 _returnvalue)))))
  (Utilities|Map|Add (Variables|/Game/Actors/Characters/BP_GameCharacter.BP_GameCharacter_C|GetPassivesData Character) "MageArmor_Armor" _output_get))

(event EventOnRemoved
  (params (Character :type BP%20Game%20Character%20Object%20Reference))
  (bind _passivesdata (Variables|/Game/Actors/Characters/BP_GameCharacter.BP_GameCharacter_C|GetPassivesData Character))
  (bind (_value _returnvalue) (Utilities|Map|Find _passivesdata "MageArmor_Armor"))
  (Variables|/Game/Actors/Characters/BP_GameCharacter.BP_GameCharacter_C|SetAC Character (- (Variables|/Game/Actors/Characters/BP_GameCharacter.BP_GameCharacter_C|GetAC Character) (Math|Integer|SelectInt _value 0 _returnvalue)))
  (Utilities|Map|Remove _passivesdata "MageArmor_Armor"))

(event EventOnRest
  (params (Character :type BP%20Game%20Character%20Object%20Reference))
  (Default|RemovePassive Character self))