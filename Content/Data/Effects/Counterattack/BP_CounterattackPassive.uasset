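; BP_CounterattackPassive is a passive effect that offers a character a counterattack reaction after an attack against them fails.
; On OnAfterReceivingAttack, it checks that the attack is of a specific school, did not succeed, and that the character has some of a specific resource left, treating a missing entry as zero.
; It then opens a UI_ReactionConfirmationWindow for the reaction, targeting the attacker.
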(event EventOnAfterReceivingAttack
  (params (Character :type BP%20Game%20Character%20Object%20Reference) (Attacker :type BP%20Game%20Character%20Object%20Reference) (Attack :type BP%20Action%20Object%20Reference) (AttackSuccess :type Boolean))
  (bind _resources (Variables|/Game/Actors/Characters/BP_GameCharacter.BP_GameCharacter_C|GetResources Character))
  (bind (_value _returnvalue) (Utilities|Map|Find _resources "NewEnumerator2"))
  (if (Math|Boolean|ANDBoolean (Utilities|Enum|Equal(Enum) (Variables|/Game/Data/Actions/BP_Action.BP_Action_C|GetSchool Attack) "NewEnumerator3") (not AttackSuccess) (> (Math|Integer|SelectInt _value 0 _returnvalue) 0))
    (bind _returnvalue_2 (UserInterface|CreateWidget Character "/Game/UI/ReactionConfirmationWindow/UI_ReactionConfirmationWindow.UI_ReactionConfirmationWindow_C" 0 (Variables|Default|GetReaction) Character Attacker))
    (UserInterface|Viewport|AddtoViewport _returnvalue_2 0)))