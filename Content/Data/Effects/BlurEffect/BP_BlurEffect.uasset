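; BP_BlurEffect is a turn-limited Blur passive that tags its character with Advantage.ReceiveAttack.Blur while active.
; Adding it sets the tag and seeds a counter in the character's PassivesData map, and removing it clears both.
; At each turn start it decrements the counter, or removes itself if the counter is already zero or missing.
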(event EventOnAdded
  (params (Character :type BP%20Game%20Character%20Object%20Reference))
  (Utilities|Map|Add (Variables|/Game/Actors/Characters/BP_GameCharacter.BP_GameCharacter_C|GetPassivesData Character) "BlurEffect_Timer" 5)
  (GameplayTags|AddGameplayTag (Variables|/Game/Actors/Characters/BP_GameCharacter.BP_GameCharacter_C|GetGameplayTags Character) "(TagName=\"Advantage.ReceiveAttack.Blur\")" :!class /Script/GameplayTags.BlueprintGameplayTagLibrary))

(event EventOnRemoved
  (params (Character :type BP%20Game%20Character%20Object%20Reference))
  (Utilities|Map|Remove (Variables|/Game/Actors/Characters/BP_GameCharacter.BP_GameCharacter_C|GetPassivesData Character) "BlurEffect_Timer")
  (GameplayTags|RemoveGameplayTag (Variables|/Game/Actors/Characters/BP_GameCharacter.BP_GameCharacter_C|GetGameplayTags Character) "(TagName=\"Advantage.ReceiveAttack.Blur\")" :!class /Script/GameplayTags.BlueprintGameplayTagLibrary))

(event EventOnBegginingTurn
  (params (Triggerer :type BP%20Game%20Character%20Object%20Reference))
  (bind _passivesdata (Variables|/Game/Actors/Characters/BP_GameCharacter.BP_GameCharacter_C|GetPassivesData Triggerer))
  (bind (_value _returnvalue) (Utilities|Map|Find _passivesdata "BlurEffect_Timer"))
  (bind _returnvalue_2 (Math|Integer|SelectInt _value 0 _returnvalue))
  (if (== _returnvalue_2 0)
    (Default|RemovePassive Triggerer self)
    (else
      (Utilities|Map|Add _passivesdata "BlurEffect_Timer" (- _returnvalue_2 1)))))