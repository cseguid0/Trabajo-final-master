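; Passive effect for Uncanny Dodge that gates a reaction offered before the character takes damage.
; It stores a single use in the character's PassivesData map, setting it when added, resetting it at the beginning of each turn and removing it with the passive.
; The before-damage check passes only if the character can afford the Reaction and the stored uses are above zero.
; The use is not decremented in this Blueprint.
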(event EventOnBegginingTurn
  (params (Triggerer :type BP%20Game%20Character%20Object%20Reference))
  (Utilities|Map|Add (Variables|/Game/Actors/Characters/BP_GameCharacter.BP_GameCharacter_C|GetPassivesData Triggerer) "UncannyDodge_Uses" 1))

(event EventOnAdded
  (params (Character :type BP%20Game%20Character%20Object%20Reference))
  (Utilities|Map|Add (Variables|/Game/Actors/Characters/BP_GameCharacter.BP_GameCharacter_C|GetPassivesData Character) "UncannyDodge_Uses" 1))

(event EventOnRemoved
  (params (Character :type BP%20Game%20Character%20Object%20Reference))
  (Utilities|Map|Remove (Variables|/Game/Actors/Characters/BP_GameCharacter.BP_GameCharacter_C|GetPassivesData Character) "UncannyDodge_Uses"))

(fn OnBeforeDamageReaction
  (params (Character :type BP%20Game%20Character%20Object%20Reference))
  (bind _passivesdata (Variables|/Game/Actors/Characters/BP_GameCharacter.BP_GameCharacter_C|GetPassivesData Character))
  (bind (_value _returnvalue) (Utilities|Map|Find _passivesdata "UncannyDodge_Uses"))
  (bind _canafford (Default|CanAfford (Variables|Default|GetReaction) Character))
  (return (and _canafford (> (Math|Integer|SelectInt _value 0 _returnvalue) 0))))