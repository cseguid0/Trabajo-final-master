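; BP_AbjurationSpecialization is an effect that shields a character when they cast a spell of one school, presumably Abjuration.
; On casting, it checks the spell's school and grants a shield equal to twice the spell's level.
; GetSpellLevel derives that level from the spell's cost keys, mapping spell-slot types to their level and other costs to zero, then taking the maximum.
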(event EventOnCasting
  (params (Character :type BP%20Game%20Character%20Object%20Reference) (Spell :type BP%20Action%20Object%20Reference))
  (if (Utilities|Enum|Equal(Enum) (Variables|/Game/Data/Actions/BP_Action.BP_Action_C|GetSchool Spell) "NewEnumerator1")
    (bind _level (CallFunction|GetSpellLevel Spell))
    (Default|ReceiveShield Character (* _level 2))))

(fn GetSpellLevel
  (params (Spell :type BP%20Action%20Object%20Reference))
  (bind _keys (Utilities|Map|Keys (Variables|/Game/Data/Actions/BP_Action.BP_Action_C|GetCost Spell)))
  (for _array_element _keys
    (Utilities|Array|Add (LocalVariables|GetCostLevelArray) (Utilities|Select :Index _array_element :NewEnumerator0 0 :NewEnumerator1 0 :NewEnumerator2 0 :NewEnumerator3 1 :NewEnumerator4 2 :NewEnumerator5 3 :NewEnumerator6 0)))
  (return (.MaxValue (Math|Integer|MaxOfIntArray (LocalVariables|GetCostLevelArray)))))