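; BP_AdditionalAttack is a passive effect that tracks an additional attack through an "AdditionalAttack" entry in the character's PassivesData.
; OnAttack toggles that entry only for the standard and ranged attack assets, adding it on one attack and removing it on the next.
; The turn-start event clears the entry, and OnAttack leaves roll and advantage modifiers at zero.
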(event EventOnBegginingTurn
  (params (Triggerer :type BP%20Game%20Character%20Object%20Reference))
  (Utilities|Map|Remove (Variables|/Game/Actors/Characters/BP_GameCharacter.BP_GameCharacter_C|GetPassivesData Triggerer) "AdditionalAttack"))

(fn OnAttack
  (params (Character :type BP%20Game%20Character%20Object%20Reference) (Target :type BP%20Game%20Character%20Object%20Reference) (Attack :type BP%20Action%20Object%20Reference))
  (bind _passivesdata (Variables|/Game/Actors/Characters/BP_GameCharacter.BP_GameCharacter_C|GetPassivesData Character))
  (if (or (== Attack "/Game/Data/Actions/Actions/Attack/DA_Attack.DA_Attack") (== Attack "/Game/Data/Actions/Actions/RangedAttack/DA_RangedAttack.DA_RangedAttack"))
    (if (Utilities|Map|Contains _passivesdata "AdditionalAttack")
      (Utilities|Map|Remove _passivesdata "AdditionalAttack")
      (else
        (Utilities|Map|Add _passivesdata "AdditionalAttack" 0))))
  (return 0 0))