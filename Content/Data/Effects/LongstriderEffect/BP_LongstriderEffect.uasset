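; Longstrider passive effect that grants a character extra movement while it is active.
; When added, it raises both the character's total and remaining movement by a fixed amount, and subtracts the same amount from both when removed.
; The effect lasts until the character rests, at which point it removes itself through RemovePassive.
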(event EventOnAdded
  (params (Character :type BP%20Game%20Character%20Object%20Reference))
  (Variables|/Game/Actors/Characters/BP_GameCharacter.BP_GameCharacter_C|SetRemainingMovement Character (+ (Variables|/Game/Actors/Characters/BP_GameCharacter.BP_GameCharacter_C|GetRemainingMovement Character) 3e+02))
  (Variables|/Game/Actors/Characters/BP_GameCharacter.BP_GameCharacter_C|SetMovement Character (+ (Variables|/Game/Actors/Characters/BP_GameCharacter.BP_GameCharacter_C|GetMovement Character) 3e+02)))

(event EventOnRemoved
  (params (Character :type BP%20Game%20Character%20Object%20Reference))
  (Variables|/Game/Actors/Characters/BP_GameCharacter.BP_GameCharacter_C|SetRemainingMovement Character (- (Variables|/Game/Actors/Characters/BP_GameCharacter.BP_GameCharacter_C|GetRemainingMovement Character) 3e+02))
  (Variables|/Game/Actors/Characters/BP_GameCharacter.BP_GameCharacter_C|SetMovement Character (- (Variables|/Game/Actors/Characters/BP_GameCharacter.BP_GameCharacter_C|GetMovement Character) 3e+02)))

(event EventOnRest
  (params (Character :type BP%20Game%20Character%20Object%20Reference))
  (Default|RemovePassive Character self))