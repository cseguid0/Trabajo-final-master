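; Shield passive effect that governs whether a character can react with a shield before an attack.
; It keeps a Shield_Uses counter in the character's PassivesData map, set to one when added and at turn start, and removed with the passive.
; The pre-attack check passes only if the reaction is affordable and uses remain, treating a missing entry as zero.
; The counter is not decremented here.
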(event EventOnAdded
  (params (Character :type BP%20Game%20Character%20Object%20Reference))
  (Utilities|Map|Add (Variables|/Game/Actors/Characters/BP_GameCharacter.BP_GameCharacter_C|GetPassivesData Character) "Shield_Uses" 1))

(event EventOnBegginingTurn
  (params (Triggerer :type BP%20Game%20Character%20Object%20Reference))
  (Utilities|Map|Add (Variables|/Game/Actors/Characters/BP_GameCharacter.BP_GameCharacter_C|GetPassivesData Triggerer) "Shield_Uses" 1))

(event EventOnRemoved
  (params (Character :type BP%20Game%20Character%20Object%20Reference))
  (Utilities|Map|Remove (Variables|/Game/Actors/Characters/BP_GameCharacter.BP_GameCharacter_C|GetPassivesData Character) "Shield_Uses"))

(fn OnBeforeAttackReaction
  (params (Character :type BP%20Game%20Character%20Object%20Reference) (Attack :type BP%20Action%20Object%20Reference))
  (bind _passivesdata (Variables|/Game/Actors/Characters/BP_GameCharacter.BP_GameCharacter_C|GetPassivesData Character))
  (bind (_value _returnvalue) (Utilities|Map|Find _passivesdata "Shield_Uses"))
  (bind _canafford (Default|CanAfford (Variables|Default|GetReaction) Character))
  (return (and _canafford (> (Math|Integer|SelectInt _value 0 _returnvalue) 0))))