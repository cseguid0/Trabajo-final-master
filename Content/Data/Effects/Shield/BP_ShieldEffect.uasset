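; BP_ShieldEffect is a Shield passive effect that gives a character a temporary armor class bonus.
; When added, it raises AC by a fixed amount and decrements the Shield_Uses counter in the character's PassivesData map, storing zero if the key is missing.
; At the beginning of a turn, it subtracts the same bonus from the triggering character and removes itself from that character's passives.
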(event EventOnAdded
  (params (Character :type BP%20Game%20Character%20Object%20Reference))
  (bind _passivesdata (Variables|/Game/Actors/Characters/BP_GameCharacter.BP_GameCharacter_C|GetPassivesData Character))
  (bind (_value _returnvalue) (Utilities|Map|Find _passivesdata "Shield_Uses"))
  (Utilities|Map|Add _passivesdata "Shield_Uses" (Math|Integer|SelectInt (- _value 1) 0 _returnvalue))
  (Variables|/Game/Actors/Characters/BP_GameCharacter.BP_GameCharacter_C|SetAC Character (+ (Variables|/Game/Actors/Characters/BP_GameCharacter.BP_GameCharacter_C|GetAC Character) 5)))

(event EventOnBegginingTurn
  (params (Triggerer :type BP%20Game%20Character%20Object%20Reference))
  (Variables|/Game/Actors/Characters/BP_GameCharacter.BP_GameCharacter_C|SetAC Triggerer (- (Variables|/Game/Actors/Characters/BP_GameCharacter.BP_GameCharacter_C|GetAC Triggerer) 5))
  (Default|RemovePassive Triggerer self))