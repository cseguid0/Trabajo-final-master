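; Spirit Guardians spell effect that deals damage over time to the triggering character at the start of its turn.
; It searches a 500-unit sphere around that character for other characters with an attached Spirit Guardians AoE actor.
; Each AoE found triggers a save against that caster's spell DC and a 3d8 roll, adding a stat modifier if the caster has the Wisdom spell-damage tag.
; A successful save halves the damage.
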(event EventOnBegginingTurn
  (params (Triggerer :type BP%20Game%20Character%20Object%20Reference))
  (bind _outactors (Collision|SphereOverlapActors Triggerer (Transformation|GetActorLocation Triggerer) 5e+02 (Utilities|Array|MakeArray "ObjectTypeQuery3") "/Game/Actors/Characters/BP_GameCharacter.BP_GameCharacter_C" (Utilities|Array|MakeArray Triggerer)))
  (for _array_element _outactors
    (bind _asbp_game_character (Utilities|Casting|CastToBP_GameCharacter _array_element))
    (for _array_element_2 (Actor|GetAttachedActors _asbp_game_character true false)
      (if (Class|GameplayStatics|ObjectIsA _array_element_2 "/Game/Data/Actions/Level3Spells/Priest/SpiritGuardians/BP_SpiritGuardiansAoE.BP_SpiritGuardiansAoE_C")
        (bind _success (Utilities|AbilitySave Triggerer "NewEnumerator4" (Utilities|GetSpellSaveThrowDifficulty _asbp_game_character "NewEnumerator4")))
        (bind _roll (Default|Roll (Utilities|GetDice) Triggerer 0 0 0 3 0 0 0 0 (select (GameplayTags|HasTag (Variables|/Game/Actors/Characters/BP_GameCharacter.BP_GameCharacter_C|GetGameplayTags _asbp_game_character) "(TagName=\"Modifier.DamageRoll.WISSpellDamage\")") (Utilities|Array|MakeArray "NewEnumerator4") "NewEnumerator0") "NewEnumerator0"))
        (if _success
          (Default|ReceiveDoTDamage Triggerer (/ _roll 2))
          (else
            (Default|ReceiveDoTDamage Triggerer _roll)))))))