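; Passive Haste effect for turn-based play that temporarily raises a character's AC, doubles Movement and grants an extra point of one resource.
; OnAdded applies the bonuses to both current and maximum values and seeds a turn timer in the character's PassivesData map.
; OnBegginingTurn counts the timer down and removes the passive once it finds zero.
; OnRemoved clears the timer and reverses the bonuses, keeping the resource maximum at least one.
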(event EventOnAdded
  (params (Character :type BP%20Game%20Character%20Object%20Reference))
  (bind _maxresources (Variables|/Game/Actors/Characters/BP_GameCharacter.BP_GameCharacter_C|GetMaxResources Character))
  (bind _resources (Variables|/Game/Actors/Characters/BP_GameCharacter.BP_GameCharacter_C|GetResources Character))
  (bind (_value _returnvalue) (Utilities|Map|Find _maxresources "NewEnumerator0"))
  (bind (_value_2 _returnvalue_2) (Utilities|Map|Find _resources "NewEnumerator0"))
  (Utilities|Map|Add (Variables|/Game/Actors/Characters/BP_GameCharacter.BP_GameCharacter_C|GetPassivesData Character) "HasteEffect_Timer" 2)
  (Variables|/Game/Actors/Characters/BP_GameCharacter.BP_GameCharacter_C|SetAC Character (+ (Variables|/Game/Actors/Characters/BP_GameCharacter.BP_GameCharacter_C|GetAC Character) 2))
  (Variables|/Game/Actors/Characters/BP_GameCharacter.BP_GameCharacter_C|SetRemainingMovement Character (+ (Variables|/Game/Actors/Characters/BP_GameCharacter.BP_GameCharacter_C|GetMovement Character) (Variables|/Game/Actors/Characters/BP_GameCharacter.BP_GameCharacter_C|GetRemainingMovement Character)))
  (Variables|/Game/Actors/Characters/BP_GameCharacter.BP_GameCharacter_C|SetMovement Character (* (Variables|/Game/Actors/Characters/BP_GameCharacter.BP_GameCharacter_C|GetMovement Character) 2.0))
  (Utilities|Map|Add _maxresources "NewEnumerator0" (+ (Math|Integer|SelectInt _value 0 _returnvalue) 1))
  (Utilities|Map|Add _resources "NewEnumerator0" (+ (Math|Integer|SelectInt _value_2 0 _returnvalue_2) 1)))

(event EventOnRemoved
  (params (Character :type BP%20Game%20Character%20Object%20Reference))
  (bind _resources (Variables|/Game/Actors/Characters/BP_GameCharacter.BP_GameCharacter_C|GetResources Character))
  (bind _maxresources (Variables|/Game/Actors/Characters/BP_GameCharacter.BP_GameCharacter_C|GetMaxResources Character))
  (bind (_value _returnvalue) (Utilities|Map|Find _resources "NewEnumerator0"))
  (bind (_value_2 _returnvalue_2) (Utilities|Map|Find _maxresources "NewEnumerator0"))
  (Utilities|Map|Remove (Variables|/Game/Actors/Characters/BP_GameCharacter.BP_GameCharacter_C|GetPassivesData Character) "HasteEffect_Timer")
  (Variables|/Game/Actors/Characters/BP_GameCharacter.BP_GameCharacter_C|SetAC Character (- (Variables|/Game/Actors/Characters/BP_GameCharacter.BP_GameCharacter_C|GetAC Character) 2))
  (bind _output_get (Variables|/Game/Actors/Characters/BP_GameCharacter.BP_GameCharacter_C|SetMovement Character (/ (Variables|/Game/Actors/Characters/BP_GameCharacter.BP_GameCharacter_C|GetMovement Character) 2.0)))
  (Variables|/Game/Actors/Characters/BP_GameCharacter.BP_GameCharacter_C|SetRemainingMovement Character (- (Variables|/Game/Actors/Characters/BP_GameCharacter.BP_GameCharacter_C|GetRemainingMovement Character) _output_get))
  (Utilities|Map|Add _maxresources "NewEnumerator0" (Math|Integer|Max(Integer) (- (Math|Integer|SelectInt _value_2 0 _returnvalue_2) 1) 1))
  (Utilities|Map|Add _resources "NewEnumerator0" (- (Math|Integer|SelectInt _value 0 _returnvalue) 1)))

(event EventOnBegginingTurn
  (params (Triggerer :type BP%20Game%20Character%20Object%20Reference))
  (bind _passivesdata (Variables|/Game/Actors/Characters/BP_GameCharacter.BP_GameCharacter_C|GetPassivesData Triggerer))
  (bind (_value _returnvalue) (Utilities|Map|Find _passivesdata "HasteEffect_Timer"))
  (bind _returnvalue_2 (Math|Integer|SelectInt _value 0 _returnvalue))
  (if (== _returnvalue_2 0)
    (Default|RemovePassive Triggerer self)
    (else
      (Utilities|Map|Add _passivesdata "HasteEffect_Timer" (- _returnvalue_2 1)))))