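; BP_BaneEffect is a timed passive that applies the Bane debuff to a character in a turn-based, dice-roll combat system.
; When added, it tags the character with 1d4 Bane modifiers for attack rolls and ability saves and starts a five-turn timer in the character's PassivesData map.
; Each turn start decrements the timer and removes the passive at zero; removal clears both tags and the timer entry.
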(event EventOnAdded
  (params (Character :type BP%20Game%20Character%20Object%20Reference))
  (bind _gameplaytags (Variables|/Game/Actors/Characters/BP_GameCharacter.BP_GameCharacter_C|GetGameplayTags Character))
  (Utilities|Map|Add (Variables|/Game/Actors/Characters/BP_GameCharacter.BP_GameCharacter_C|GetPassivesData Character) "BaneEffect_Timer" 5)
  (GameplayTags|AddGameplayTag _gameplaytags "(TagName=\"Modifier.AttackRoll.-1d4.Bane\")" :!class /Script/GameplayTags.BlueprintGameplayTagLibrary)
  (GameplayTags|AddGameplayTag _gameplaytags "(TagName=\"Modifier.AbilitySave.-1d4.Bane\")" :!class /Script/GameplayTags.BlueprintGameplayTagLibrary))

(event EventOnRemoved
  (params (Character :type BP%20Game%20Character%20Object%20Reference))
  (bind _gameplaytags (Variables|/Game/Actors/Characters/BP_GameCharacter.BP_GameCharacter_C|GetGameplayTags Character))
  (Utilities|Map|Remove (Variables|/Game/Actors/Characters/BP_GameCharacter.BP_GameCharacter_C|GetPassivesData Character) "BaneEffect_Timer")
  (GameplayTags|RemoveGameplayTag _gameplaytags "(TagName=\"Modifier.AttackRoll.-1d4.Bane\")" :!class /Script/GameplayTags.BlueprintGameplayTagLibrary)
  (GameplayTags|RemoveGameplayTag _gameplaytags "(TagName=\"Modifier.AbilitySave.-1d4.Bane\")" :!class /Script/GameplayTags.BlueprintGameplayTagLibrary))

(event EventOnBegginingTurn
  (params (Triggerer :type BP%20Game%20Character%20Object%20Reference))
  (bind _passivesdata (Variables|/Game/Actors/Characters/BP_GameCharacter.BP_GameCharacter_C|GetPassivesData Triggerer))
  (bind (_value _returnvalue) (Utilities|Map|Find _passivesdata "BaneEffect_Timer"))
  (bind _returnvalue_2 (Math|Integer|SelectInt _value 0 _returnvalue))
  (Utilities|Map|Add _passivesdata "BaneEffect_Timer" (- _returnvalue_2 1))
  (if (== _returnvalue_2 0)
    (Default|RemovePassive Triggerer self)))