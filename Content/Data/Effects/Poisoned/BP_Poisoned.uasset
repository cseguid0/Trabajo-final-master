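; Poisoned passive status effect that deals 1d4 damage, attributed to Ray of Sickness, when applied to a character.
; Each turn start, the character rolls an ability save: success removes the passive, failure deals another 1d4.
; The save difficulty lives in the character's PassivesData under "Poisoned_DC", defaulting on application only if absent, and is cleared on removal.
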(event EventOnAdded
  (params (Character :type BP%20Game%20Character%20Object%20Reference))
  (bind _passivesdata (Variables|/Game/Actors/Characters/BP_GameCharacter.BP_GameCharacter_C|GetPassivesData Character))
  (bind _roll (Default|Roll (Utilities|GetDice) 0 0 1 0 0 0 0 0 0 "NewEnumerator0" "NewEnumerator0"))
  (Default|ReceiveDamage Character _roll "/Game/Data/Actions/Level1Spells/RayOfSickness/DA_RayOfSickness.DA_RayOfSickness")
  (if (not (.ReturnValue (Utilities|Map|Find _passivesdata "Poisoned_DC")))
    (Utilities|Map|Add _passivesdata "Poisoned_DC" 10)))

(event EventOnBegginingTurn
  (params (Triggerer :type BP%20Game%20Character%20Object%20Reference))
  (bind _passivesdata (Variables|/Game/Actors/Characters/BP_GameCharacter.BP_GameCharacter_C|GetPassivesData Triggerer))
  (bind (_value _returnvalue) (Utilities|Map|Find _passivesdata "Poisoned_DC"))
  (bind _success (Utilities|AbilitySave Triggerer "NewEnumerator2" (Math|Integer|SelectInt _value 0 _returnvalue)))
  (if _success
    (Default|RemovePassive Triggerer self)
    (else
      (bind _roll (Default|Roll (Utilities|GetDice) 0 0 1 0 0 0 0 0 0 "NewEnumerator0" "NewEnumerator0"))
      (Default|ReceiveDamage Triggerer _roll "/Game/Data/Actions/Level1Spells/RayOfSickness/DA_RayOfSickness.DA_RayOfSickness"))))

(event EventOnRemoved
  (params (Character :type BP%20Game%20Character%20Object%20Reference))
  (Utilities|Map|Remove (Variables|/Game/Actors/Characters/BP_GameCharacter.BP_GameCharacter_C|GetPassivesData Character) "Poisoned_DC"))