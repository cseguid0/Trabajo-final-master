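; BP_CombatStyleDefense is the Defense combat style effect, granting a character +1 AC while a shield is equipped.
; Equip and unequip events adjust AC when the item casts to BP_Shield.
; Adding or removing the style applies or reverts the bonus if the left weapon slot already holds a shield.
; AC is changed directly by increments rather than recalculated.
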(event EventOnEquip
  (params (Character :type BP%20Game%20Character%20Object%20Reference) (Equipment :type BP%20Equipable%20Item%20Object%20Reference))
  (Utilities|Casting|CastToBP_Shield Equipment)
  (Variables|/Game/Actors/Characters/BP_GameCharacter.BP_GameCharacter_C|SetAC Character (+ (Variables|/Game/Actors/Characters/BP_GameCharacter.BP_GameCharacter_C|GetAC Character) 1)))

(event EventOnRemoveEquipment
  (params (Character :type BP%20Game%20Character%20Object%20Reference) (Equipment :type BP%20Equipable%20Item%20Object%20Reference))
  (Utilities|Casting|CastToBP_Shield Equipment)
  (Variables|/Game/Actors/Characters/BP_GameCharacter.BP_GameCharacter_C|SetAC Character (- (Variables|/Game/Actors/Characters/BP_GameCharacter.BP_GameCharacter_C|GetAC Character) 1)))

(event EventOnAdded
  (params (Character :type BP%20Game%20Character%20Object%20Reference))
  (bind _leftweaponslot (Variables|/Game/Actors/Characters/BP_GameCharacter.BP_GameCharacter_C|GetLeftWeaponSlot Character))
  (Utilities|IsValid _leftweaponslot
    (:Is%20Valid
      (Utilities|Casting|CastToBP_Shield _leftweaponslot)
      (Variables|/Game/Actors/Characters/BP_GameCharacter.BP_GameCharacter_C|SetAC Character (+ (Variables|/Game/Actors/Characters/BP_GameCharacter.BP_GameCharacter_C|GetAC Character) 1)))))

(event EventOnRemoved
  (params (Character :type BP%20Game%20Character%20Object%20Reference))
  (bind _leftweaponslot (Variables|/Game/Actors/Characters/BP_GameCharacter.BP_GameCharacter_C|GetLeftWeaponSlot Character))
  (Utilities|IsValid _leftweaponslot
    (:Is%20Valid
      (Utilities|Casting|CastToBP_Shield _leftweaponslot)
      (Variables|/Game/Actors/Characters/BP_GameCharacter.BP_GameCharacter_C|SetAC Character (- (Variables|/Game/Actors/Characters/BP_GameCharacter.BP_GameCharacter_C|GetAC Character) 1)))))