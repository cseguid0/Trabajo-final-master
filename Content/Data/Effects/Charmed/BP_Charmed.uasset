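; BP_Charmed is a passive status effect that gives a character a Charisma disadvantage gameplay tag for a limited number of turns.
; Adding it applies the tag and stores a countdown in the character's PassivesData, and removal clears both.
; Each turn start decrements the countdown and removes the passive at zero.
; Receiving damage also removes it, leaving the damage unmodified.
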(event EventOnAdded
  (params (Character :type BP%20Game%20Character%20Object%20Reference))
  (GameplayTags|AddGameplayTag (Variables|/Game/Actors/Characters/BP_GameCharacter.BP_GameCharacter_C|GetGameplayTags Character) "(TagName=\"Disadvantage.CHA\")" :!class /Script/GameplayTags.BlueprintGameplayTagLibrary)
  (Utilities|Map|Add (Variables|/Game/Actors/Characters/BP_GameCharacter.BP_GameCharacter_C|GetPassivesData Character) "Charmed_Timer" 5))

(event EventOnRemoved
  (params (Character :type BP%20Game%20Character%20Object%20Reference))
  (GameplayTags|RemoveGameplayTag (Variables|/Game/Actors/Characters/BP_GameCharacter.BP_GameCharacter_C|GetGameplayTags Character) "(TagName=\"Disadvantage.CHA\")" :!class /Script/GameplayTags.BlueprintGameplayTagLibrary)
  (Utilities|Map|Remove (Variables|/Game/Actors/Characters/BP_GameCharacter.BP_GameCharacter_C|GetPassivesData Character) "Charmed_Timer"))

(event EventOnBegginingTurn
  (params (Triggerer :type BP%20Game%20Character%20Object%20Reference))
  (bind _passivesdata (Variables|/Game/Actors/Characters/BP_GameCharacter.BP_GameCharacter_C|GetPassivesData Triggerer))
  (bind (_value _returnvalue) (Utilities|Map|Find _passivesdata "Charmed_Timer"))
  (bind _returnvalue_2 (Math|Integer|SelectInt _value 0 _returnvalue))
  (Utilities|Map|Add _passivesdata "Charmed_Timer" (- _returnvalue_2 1))
  (if (== _returnvalue_2 0)
    (Default|RemovePassive Triggerer self)))

(fn OnReceivingDamage
  (params (Damage :type Integer) (Character :type BP%20Game%20Character%20Object%20Reference) (AttackType :type Enum_ActionClassification%20Enum :default "NewEnumerator0"))
  (Default|RemovePassive Character self)
  (return 0 1.0))