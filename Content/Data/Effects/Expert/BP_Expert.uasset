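; BP_Expert is an effect that grants expertise by doubling a character's value for its configured Proficiency.
; On add, it looks up the Proficiency in the character's Proficiencies map, treating a missing entry as zero, and writes back double the value.
; On removal, it repeats the lookup and writes back half, using integer division on the current value rather than restoring a stored original.
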(event EventOnAdded
  (params (Character :type BP%20Game%20Character%20Object%20Reference))
  (bind _proficiencies (Variables|/Game/Actors/Characters/BP_GameCharacter.BP_GameCharacter_C|GetProficiencies Character))
  (bind _proficiency (Variables|Default|GetProficiency))
  (bind (_value _returnvalue) (Utilities|Map|Find _proficiencies _proficiency))
  (Utilities|Map|Add _proficiencies (Variables|Default|GetProficiency) (* (Math|Integer|SelectInt _value 0 _returnvalue) 2)))

(event EventOnRemoved
  (params (Character :type BP%20Game%20Character%20Object%20Reference))
  (bind _proficiencies (Variables|/Game/Actors/Characters/BP_GameCharacter.BP_GameCharacter_C|GetProficiencies Character))
  (bind _proficiency (Variables|Default|GetProficiency))
  (bind (_value _returnvalue) (Utilities|Map|Find _proficiencies _proficiency))
  (Utilities|Map|Add _proficiencies (Variables|Default|GetProficiency) (/ (Math|Integer|SelectInt _value 0 _returnvalue) 2)))