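; True Strike passive effect that marks its holder with the Disadvantage.ReceiveAttack.TrueStrike gameplay tag.
; On add it applies the tag and starts a two-turn counter in the character's PassivesData map, and removal clears both.
; The counter drops at the start of each holder turn, removing the passive at zero.
; Damage of the first attack type also removes it early, without modifying the damage.
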(event EventOnAdded
  (params (Character :type BP%20Game%20Character%20Object%20Reference))
  (Utilities|Map|Add (Variables|/Game/Actors/Characters/BP_GameCharacter.BP_GameCharacter_C|GetPassivesData Character) "TrueStrikeEffect_Timer" 2)
  (GameplayTags|AddGameplayTag (Variables|/Game/Actors/Characters/BP_GameCharacter.BP_GameCharacter_C|GetGameplayTags Character) "(TagName=\"Disadvantage.ReceiveAttack.TrueStrike\")" :!class /Script/GameplayTags.BlueprintGameplayTagLibrary))

(event EventOnRemoved
  (params (Character :type BP%20Game%20Character%20Object%20Reference))
  (Utilities|Map|Remove (Variables|/Game/Actors/Characters/BP_GameCharacter.BP_GameCharacter_C|GetPassivesData Character) "TrueStrikeEffect_Timer")
  (GameplayTags|RemoveGameplayTag (Variables|/Game/Actors/Characters/BP_GameCharacter.BP_GameCharacter_C|GetGameplayTags Character) "(TagName=\"Disadvantage.ReceiveAttack.TrueStrike\")" :!class /Script/GameplayTags.BlueprintGameplayTagLibrary))

(event EventOnBegginingTurn
  (params (Triggerer :type BP%20Game%20Character%20Object%20Reference))
  (bind _passivesdata (Variables|/Game/Actors/Characters/BP_GameCharacter.BP_GameCharacter_C|GetPassivesData Triggerer))
  (bind (_value _returnvalue) (Utilities|Map|Find _passivesdata "TrueStrikeEffect_Timer"))
  (bind _returnvalue_2 (Math|Integer|SelectInt _value 0 _returnvalue))
  (Utilities|Map|Add _passivesdata "TrueStrikeEffect_Timer" (- _returnvalue_2 1))
  (if (== _returnvalue_2 0)
    (Default|RemovePassive Triggerer self)))

(fn OnReceivingDamage
  (params (Damage :type Integer) (Character :type BP%20Game%20Character%20Object%20Reference) (AttackType :type Enum_ActionClassification%20Enum :default "NewEnumerator0"))
  (if (Utilities|Enum|Equal(Enum) AttackType "NewEnumerator0")
    (Default|RemovePassive Character self))
  (return 0 1.0))