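; BP_WarDomain is an effect Blueprint for the War Domain that manages an extra-attack modifier tag on a character.
; OnAttack toggles the Modifier.ExtraAttack.WarDomain gameplay tag whenever the attack is DA_Attack, adding it if absent and removing it if present.
; It leaves roll and advantage modifiers at zero, and the turn-start event clears the tag from the triggerer.
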(event EventOnBegginingTurn
  (params (Triggerer :type BP%20Game%20Character%20Object%20Reference))
  (GameplayTags|RemoveGameplayTag (Variables|/Game/Actors/Characters/BP_GameCharacter.BP_GameCharacter_C|GetGameplayTags Triggerer) "(TagName=\"Modifier.ExtraAttack.WarDomain\")" :!class /Script/GameplayTags.BlueprintGameplayTagLibrary))

(fn OnAttack
  (params (Character :type BP%20Game%20Character%20Object%20Reference) (Target :type BP%20Game%20Character%20Object%20Reference) (Attack :type BP%20Action%20Object%20Reference))
  (bind _gameplaytags (Variables|/Game/Actors/Characters/BP_GameCharacter.BP_GameCharacter_C|GetGameplayTags Character))
  (if (== Attack "/Game/Data/Actions/Actions/Attack/DA_Attack.DA_Attack")
    (if (GameplayTags|HasTag _gameplaytags "(TagName=\"Modifier.ExtraAttack.WarDomain\")")
      (GameplayTags|RemoveGameplayTag _gameplaytags "(TagName=\"Modifier.ExtraAttack.WarDomain\")" :!class /Script/GameplayTags.BlueprintGameplayTagLibrary)
      (else
        (GameplayTags|AddGameplayTag _gameplaytags "(TagName=\"Modifier.ExtraAttack.WarDomain\")" :!class /Script/GameplayTags.BlueprintGameplayTagLibrary))))
  (return 0 0))