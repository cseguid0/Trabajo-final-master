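; RPG game mode that runs initiative-based turn combat and picks player starts by the game instance's spawn tag, except when loading saves.
; A looping timer triggers every character's turn-start passives and pauses when combat starts.
; StartCombat sorts characters by rolled initiative; turn changes and removals message their controllers, with HUD frames refreshed on start and EndTurn.
; CheckCombatEnd clears combat when only the player remains, but unpauses the timer only while combat continues.
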(event Custom|StartCombat
  (params (Characters :type Array%20of%20BP%20Game%20Character%20Object%20References))
  (if (not (Variables|Default|GetisInCombat))
    (Utilities|Time|PauseTimerbyHandle (Variables|Default|GetTurnBeginingTimer))
    (Variables|Default|SetisInCombat true)
    (Variables|Default|SetcurrentTurn 0)
    (Variables|Default|SetcombatOrder (Utilities|Array|MakeArray))
    (for _array_element Characters
      (bind _initiative (Default|RollInitiative _array_element))
      (CallFunction|CombatSortedInsertion _array_element _initiative))
    (bind _asbp_player_hud (Utilities|Casting|CastToBP_PlayerHUD (HUD|GetHUD (Game|GetPlayerController 0))))
    (Default|UpdateCombatFrames (Variables|/Game/UI/PlayerHUD/BP_PlayerHUD.BP_PlayerHUD_C|GetHUD _asbp_player_hud))
    (Class|BPIControllerOperations|MakeTurn(Message) (Pawn|GetController (.character (Utilities|Array|Get(acopy) (Variables|Default|GetcombatOrder) (Variables|Default|GetcurrentTurn)))))))

(event Custom|EndTurn
  (Class|BPIControllerOperations|EndTurn(Message) (Pawn|GetController (.character (Utilities|Array|Get(acopy) (Variables|Default|GetcombatOrder) (Variables|Default|GetcurrentTurn)))))
  (bind _output_get (Variables|Default|SetcurrentTurn (Math|Integer|%(Integer) (+ (Variables|Default|GetcurrentTurn) 1) (Utilities|Array|Length (Variables|Default|GetcombatOrder)))))
  (Class|BPIControllerOperations|MakeTurn(Message) (Pawn|GetController (.character (Utilities|Array|Get(acopy) (Variables|Default|GetcombatOrder) _output_get))))
  (bind _asbp_player_hud (Utilities|Casting|CastToBP_PlayerHUD (HUD|GetHUD (Game|GetPlayerController 0))))
  (Default|UpdateCombatFrames (Variables|/Game/UI/PlayerHUD/BP_PlayerHUD.BP_PlayerHUD_C|GetHUD _asbp_player_hud)))

(event Custom|CheckCombatEnd
  (bind _combatorder (Variables|Default|GetcombatOrder))
  (bind _output_get (Variables|Default|SetisInCombat (not (and (== (Utilities|Array|Length _combatorder) 1) (== (.character (Utilities|Array|Get(acopy) _combatorder)) (Pawn|GetControlledPawn (Game|GetPlayerController 0)))))))
  (if _output_get
    (Utilities|Time|UnpauseTimerbyHandle (Variables|Default|GetTurnBeginingTimer))))

(event Custom|TriggerAllBeginingTurnPassives
  (bind _outactors (Actor|GetAllActorsOfClass "/Game/Actors/Characters/BP_GameCharacter.BP_GameCharacter_C"))
  (for _array_element _outactors
    (for _array_element_2 (Variables|/Game/Actors/Characters/BP_GameCharacter.BP_GameCharacter_C|GetPassives _array_element)
      (Class|BPIBegginingTurnTrigger|BegginingTurnTrigger(Message) _array_element_2 _array_element))))

(event EventBeginPlay
  (bind _returnvalue (Utilities|Time|SetTimerbyEvent (delegate Custom|TriggerAllBeginingTurnPassives) 5.0 true))
  (Variables|Default|SetTurnBeginingTimer _returnvalue))

(event EventTick
  (params (DeltaSeconds :type Float%20%28single-precision%29)))

(fn ConstructionScript)

(fn CombatSortedInsertion
  (params (Character :type BP%20Game%20Character%20Object%20Reference) (Weight :type Integer))
  (bind (_array_element _array_index) (Utilities|Array|ForEachLoopwithBreak (Variables|Default|GetcombatOrder) :!label _label)
    (:LoopBody
      (if (> Weight (.initiative _array_element))
        (Utilities|Array|Insert (Variables|Default|GetcombatOrder) (Utilities|Struct|MakeST_CharacterWithInitiative Character Weight) _array_index)
        (LocalVariables|SetInserted true)
        (goto _label Break)))
    (:Completed
      (if (not (LocalVariables|GetInserted))
        (Utilities|Array|Add (Variables|Default|GetcombatOrder) (Utilities|Struct|MakeST_CharacterWithInitiative Character Weight))))))

(fn RemovefromCombatOrder
  (params (Character :type BP%20Game%20Character%20Object%20Reference))
  (bind (_array_element _array_index) (Utilities|Array|ForEachLoopwithBreak (Variables|Default|GetcombatOrder) :!label _label)
    (:LoopBody
      (if (== (.character _array_element) Character)
        (LocalVariables|SetIndex _array_index)
        (LocalVariables|SetFound true)
        (goto _label Break)))
    (:Completed
      (if (LocalVariables|GetFound)
        (Utilities|Array|RemoveIndex (Variables|Default|GetcombatOrder) (LocalVariables|GetIndex))
        (if (== (LocalVariables|GetIndex) (Variables|Default|GetcurrentTurn))
          (Class|BPIControllerOperations|EndTurn(Message) (Pawn|GetController Character))
          (Class|BPIControllerOperations|MakeTurn(Message) (Pawn|GetController (.character (Utilities|Array|Get(acopy) (Variables|Default|GetcombatOrder) (Variables|Default|GetcurrentTurn))))))))))

(fn ChoosePlayerStart
  (params (Player :type Controller%20Object%20Reference))
  (bind _asbp_game_instance (Utilities|Casting|CastToBP_GameInstance (Game|GetGameInstance))
    (:then
      (if (Variables|/Game/GameInstance/BP_GameInstance.BP_GameInstance_C|GetLoadingFromSaveFile _asbp_game_instance)
        (return 0)
        (else
          (bind _outactors (Actor|GetAllActorsOfClass "/Script/Engine.PlayerStart"))
          (for _array_element _outactors
            (if (== (Variables|/Script/Engine.PlayerStart|GetPlayerStartTag _array_element) (Variables|/Game/GameInstance/BP_GameInstance.BP_GameInstance_C|GetSpawnPoint _asbp_game_instance))
              (return _array_element)))
          (return 0))))
    (:CastFailed
      (return 0))))