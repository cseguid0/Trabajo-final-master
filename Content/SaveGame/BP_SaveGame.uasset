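; BP_SaveGame is a save game object that holds a snapshot of game state.
; SetSaveData fills it from the passed GameInstance, storing the current level name as CurrentMap and copying player, NPC, recipient, pickable item, action bar and quest data.
; The file only captures state, with no logic for writing it to a slot or restoring it.
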(fn SetSaveData
  (params (GameInstance :type BP%20Game%20Instance%20Object%20Reference))
  (bind _returnvalue (Game|GetCurrentLevelName GameInstance))
  (Variables|Default|SetCurrentMap _returnvalue)
  (Variables|Default|SetPlayerData (Variables|/Game/GameInstance/BP_GameInstance.BP_GameInstance_C|GetPlayerData GameInstance))
  (Variables|Default|SetNPCData (Variables|/Game/GameInstance/BP_GameInstance.BP_GameInstance_C|GetNPCData GameInstance))
  (Variables|Default|SetRecipientData (Variables|/Game/GameInstance/BP_GameInstance.BP_GameInstance_C|GetRecipientData GameInstance))
  (Variables|Default|SetPickableItemData (Variables|/Game/GameInstance/BP_GameInstance.BP_GameInstance_C|GetPickableItemData GameInstance))
  (Variables|Default|SetActionBarData (Variables|/Game/GameInstance/BP_GameInstance.BP_GameInstance_C|GetActionBarData GameInstance))
  (Variables|Default|SetQuestData (Variables|/Game/GameInstance/BP_GameInstance.BP_GameInstance_C|GetQuestData GameInstance)))